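; Drivable catapult that the player steers, aims and fires once it holds a picked-up projectile.
; Throttle and steer axes interpolate speed and steering angle, moving the actor along its right vector without sweep and yawing it in proportion to speed.
; The Catapult axis tilts the spoon within a clamped range, which CheckAngleOfSpoon converts into stepped vertical launch velocity alongside a fixed X velocity.
; Look inputs and speed-based spring arm logic are unconnected.
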(event Input|ActionEvents|InputActionAButton
  (params (Key :type Key%20Structure :default "None"))
  (:Pressed
    (if (Variables|Default|GetPicked%20up%20Projectile)
      (Utilities|FlowControl|DoOnce false :!label _label
        (:Completed
          (CallFunction|CheckAngleOfSpoon)
          (bind _returnvalue (Game|SpawnActorfromClass "/Game/CatapultCatch/Blueprints/Projectile_BP.Projectile_BP_C" (Transformation|GetWorldTransform (Variables|Default|GetProjectileLocation)) "AlwaysSpawn" "MultiplyWithRoot" 0 0))
          (Variables|/Script/Engine.MovementComponent|SetVelocity (Variables|/Game/CatapultCatch/Blueprints/Projectile_BP.Projectile_BP_C|GetProjectileMovement _returnvalue) (Math|Vector|MakeVector -1e+03 0.0 (Variables|Default|GetVelocity%20Z)))
          (Development|SetHiddeninGame (Variables|Default|GetSphere) true false)))))
  (:Released
    (Variables|Default|SetPicked%20up%20Projectile false)
    (goto _label Reset)))

(event Input|AxisEvents|InputAxisThrottle
  (params (AxisValue :type Float%20%28single-precision%29))
  (Variables|Default|SetCurrentSpeed (Math|Interpolation|FInterpTo (Variables|Default|GetCurrentSpeed) (* (* AxisValue (Variables|Default|GetThrottle%20Axis)) (Variables|Default|GetMaxSpeed)) (Utilities|Time|GetWorldDeltaSeconds) 4.0))
  (Transformation|AddActorWorldOffset (* (Utilities|Time|GetWorldDeltaSeconds) (* (Transformation|GetActorRightVector) (Variables|Default|GetCurrentSpeed))) false true))

(event Input|AxisEvents|InputAxisLookRight
  (params (AxisValue :type Float%20%28single-precision%29)))

(event Input|AxisEvents|InputAxisLookUp
  (params (AxisValue :type Float%20%28single-precision%29)))

(event Input|AxisEvents|InputAxisCatapult
  (params (AxisValue :type Float%20%28single-precision%29))
  (bind _returnvalue (/ AxisValue 2.5))
  (bind _catapult_spoon (Variables|Default|GetCatapult_Spoon))
  (bind _catapult_spoon_2 (Variables|Default|GetCatapult_Spoon))
  (bind _relativerotation (Variables|/Script/Engine.SceneComponent|GetRelativeRotation _catapult_spoon))
  (bind _relativerotation_2 (Variables|/Script/Engine.SceneComponent|GetRelativeRotation _catapult_spoon_2))
  (bind _returnvalue_2 (+ (.roll _relativerotation) _returnvalue))
  (bind _returnvalue_3 (Math|Float|Clamp(Float) _returnvalue_2 0.0 3e+01))
  (Variables|Default|SetSpoonAngle _returnvalue_3)
  (Transformation|SetRelativeRotation _catapult_spoon (Math|Rotator|MakeRotator _returnvalue_3 (.pitch _relativerotation_2) (.yaw _relativerotation_2)) false false))

(event Input|AxisEvents|InputAxisSteer
  (params (AxisValue :type Float%20%28single-precision%29))
  (Variables|Default|SetCurrentSteeringAngle (Math|Interpolation|FInterpTo (Variables|Default|GetCurrentSteeringAngle) (* (* AxisValue (Variables|Default|GetSteer%20Axis)) (Variables|Default|GetMaxSteeringAngle)) (Utilities|Time|GetWorldDeltaSeconds) 4.0))
  (Class|Actor|AddActorWorldRotation (Math|Rotator|MakeRotator 0.0 0.0 (* (Variables|Default|GetCurrentSpeed) (Variables|Default|GetCurrentSteeringAngle) (Variables|Default|GetSpeedToRotationFactor) (Utilities|Time|GetWorldDeltaSeconds)))))

(fn ConstructionScript)

(fn CheckAngleOfSpoon
  (bind _output_get (Variables|Default|SetSpoonAngle%20%28I%29 (Math|Float|Truncate (Variables|Default|GetSpoonAngle))))
  (if (== _output_get 0)
    (Variables|Default|SetVelocity%20Z 3e+03)
    (elif (and (> _output_get 0) (<= _output_get 10))
      (Variables|Default|SetVelocity%20Z 2.5e+03)
      (elif (and (> _output_get 10) (<= _output_get 18))
        (Variables|Default|SetVelocity%20Z 2e+03)
        (elif (and (> _output_get 18) (<= _output_get 25))
          (Variables|Default|SetVelocity%20Z 1.5e+03)
          (elif (and (> _output_get 25) (<= _output_get 30))
            (Variables|Default|SetVelocity%20Z 1e+03)))))))