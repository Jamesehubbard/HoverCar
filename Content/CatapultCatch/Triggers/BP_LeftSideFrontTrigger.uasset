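; BP_LeftSideFrontTrigger is a Catapult Catch scoring trigger that awards the right side two points when a tagged projectile enters it.
; A DoOnce gates each hit, writing the score directly into the first W_Score widget found.
; After a delay it destroys the projectile, resets the gate, then spawns a pickupable projectile at the captured mesh position with a fixed height.
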(event Custom|Reset
  (bind _as_projectile_bp (Variables|Default|GetAs%20Projectile%20BP))
  (Utilities|FlowControl|DoOnce false) ; enters at Reset
)

(event Collision|EventActorBeginOverlap
  (params (OtherActor :type Actor%20Object%20Reference))
  (if (Actor|ActorHasTag OtherActor "Projectile")
    (bind _asprojectile_bp (Utilities|Casting|CastToProjectile_BP OtherActor))
    (Variables|Default|SetAs%20Projectile%20BP _asprojectile_bp)
    (Utilities|FlowControl|DoOnce false
      (:Completed
        (Utilities|FlowControl|Sequence
          (:then_0
            (bind _foundwidgets (Widget|GetAllWidgetsOfClass "/Game/CatapultCatch/UI/W_Score.W_Score_C" true))
            (bind _asw_score (Utilities|Casting|CastToW_Score (Utilities|Array|Get(acopy) _foundwidgets)))
            (Variables|/Game/CatapultCatch/UI/W_Score.W_Score_C|SetRightSideScore _asw_score (+ (Variables|/Game/CatapultCatch/UI/W_Score.W_Score_C|GetRightSideScore _asw_score) 2)))
          (:then_1
            (Utilities|FlowControl|Delay 5.0)
            (Utilities|IsValid (Variables|Default|GetAs%20Projectile%20BP)
              (:Is%20Valid
                (Variables|Default|SetProjectile%20Location (Transformation|GetWorldTransform (Variables|/Game/CatapultCatch/Blueprints/Projectile_BP.Projectile_BP_C|GetMesh (Variables|Default|GetAs%20Projectile%20BP))))
                (Actor|DestroyActor (Variables|Default|GetAs%20Projectile%20BP))
                (CallFunction|Reset)
                (Utilities|FlowControl|Delay 1.0)
                (Game|SpawnActorfromClass "/Game/CatapultCatch/Blueprints/PickupableProjectile_BP.PickupableProjectile_BP_C" (Math|Transform|MakeTransform (Math|Vector|MakeVector (.x (.location (Variables|Default|GetProjectile%20Location))) (.y (.location (Variables|Default|GetProjectile%20Location))) 588.0) (.rotation (Variables|Default|GetProjectile%20Location)) (.scale (Variables|Default|GetProjectile%20Location))) "Undefined" "MultiplyWithRoot" 0 0)))))))))

(fn ConstructionScript)