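; Hover component that caches its owner's root primitive on BeginPlay, keeping it only if it simulates physics.
; Its spring-damper suspension logic is disconnected from the empty Tick, so no hover force is applied.
; That unwired logic traces down the component's local axis, derives force from compression and its rate of change, and applies it at the component's location.
; It also draws the trace and prints hit distance for debugging.
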(event EventBeginPlay
  (bind _asprimitive_component (Utilities|Casting|CastToPrimitiveComponent (Variables|/Script/Engine.Actor|GetRootComponent (Components|GetOwner))))
  (bind _output_get (Variables|Default|SetBody%20Reference _asprimitive_component))
  (if (not (Physics|IsSimulatingPhysics _output_get "None"))
    (Variables|Default|SetBody%20Reference 0)))

(event EventTick
  (params (DeltaSeconds :type Float%20%28single-precision%29)))