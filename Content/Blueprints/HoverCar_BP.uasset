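; Player-controlled hover car pawn built on a physics Cube held up by four hover components, each initialized with that Cube on BeginPlay.
; Enhanced Input drives it, with move and jump applying forces to the Cube.
; Swivel sets the Cube's relative yaw directly within clamped limits, rather than applying torque.
; Hover height input steps all four components' trace lengths up or down within a clamped range.
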(event Input|EnhancedActionEvents|EnhancedInputActionJump_IA
  (params (ActionValue :type Boolean) (ElapsedSeconds :type Float%20%28double-precision%29) (TriggeredSeconds :type Float%20%28double-precision%29) (InputAction :type Input%20Action%20Object%20Reference :default "/Game/Input/Jump_IA.Jump_IA"))
  (Physics|AddForce (Variables|Default|GetCube) "0.000000,0.000000,1000000.000000" "None" false))

(event Input|EnhancedActionEvents|EnhancedInputActionMove_IA
  (params (ActionValue :type Vector%202D%20Structure) (ElapsedSeconds :type Float%20%28double-precision%29) (TriggeredSeconds :type Float%20%28double-precision%29) (InputAction :type Input%20Action%20Object%20Reference :default "/Game/Input/Move_IA.Move_IA"))
  (Physics|AddForce (Variables|Default|GetCube) (* (* (Math|Vector|GetForwardVector (Variables|Default|GetCube)) 5e+05) (.y ActionValue)) "None" false)
  (Physics|AddForce (Variables|Default|GetCube) (* (* (Math|Vector|GetRightVector (Variables|Default|GetCube)) 5e+05) (.x ActionValue)) "None" false))

(event Input|EnhancedActionEvents|EnhancedInputActionSwivel_IA
  (params (ActionValue :type Vector%202D%20Structure) (ElapsedSeconds :type Float%20%28double-precision%29) (TriggeredSeconds :type Float%20%28double-precision%29) (InputAction :type Input%20Action%20Object%20Reference :default "/Game/Input/Swivel_IA.Swivel_IA"))
  (:Triggered
    (Transformation|SetRelativeRotation (Variables|Default|GetCube) (Math|Rotator|MakeRotator 0.0 0.0 (Math|Float|Clamp(Float) (+ (.yaw (Variables|/Script/Engine.SceneComponent|GetRelativeRotation (Variables|Default|GetCube))) (* (.x ActionValue) 1e+01)) -9e+01 9e+01)) false false)))

(event Input|EnhancedActionEvents|EnhancedInputActionHoverHeight_IA
  (params (ActionValue :type Vector%202D%20Structure) (ElapsedSeconds :type Float%20%28double-precision%29) (TriggeredSeconds :type Float%20%28double-precision%29) (InputAction :type Input%20Action%20Object%20Reference :default "/Game/Input/HoverHeight_IA.HoverHeight_IA"))
  (if (> (.x ActionValue) 0.0)
    (Variables|/Game/Blueprints/HoverComponent.HoverComponent_C|SetTraceLength (Variables|Default|GetHoverComponent1) (Math|Float|Clamp(Float) (+ (Variables|/Game/Blueprints/HoverComponent.HoverComponent_C|GetTraceLength (Variables|Default|GetHoverComponent1)) 1e+01) 4e+01 2e+02))
    (Variables|/Game/Blueprints/HoverComponent.HoverComponent_C|SetTraceLength (Variables|Default|GetHoverComponent2) (Math|Float|Clamp(Float) (+ (Variables|/Game/Blueprints/HoverComponent.HoverComponent_C|GetTraceLength (Variables|Default|GetHoverComponent2)) 1e+01) 4e+01 2e+02))
    (Variables|/Game/Blueprints/HoverComponent.HoverComponent_C|SetTraceLength (Variables|Default|GetHoverComponent3) (Math|Float|Clamp(Float) (+ (Variables|/Game/Blueprints/HoverComponent.HoverComponent_C|GetTraceLength (Variables|Default|GetHoverComponent3)) 1e+01) 4e+01 2e+02))
    (Variables|/Game/Blueprints/HoverComponent.HoverComponent_C|SetTraceLength (Variables|Default|GetHoverComponent4) (Math|Float|Clamp(Float) (+ (Variables|/Game/Blueprints/HoverComponent.HoverComponent_C|GetTraceLength (Variables|Default|GetHoverComponent4)) 1e+01) 4e+01 2e+02))
    (elif (< (.x ActionValue) 0.0)
      (Variables|/Game/Blueprints/HoverComponent.HoverComponent_C|SetTraceLength (Variables|Default|GetHoverComponent1) (Math|Float|Clamp(Float) (- (Variables|/Game/Blueprints/HoverComponent.HoverComponent_C|GetTraceLength (Variables|Default|GetHoverComponent1)) 1e+01) 4e+01 2e+02))
      (Variables|/Game/Blueprints/HoverComponent.HoverComponent_C|SetTraceLength (Variables|Default|GetHoverComponent2) (Math|Float|Clamp(Float) (- (Variables|/Game/Blueprints/HoverComponent.HoverComponent_C|GetTraceLength (Variables|Default|GetHoverComponent2)) 1e+01) 4e+01 2e+02))
      (Variables|/Game/Blueprints/HoverComponent.HoverComponent_C|SetTraceLength (Variables|Default|GetHoverComponent3) (Math|Float|Clamp(Float) (- (Variables|/Game/Blueprints/HoverComponent.HoverComponent_C|GetTraceLength (Variables|Default|GetHoverComponent3)) 1e+01) 4e+01 2e+02))
      (Variables|/Game/Blueprints/HoverComponent.HoverComponent_C|SetTraceLength (Variables|Default|GetHoverComponent4) (Math|Float|Clamp(Float) (- (Variables|/Game/Blueprints/HoverComponent.HoverComponent_C|GetTraceLength (Variables|Default|GetHoverComponent4)) 1e+01) 4e+01 2e+02)))))

(event EventBeginPlay
  (Variables|/Script/Engine.PlayerController|SetbShowMouseCursor (Game|GetPlayerController 0) true)
  (Utilities|FlowControl|Sequence
    (:then_0
      (Default|InitComponent (Variables|Default|GetHoverComponent1) (Variables|Default|GetCube))
      (Default|InitComponent (Variables|Default|GetHoverComponent2) (Variables|Default|GetCube))
      (Default|InitComponent (Variables|Default|GetHoverComponent3) (Variables|Default|GetCube))
      (Default|InitComponent (Variables|Default|GetHoverComponent4) (Variables|Default|GetCube)))
    (:then_1
      (bind _asplayer_controller (Utilities|Casting|CastToPlayerController (Pawn|GetController)))
      (Utilities|IsValid (PlayerController|LocalPlayerSubsystems|GetEnhancedInputLocalPlayerSubsystem _asplayer_controller)
        (:Is%20Valid
          (Input|AddMappingContext (PlayerController|LocalPlayerSubsystems|GetEnhancedInputLocalPlayerSubsystem _asplayer_controller) "/Game/Input/InputMappingContext.InputMappingContext" 0 "(bIgnoreAllPressedKeysUntilRelease=True,bForceImmediately=False,bNotifyUserSettings=False)"))))))

(fn ConstructionScript)