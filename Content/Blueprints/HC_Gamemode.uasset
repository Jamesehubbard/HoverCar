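; Hover car game mode whose StartGame event builds a random track and spawns local players.
; Tiles chain through each piece's attach point between start and end tiles, with a random trap tile inserted whenever the straight counter exceeds four.
; Each PlayerStart gets a possessed hover car and input mapping; player zero's car is offset along X by a head start.
; AddTurnTile exists but is not called here.
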(event Custom|StartGame
  (Utilities|FlowControl|Sequence
    (:then_0
      (bind _returnvalue (Game|SpawnActorfromClass "/Game/Blueprints/Track/TileTrack_StartTile.TileTrack_StartTile_C" (Variables|Default|GetNext%20Spawn%20Point) "Undefined" "MultiplyWithRoot" 0 0))
      (bind _astile_track_start_tile (Utilities|Casting|CastToTileTrack_StartTile _returnvalue))
      (bind _returnvalue_2 (Default|GetAttachPoint _astile_track_start_tile))
      (Variables|Default|SetNext%20Spawn%20Point _returnvalue_2)
      (Variables|Default|SetCurrentStraights (+ (Variables|Default|GetCurrentStraights) 1))
      (for _index (range 0 (- (Variables|Default|GetNumber%20Of%20Tiles) 2))
        (CallFunction|AddTrackTile))
      (Game|SpawnActorfromClass "/Game/Blueprints/Track/TileTrack_EndTile.TileTrack_EndTile_C" (Variables|Default|GetNext%20Spawn%20Point) "Undefined" "MultiplyWithRoot" 0 0)
      (Variables|Default|SetCurrentStraights (+ (Variables|Default|GetCurrentStraights) 1)))
    (:then_1
      (bind _outactors (Actor|GetAllActorsOfClass "/Script/Engine.PlayerStart"))
      (for (_array_element _array_index) _outactors
        (bind _output_get (Variables|Default|SetArray%20Index _array_index))
        (bind _returnvalue_3 (Class|GameplayStatics|CreatePlayer _output_get))
        (if (> (Variables|Default|GetArray%20Index) 0)
          (Input|AddMappingContext (PlayerController|LocalPlayerSubsystems|GetEnhancedInputLocalPlayerSubsystem _returnvalue_3) "/Game/Input/InputMappingContext.InputMappingContext" 0 "(bIgnoreAllPressedKeysUntilRelease=True,bForceImmediately=False,bNotifyUserSettings=False)")
          (bind _returnvalue_4 (Game|SpawnActorfromClass "/Game/Blueprints/HoverCar_BP.HoverCar_BP_C" (Transformation|GetActorTransform _array_element) "Undefined" "MultiplyWithRoot" 0 0))
          (bind _output_get_2 (Variables|Default|SetPlayer1 _returnvalue_4))
          (Variables|/Game/Blueprints/HoverCar_BP.HoverCar_BP_C|SetChaser _output_get_2 false)
          (Pawn|Possess (Game|GetPlayerController (Variables|Default|GetArray%20Index)) _returnvalue_4)
          (else
            (Input|AddMappingContext (PlayerController|LocalPlayerSubsystems|GetEnhancedInputLocalPlayerSubsystem (Game|GetPlayerController 0)) "/Game/Input/InputMappingContext.InputMappingContext" 0 "(bIgnoreAllPressedKeysUntilRelease=True,bForceImmediately=False,bNotifyUserSettings=False)")
            (bind _returnvalue_5 (Game|SpawnActorfromClass "/Game/Blueprints/HoverCar_BP.HoverCar_BP_C" (Transformation|GetActorTransform _array_element) "Undefined" "MultiplyWithRoot" 0 0))
            (Pawn|Possess (Game|GetPlayerController 0) _returnvalue_5)
            (Transformation|SetActorLocation _returnvalue_5 (+ (Transformation|GetActorLocation _returnvalue_5) (Math|Vector|MakeVector (Variables|Default|GetHeadStartNum) 0.0 0.0)) false false)))))))

(event EventBeginPlay)

(fn ConstructionScript)

(fn AddTrackTile
  (if (> (Variables|Default|GetCurrentStraights) 4)
    (bind _returnvalue (Game|SpawnActorfromClass (.OutItem (Utilities|Array|Random (Variables|Default|GetTrapTiles))) (Variables|Default|GetNext%20Spawn%20Point) "Undefined" "MultiplyWithRoot" 0 0))
    (bind _astrap_tile_bp (Utilities|Casting|CastToTrapTile_BP _returnvalue))
    (bind _returnvalue_2 (Default|GetAttachPoint _astrap_tile_bp))
    (Variables|Default|SetNext%20Spawn%20Point _returnvalue_2)
    (Variables|Default|SetCurrentStraights 0)
    (else
      (bind _returnvalue_3 (Game|SpawnActorfromClass (.OutItem (Utilities|Array|Random (Variables|Default|GetTrackTiles))) (Variables|Default|GetNext%20Spawn%20Point) "Undefined" "MultiplyWithRoot" 0 0))
      (bind _asfloor_bp (Utilities|Casting|CastToFloor_BP _returnvalue_3))
      (bind _returnvalue_4 (Default|GetAttachPoint _asfloor_bp))
      (Variables|Default|SetNext%20Spawn%20Point _returnvalue_4)
      (Variables|Default|SetCurrentStraights (+ (Variables|Default|GetCurrentStraights) 1)))))

(fn AddTurnTile
  (bind _returnvalue (Game|SpawnActorfromClass (Utilities|Array|Get(acopy) (Variables|Default|GetTurn%20Tiles)) (Variables|Default|GetNext%20Spawn%20Point) "Undefined" "MultiplyWithRoot" 0 0))
  (bind _asfloor_bp (Utilities|Casting|CastToFloor_BP _returnvalue))
  (bind _returnvalue_2 (Default|GetAttachPoint _asfloor_bp))
  (Variables|Default|SetNext%20Spawn%20Point _returnvalue_2)
  (Variables|Default|SetCurrentStraights 0))

(fn GetNumTiles
  (return (Variables|Default|GetNumber%20Of%20Tiles)))

(fn SetNumTiles
  (params (Num%20of%20Tiles :type Integer))
  (Variables|Default|SetNumber%20Of%20Tiles Num%20of%20Tiles)
  (return))