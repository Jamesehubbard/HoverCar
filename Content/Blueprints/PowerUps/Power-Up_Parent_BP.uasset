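; Base power-up Blueprint that lets a HoverCar_BP pick it up on box overlap.
; Overlap with the first HoverCar found destroys the actor, then calls PowerupPickedUp.
; Overlap with the second HoverCar only sets the static mesh to NoCollision, leaving the pickup in place.
; PowerupPickedUp and PowerUpActivated are empty events, and cars are told apart by their GetAllActorsOfClass index.
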(event OnComponentBeginOverlap(Box)
  (params (OverlappedComponent :type Primitive%20Component%20Object%20Reference) (OtherActor :type Actor%20Object%20Reference) (OtherComp :type Primitive%20Component%20Object%20Reference) (OtherBodyIndex :type Integer) (bFromSweep :type Boolean) (SweepResult :type Hit%20Result%20Structure%20%28by%20ref%29))
  (Utilities|FlowControl|Sequence
    (:then_0
      (bind _outactors (Actor|GetAllActorsOfClass "/Game/Blueprints/HoverCar_BP.HoverCar_BP_C"))
      (if (== (Utilities|Array|Get(acopy) _outactors) OtherActor)
        (Actor|DestroyActor)
        (CallFunction|PowerupPickedUp)))
    (:then_1
      (bind _outactors_2 (Actor|GetAllActorsOfClass "/Game/Blueprints/HoverCar_BP.HoverCar_BP_C"))
      (if (== (Utilities|Array|Get(acopy) _outactors_2 1) OtherActor)
        (Collision|SetCollisionProfileName (Variables|Default|GetStaticMesh) "NoCollision" true :!class /Script/Engine.PrimitiveComponent)))))

(event Custom|PowerUp%20Activated)

(event Custom|Powerup%20Picked%20Up)

(fn ConstructionScript)