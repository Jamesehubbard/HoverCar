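; Reverse power-up for the hover car game, built on a parent power-up that handles overlap.
; On pickup, it sets ReverseActivatable on the first HoverCar_BP found in the level.
; On activation, it sets that flag to true again and calls ReverseEffect on the second car found.
; Cars are picked by fixed GetAllActorsOfClass index, regardless of which one overlapped the power-up.
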(event EventPowerupPickedUp
  (bind _outactors (Actor|GetAllActorsOfClass "/Game/Blueprints/HoverCar_BP.HoverCar_BP_C"))
  (bind _ashover_car_bp (Utilities|Casting|CastToHoverCar_BP (Utilities|Array|Get(acopy) _outactors)))
  (Variables|/Game/Blueprints/HoverCar_BP.HoverCar_BP_C|SetReverse%20Activatable _ashover_car_bp true))

(event Collision|EventActorBeginOverlap
  (params (OtherActor :type Actor%20Object%20Reference))
  (|CallParentFunction OtherActor))

(event EventPowerUpActivated
  (bind _outactors (Actor|GetAllActorsOfClass "/Game/Blueprints/HoverCar_BP.HoverCar_BP_C"))
  (bind _ashover_car_bp (Utilities|Casting|CastToHoverCar_BP (Utilities|Array|Get(acopy) _outactors)))
  (Variables|/Game/Blueprints/HoverCar_BP.HoverCar_BP_C|SetReverse%20Activatable _ashover_car_bp true)
  (bind _outactors_2 (Actor|GetAllActorsOfClass "/Game/Blueprints/HoverCar_BP.HoverCar_BP_C"))
  (bind _ashover_car_bp_2 (Utilities|Casting|CastToHoverCar_BP (Utilities|Array|Get(acopy) _outactors_2 1)))
  (Default|ReverseEffect _ashover_car_bp_2))

(fn ConstructionScript
  (|CallParentFunction))