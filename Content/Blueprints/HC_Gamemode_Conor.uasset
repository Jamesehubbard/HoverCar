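; Game mode for a local multiplayer hover car chase on an endless, randomly tiled track.
; StartGame creates a player per PlayerStart, adds input mapping, possesses a spawned car and offsets it by chaser role or head start.
; ExtendFloor chains random tiles at each piece's attach point, forces turns after straight runs and removes old tiles.
; The initial track-building nodes in the event graph are disconnected.
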(event Custom|StartGame
  (Utilities|FlowControl|Sequence
    (:then_1
      (bind _outactors (Actor|GetAllActorsOfClass "/Script/Engine.PlayerStart"))
      (for (_array_element _array_index) _outactors
        (bind _output_get (Variables|Default|SetArray%20Index _array_index))
        (bind _returnvalue (Class|GameplayStatics|CreatePlayer _output_get))
        (if (> (Variables|Default|GetArray%20Index) 0)
          (Input|AddMappingContext (PlayerController|LocalPlayerSubsystems|GetEnhancedInputLocalPlayerSubsystem _returnvalue) "/Game/Input/InputMappingContext.InputMappingContext" 0 "(bIgnoreAllPressedKeysUntilRelease=True,bForceImmediately=False,bNotifyUserSettings=False)")
          (bind _returnvalue_2 (Game|SpawnActorfromClass "/Game/Blueprints/HoverCar_BP.HoverCar_BP_C" (Transformation|GetActorTransform _array_element) "Undefined" "MultiplyWithRoot" 0 0))
          (bind _output_get_2 (Variables|Default|SetPlayer1 _returnvalue_2))
          (Pawn|Possess (Game|GetPlayerController (Variables|Default|GetArray%20Index)) _output_get_2)
          (if (Variables|Default|GetIsP1Chaser)
            (Transformation|SetActorLocation (Variables|Default|GetPlayer1) (+ (Transformation|GetActorLocation) (Math|Vector|MakeVector 6e+02 0.0 0.0)) false false)
            (else
              (Transformation|SetActorLocation (Variables|Default|GetPlayer1) (+ (Transformation|GetActorLocation (Variables|Default|GetPlayer1)) (Math|Vector|MakeVector (Variables|Default|GetHeadStartNum) 0.0 0.0)) false false)))
          (else
            (Input|AddMappingContext (PlayerController|LocalPlayerSubsystems|GetEnhancedInputLocalPlayerSubsystem (Game|GetPlayerController 0)) "/Game/Input/InputMappingContext.InputMappingContext" 0 "(bIgnoreAllPressedKeysUntilRelease=True,bForceImmediately=False,bNotifyUserSettings=False)")
            (bind _returnvalue_3 (Game|SpawnActorfromClass "/Game/Blueprints/HoverCar_BP.HoverCar_BP_C" (Transformation|GetActorTransform _array_element) "Undefined" "MultiplyWithRoot" 0 0))
            (bind _output_get_3 (Variables|Default|SetPlayer2 _returnvalue_3))
            (Pawn|Possess (Game|GetPlayerController 0) _output_get_3)
            (if (Variables|Default|GetIsP1Chaser)
              (Transformation|SetActorLocation (Variables|Default|GetPlayer2) (+ (Transformation|GetActorLocation) (Math|Vector|MakeVector -6e+02 0.0 0.0)) false false)
              (else
                (Transformation|SetActorLocation (Variables|Default|GetPlayer2) (+ (Transformation|GetActorLocation (Variables|Default|GetPlayer2)) (Math|Vector|MakeVector (Variables|Default|GetHeadStartNum) 0.0 0.0)) false false)))))))))

(event EventBeginPlay)

(fn ConstructionScript)

(fn AddFloor
  (if (> (Variables|Default|GetCurrentStraights) 7)
    (CallFunction|AddFloorTurn)
    (else
      (bind _returnvalue (Game|SpawnActorfromClass (Utilities|Array|Get(acopy) (Variables|Default|GetFloor%20Tiles) (Math|Random|RandomIntegerinRange 0 (Utilities|Array|LastIndex (Variables|Default|GetFloor%20Tiles)))) (Variables|Default|GetNext%20Spawn%20Point) "Undefined" "MultiplyWithRoot" 0 0))
      (bind _asfloor_bp (Utilities|Casting|CastToFloor_BP _returnvalue))
      (bind _returnvalue_2 (Default|GetAttachPoint _asfloor_bp))
      (Variables|Default|SetNext%20Spawn%20Point _returnvalue_2)
      (Variables|Default|SetCurrentStraights (+ (Variables|Default|GetCurrentStraights) 1))
      (Utilities|Array|Add (Variables|Default|GetFloors) _asfloor_bp))))

(fn AddFloorTurn
  (bind _returnvalue (Game|SpawnActorfromClass (Utilities|Array|Get(acopy) (Variables|Default|GetFloor%20Turns) (Math|Random|RandomIntegerinRange 0 (Utilities|Array|LastIndex (Variables|Default|GetFloor%20Turns)))) (Variables|Default|GetNext%20Spawn%20Point) "Undefined" "MultiplyWithRoot" 0 0))
  (bind _asfloor_bp (Utilities|Casting|CastToFloor_BP _returnvalue))
  (bind _returnvalue_2 (Default|GetAttachPoint _asfloor_bp))
  (Variables|Default|SetNext%20Spawn%20Point _returnvalue_2)
  (Variables|Default|SetCurrentStraights 0)
  (Utilities|Array|Add (Variables|Default|GetFloors) _asfloor_bp))

(fn ExtendFloor
  (bind _floors (Variables|Default|GetFloors))
  (bind _output (Utilities|Array|Get(acopy) _floors))
  (CallFunction|AddFloor)
  (if (> (Utilities|Array|Length (Variables|Default|GetFloors)) (+ (Variables|Default|GetNumber%20Of%20Tiles) 2))
    (Actor|DestroyActor _output)
    (Utilities|Array|RemoveItem _floors _output)))

(fn GetNumTiles
  (return (Variables|Default|GetNumber%20Of%20Tiles)))

(fn SetNumTiles
  (params (Num%20of%20Tiles :type Integer))
  (Variables|Default|SetNumber%20Of%20Tiles Num%20of%20Tiles)
  (return))