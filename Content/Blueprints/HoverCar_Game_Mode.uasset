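; Game mode that sets up local multiplayer hover car play, one player per PlayerStart in the level.
; On BeginPlay it loops over all PlayerStarts, creating a local player for each index and adding the input mapping context to that player's Enhanced Input subsystem.
; It spawns a NewHoverCar_BP at each start and has that player's controller possess it, with index 0 using the existing first controller.
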(event EventBeginPlay
  (bind _outactors (Actor|GetAllActorsOfClass "/Script/Engine.PlayerStart"))
  (for (_array_element _array_index) _outactors
    (bind _output_get (Variables|Default|SetArray%20Index _array_index))
    (bind _returnvalue (Class|GameplayStatics|CreatePlayer _output_get))
    (if (> (Variables|Default|GetArray%20Index) 0)
      (Input|AddMappingContext (PlayerController|LocalPlayerSubsystems|GetEnhancedInputLocalPlayerSubsystem _returnvalue) "/Game/Input/InputMappingContext.InputMappingContext" 0 "(bIgnoreAllPressedKeysUntilRelease=True,bForceImmediately=False,bNotifyUserSettings=False)")
      (bind _returnvalue_2 (Game|SpawnActorfromClass "/Game/Blueprints/NewHoverCar_BP.NewHoverCar_BP_C" (Transformation|GetActorTransform _array_element) "Undefined" "MultiplyWithRoot" 0 0))
      (Pawn|Possess (Game|GetPlayerController (Variables|Default|GetArray%20Index)) _returnvalue_2)
      (else
        (Input|AddMappingContext (PlayerController|LocalPlayerSubsystems|GetEnhancedInputLocalPlayerSubsystem (Game|GetPlayerController 0)) "/Game/Input/InputMappingContext.InputMappingContext" 0 "(bIgnoreAllPressedKeysUntilRelease=True,bForceImmediately=False,bNotifyUserSettings=False)")
        (bind _returnvalue_3 (Game|SpawnActorfromClass "/Game/Blueprints/NewHoverCar_BP.NewHoverCar_BP_C" (Transformation|GetActorTransform _array_element) "Undefined" "MultiplyWithRoot" 0 0))
        (Pawn|Possess (Game|GetPlayerController 0) _returnvalue_3)))))

(fn ConstructionScript)