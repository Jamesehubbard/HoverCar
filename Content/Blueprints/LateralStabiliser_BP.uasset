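; Actor component that stabilises its owning physics body against sideways sliding.
; On BeginPlay it caches the owner's root as a primitive component.
; Each tick it projects linear velocity onto the body's right vector and applies an opposing force along that axis, scaled by SpeedToForceFactor.
; The force is mass-dependent and not scaled by delta time, acting as linear lateral drag.
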(event EventBeginPlay
  (bind _asprimitive_component (Utilities|Casting|CastToPrimitiveComponent (Variables|/Script/Engine.Actor|GetRootComponent (Components|GetOwner))))
  (Variables|Default|SetBody%20Reference _asprimitive_component))

(event EventTick
  (params (DeltaSeconds :type Float%20%28single-precision%29))
  (bind _body_reference (Variables|Default|GetBody%20Reference)
    (:then
      (bind _returnvalue (Physics|GetPhysicsLinearVelocity _body_reference "None"))
      (Physics|AddForce (Variables|Default|GetBody%20Reference) (* (* (Math|Vector|DotProduct _returnvalue (Math|Vector|GetRightVector _body_reference)) -1.0 (Variables|Default|GetSpeedToForceFactor)) (Math|Vector|GetRightVector (Variables|Default|GetBody%20Reference))) "None" false))
    (:else)))