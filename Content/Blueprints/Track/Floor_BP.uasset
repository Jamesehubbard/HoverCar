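; Track floor segment that randomizes its power-up and flanking buildings on BeginPlay, exposing an Arrow transform through GetAttachPoint.
; A coin flip decides whether a random power-up spawns at one of two scene points; only that branch also randomizes the four building stacks' meshes.
; Chained random branches hide top or middle pieces to vary heights, with some outcomes ending the chain early.
; Bottom pieces get random Y positions within per-side ranges.
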(event EventBeginPlay
  (bind _building_square_r_02_bottom (Variables|Default|GetBuilding_Square_R_02_Bottom))
  (bind _building_square_l_01_bottom (Variables|Default|GetBuilding_Square_L_01_Bottom))
  (bind _building_square_l_02_bottom (Variables|Default|GetBuilding_Square_L_02_Bottom))
  (bind _building_square_r_01_bottom (Variables|Default|GetBuilding_Square_R_01_Bottom))
  (bind _returnvalue (Transformation|GetWorldLocation _building_square_r_02_bottom))
  (bind _returnvalue_2 (Transformation|GetWorldLocation _building_square_l_01_bottom))
  (bind _returnvalue_3 (Transformation|GetWorldLocation _building_square_l_02_bottom))
  (bind _returnvalue_4 (Transformation|GetWorldLocation _building_square_r_01_bottom))
  (Utilities|FlowControl|Sequence
    (:then_0
      (switch int (Math|Random|RandomIntegerinRange 0 1)
        (:0
          (Variables|Default|SetPowerUp%20Location (Transformation|GetWorldTransform (Variables|Default|GetScene))))
        (:1
          (Variables|Default|SetPowerUp%20Location (Transformation|GetWorldTransform (Variables|Default|GetScene1)))))
      (switch int (Math|Random|RandomIntegerinRange 0 1)
        (:0
          (Game|SpawnActorfromClass (.OutItem (Utilities|Array|Random (Variables|Default|GetPowerUps))) (Variables|Default|GetPowerUp%20Location) "Undefined" "MultiplyWithRoot" 0 0)
          (bind _output_get (Variables|Default|SetBuilding%20Square%20L%2001%20Mesh (.OutItem (Utilities|Array|Random (Variables|Default|GetBuilding%20Meshes)))))
          (Components|StaticMesh|SetStaticMesh (Variables|Default|GetBuilding_Square_L_01_Bottom) _output_get)
          (Components|StaticMesh|SetStaticMesh (Variables|Default|GetBuilding_Square_L_01_Top) (Variables|Default|GetBuilding%20Square%20L%2001%20Mesh))
          (Components|StaticMesh|SetStaticMesh (Variables|Default|GetBuilding_Square_L_01_Middle) (Variables|Default|GetBuilding%20Square%20L%2001%20Mesh))
          (bind _output_get_2 (Variables|Default|SetBuilding%20Square%20L%2002%20Mesh (.OutItem (Utilities|Array|Random (Variables|Default|GetBuilding%20Meshes)))))
          (Components|StaticMesh|SetStaticMesh (Variables|Default|GetBuilding_Square_L_02_Bottom) _output_get_2)
          (Components|StaticMesh|SetStaticMesh (Variables|Default|GetBuilding_Square_L_02_Middle) (Variables|Default|GetBuilding%20Square%20L%2002%20Mesh))
          (Components|StaticMesh|SetStaticMesh (Variables|Default|GetBuilding_Square_L_02_Top) (Variables|Default|GetBuilding%20Square%20L%2002%20Mesh))
          (bind _output_get_3 (Variables|Default|SetBuilding%20Square%20R%2001%20Mesh (.OutItem (Utilities|Array|Random (Variables|Default|GetBuilding%20Meshes)))))
          (Components|StaticMesh|SetStaticMesh (Variables|Default|GetBuilding_Square_R_01_Bottom) _output_get_3)
          (Components|StaticMesh|SetStaticMesh (Variables|Default|GetBuilding_Square_R_01_Middle) (Variables|Default|GetBuilding%20Square%20R%2001%20Mesh))
          (Components|StaticMesh|SetStaticMesh (Variables|Default|GetBuilding_Square_R_01_Top) (Variables|Default|GetBuilding%20Square%20R%2001%20Mesh))
          (bind _output_get_4 (Variables|Default|SetBuilding%20Square%20R%2002%20Mesh (.OutItem (Utilities|Array|Random (Variables|Default|GetBuilding%20Meshes)))))
          (Components|StaticMesh|SetStaticMesh (Variables|Default|GetBuilding_Square_R_02_Bottom) _output_get_4)
          (Components|StaticMesh|SetStaticMesh (Variables|Default|GetBuilding_Square_R_02_Middle) (Variables|Default|GetBuilding%20Square%20R%2002%20Mesh))
          (Components|StaticMesh|SetStaticMesh (Variables|Default|GetBuilding_Square_R_02_Top) (Variables|Default|GetBuilding%20Square%20R%2002%20Mesh)))))
    (:then_1
      (switch int (Math|Random|RandomIntegerinRange 0 2)
        (:0
          (switch int (Math|Random|RandomIntegerinRange 0 1) :!label _label
            (:0
              (switch int (Math|Random|RandomIntegerinRange 0 2) :!label _label_2
                (:0
                  (switch int (Math|Random|RandomIntegerinRange 0 2) :!label _label_3
                    (:1
                      (Development|SetHiddeninGame (Variables|Default|GetBuilding_Square_L_02_Top) true false))
                    (:2
                      (Development|SetHiddeninGame (Variables|Default|GetBuilding_Square_L_02_Top) true false)
                      (Development|SetHiddeninGame (Variables|Default|GetBuilding_Square_L_02_Middle) true false))))
                (:1
                  (Development|SetHiddeninGame (Variables|Default|GetBuilding_Square_R_02_Top) true false)
                  (goto _label_3))
                (:2
                  (Development|SetHiddeninGame (Variables|Default|GetBuilding_Square_R_02_Top) true false)
                  (Development|SetHiddeninGame (Variables|Default|GetBuilding_Square_R_02_Middle) true false))))
            (:1
              (Development|SetHiddeninGame (Variables|Default|GetBuilding_Square_L_01_Top) true false)
              (goto _label_2))
            (:2
              (Development|SetHiddeninGame (Variables|Default|GetBuilding_Square_L_01_Top) true false)
              (Development|SetHiddeninGame (Variables|Default|GetBuilding_Square_L_01_Middle) true false))))
        (:1
          (Development|SetHiddeninGame (Variables|Default|GetBuilding_Square_R_01_Top) true false)
          (goto _label))
        (:2
          (Development|SetHiddeninGame (Variables|Default|GetBuilding_Square_R_01_Top) true false)
          (Development|SetHiddeninGame (Variables|Default|GetBuilding_Square_R_01_Middle) true false))))
    (:then_2
      (Transformation|SetWorldLocation _building_square_l_01_bottom (Math|Vector|MakeVector (.x _returnvalue_2) (Math|Random|RandomFloatinRange -1e+03 0.0) (.z _returnvalue_2)) false false)
      (Transformation|SetWorldLocation _building_square_l_02_bottom (Math|Vector|MakeVector (.x _returnvalue_3) (Math|Random|RandomFloatinRange -1e+03 0.0) (.z _returnvalue_3)) false false)
      (Transformation|SetWorldLocation _building_square_r_01_bottom (Math|Vector|MakeVector (.x _returnvalue_4) (Math|Random|RandomFloatinRange 3e+03 4e+03) (.z _returnvalue_4)) false false)
      (Transformation|SetWorldLocation _building_square_r_02_bottom (Math|Vector|MakeVector (.x _returnvalue) (Math|Random|RandomFloatinRange 3e+03 4e+03) (.z _returnvalue)) false false))))

(fn ConstructionScript)

(fn GetAttachPoint
  (return (Transformation|GetWorldTransform (Variables|Default|GetArrow))))