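; Straight track floor piece that randomizes its flanking buildings on BeginPlay and exposes its Arrow transform through GetAttachPoint.
; Each of four three-segment buildings, two per side, gets a random mesh from BuildingMeshes.
; Chained random switches hide upper segments to vary height; two-segment cuts end the chain early, and L01's is unreachable because its range stops at 1.
; The random position-offset logic is never run.
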(event EventBeginPlay
  (Utilities|FlowControl|Sequence
    (:then_0
      (bind _output_get (Variables|Default|SetBuilding%20Square%20L%2001%20Mesh (.OutItem (Utilities|Array|Random (Variables|Default|GetBuilding%20Meshes)))))
      (Components|StaticMesh|SetStaticMesh (Variables|Default|GetBuilding_Square_L_01_Bottom) _output_get)
      (Components|StaticMesh|SetStaticMesh (Variables|Default|GetBuilding_Square_L_01_Top) (Variables|Default|GetBuilding%20Square%20L%2001%20Mesh))
      (Components|StaticMesh|SetStaticMesh (Variables|Default|GetBuilding_Square_L_01_Middle) (Variables|Default|GetBuilding%20Square%20L%2001%20Mesh))
      (bind _output_get_2 (Variables|Default|SetBuilding%20Square%20L%2002%20Mesh (.OutItem (Utilities|Array|Random (Variables|Default|GetBuilding%20Meshes)))))
      (Components|StaticMesh|SetStaticMesh (Variables|Default|GetBuilding_Square_L_02_Bottom) _output_get_2)
      (Components|StaticMesh|SetStaticMesh (Variables|Default|GetBuilding_Square_L_02_Middle) (Variables|Default|GetBuilding%20Square%20L%2002%20Mesh))
      (Components|StaticMesh|SetStaticMesh (Variables|Default|GetBuilding_Square_L_02_Top) (Variables|Default|GetBuilding%20Square%20L%2002%20Mesh))
      (bind _output_get_3 (Variables|Default|SetBuilding%20Square%20R%2001%20Mesh (.OutItem (Utilities|Array|Random (Variables|Default|GetBuilding%20Meshes)))))
      (Components|StaticMesh|SetStaticMesh (Variables|Default|GetBuilding_Square_R_01_Bottom) _output_get_3)
      (Components|StaticMesh|SetStaticMesh (Variables|Default|GetBuilding_Square_R_01_Middle) (Variables|Default|GetBuilding%20Square%20R%2001%20Mesh))
      (Components|StaticMesh|SetStaticMesh (Variables|Default|GetBuilding_Square_R_01_Top) (Variables|Default|GetBuilding%20Square%20R%2001%20Mesh))
      (bind _output_get_4 (Variables|Default|SetBuilding%20Square%20R%2002%20Mesh (.OutItem (Utilities|Array|Random (Variables|Default|GetBuilding%20Meshes)))))
      (Components|StaticMesh|SetStaticMesh (Variables|Default|GetBuilding_Square_R_02_Bottom) _output_get_4)
      (Components|StaticMesh|SetStaticMesh (Variables|Default|GetBuilding_Square_R_02_Middle) (Variables|Default|GetBuilding%20Square%20R%2002%20Mesh))
      (Components|StaticMesh|SetStaticMesh (Variables|Default|GetBuilding_Square_R_02_Top) (Variables|Default|GetBuilding%20Square%20R%2002%20Mesh)))
    (:then_1
      (switch int (Math|Random|RandomIntegerinRange 0 2)
        (:0
          (switch int (Math|Random|RandomIntegerinRange 0 1) :!label _label
            (:0
              (switch int (Math|Random|RandomIntegerinRange 0 2) :!label _label_2
                (:0
                  (switch int (Math|Random|RandomIntegerinRange 0 2) :!label _label_3
                    (:1
                      (Development|SetHiddeninGame (Variables|Default|GetBuilding_Square_L_02_Top) true false))
                    (:2
                      (Development|SetHiddeninGame (Variables|Default|GetBuilding_Square_L_02_Top) true false)
                      (Development|SetHiddeninGame (Variables|Default|GetBuilding_Square_L_02_Middle) true false))))
                (:1
                  (Development|SetHiddeninGame (Variables|Default|GetBuilding_Square_R_02_Top) true false)
                  (goto _label_3))
                (:2
                  (Development|SetHiddeninGame (Variables|Default|GetBuilding_Square_R_02_Top) true false)
                  (Development|SetHiddeninGame (Variables|Default|GetBuilding_Square_R_02_Middle) true false))))
            (:1
              (Development|SetHiddeninGame (Variables|Default|GetBuilding_Square_L_01_Top) true false)
              (goto _label_2))
            (:2
              (Development|SetHiddeninGame (Variables|Default|GetBuilding_Square_L_01_Top) true false)
              (Development|SetHiddeninGame (Variables|Default|GetBuilding_Square_L_01_Middle) true false))))
        (:1
          (Development|SetHiddeninGame (Variables|Default|GetBuilding_Square_R_01_Top) true false)
          (goto _label))
        (:2
          (Development|SetHiddeninGame (Variables|Default|GetBuilding_Square_R_01_Top) true false)
          (Development|SetHiddeninGame (Variables|Default|GetBuilding_Square_R_01_Middle) true false))))
    (:then_2)))

(fn ConstructionScript)

(fn GetAttachPoint
  (return (Transformation|GetWorldTransform (Variables|Default|GetArrow))))