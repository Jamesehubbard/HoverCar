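; Straight track tile Blueprint that periodically spawns a random power-up as tiles are created.
; On BeginPlay it increments a shared TileNumber counter on HC_Gamemode until that counter exceeds four.
; The tile that finds it above four spawns a random PowerUps class at one of two scene-component positions, chosen at random, and resets the counter.
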(event EventBeginPlay
  (|CallParentFunction)
  (bind _returnvalue (Actor|GetActorOfClass "/Game/Blueprints/Engine/HC_Gamemode.HC_Gamemode_C"))
  (bind _ashc_gamemode (Utilities|Casting|CastToHC_Gamemode _returnvalue))
  (if (> (Variables|/Game/Blueprints/Engine/HC_Gamemode.HC_Gamemode_C|GetTile%20Number _ashc_gamemode) 4)
    (switch int (Math|Random|RandomIntegerinRange 0 1)
      (:0
        (Variables|Default|SetPowerUp%20Location (Transformation|GetWorldTransform (Variables|Default|GetScene))))
      (:1
        (Variables|Default|SetPowerUp%20Location (Transformation|GetWorldTransform (Variables|Default|GetScene1)))))
    (Game|SpawnActorfromClass (.OutItem (Utilities|Array|Random (Variables|Default|GetPowerUps))) (Variables|Default|GetPowerUp%20Location) "Undefined" "MultiplyWithRoot" 0 0)
    (Variables|/Game/Blueprints/Engine/HC_Gamemode.HC_Gamemode_C|SetTile%20Number _ashc_gamemode 0)
    (else
      (Math|Integer|IncrementInt (Variables|/Game/Blueprints/Engine/HC_Gamemode.HC_Gamemode_C|GetTile%20Number _ashc_gamemode)))))

(fn ConstructionScript
  (|CallParentFunction))