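; Straight-track pit trap Blueprint whose door slides open when the hover car enters its trigger box.
; On Box overlap, it checks the other actor against the first HoverCar_BP found in the level, so any other actor only prints a failure message.
; A match plays the OpenTrap timeline from the start, lerping the Door's relative X position while printing debug text each update.
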(event OnComponentBeginOverlap(Box)
  (params (OverlappedComponent :type Primitive%20Component%20Object%20Reference) (OtherActor :type Actor%20Object%20Reference) (OtherComp :type Primitive%20Component%20Object%20Reference) (OtherBodyIndex :type Integer) (bFromSweep :type Boolean) (SweepResult :type Hit%20Result%20Structure%20%28by%20ref%29))
  (bind _door (Variables|Default|GetDoor))
  (bind _relativelocation (Variables|/Script/Engine.SceneComponent|GetRelativeLocation _door))
  (bind _outactors (Actor|GetAllActorsOfClass "/Game/Blueprints/HoverCar_BP.HoverCar_BP_C"))
  (if (== OtherActor (Utilities|Array|Get(acopy) _outactors))
    (bind _opentrapdoor (Timeline|OpenTrap PlayFromStart)
      (:Update
        (Transformation|SetRelativeLocation _door (Math|Vector|MakeVector (Math|Float|Lerp 0.0 2e+02 _opentrapdoor) (.y _relativelocation) (.z _relativelocation)) false false)
        (Development|PrintString "UPDATING")))
    (else
      (Development|PrintString "BIG FAIL"))))

(event EventBeginPlay)

(event Collision|EventActorBeginOverlap
  (params (OtherActor :type Actor%20Object%20Reference)))

(event EventTick
  (params (DeltaSeconds :type Float%20%28single-precision%29)))

(fn ConstructionScript)