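; Bubble trap tile for the track that stops the hover car when it is inside the sphere as the bubble fully expands.
; Sphere overlap events track whether the first HoverCar_BP found in the level is inside.
; BubbleFullyExpanded zeroes that car's speed behind a DoOnce with no reset wired, while BubbleNotExpanded restores normal speed.
; Nothing in this graph calls either bubble event.
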(event OnComponentEndOverlap(Sphere)
  (params (OverlappedComponent :type Primitive%20Component%20Object%20Reference) (OtherActor :type Actor%20Object%20Reference) (OtherComp :type Primitive%20Component%20Object%20Reference) (OtherBodyIndex :type Integer))
  (bind _outactors (Actor|GetAllActorsOfClass "/Game/Blueprints/HoverCar_BP.HoverCar_BP_C"))
  (if (== OtherActor (Utilities|Array|Get(acopy) _outactors))
    (Variables|Default|SetIsOverlappingBubble false)))

(event OnComponentBeginOverlap(Sphere)
  (params (OverlappedComponent :type Primitive%20Component%20Object%20Reference) (OtherActor :type Actor%20Object%20Reference) (OtherComp :type Primitive%20Component%20Object%20Reference) (OtherBodyIndex :type Integer) (bFromSweep :type Boolean) (SweepResult :type Hit%20Result%20Structure%20%28by%20ref%29))
  (bind _outactors (Actor|GetAllActorsOfClass "/Game/Blueprints/HoverCar_BP.HoverCar_BP_C"))
  (if (== OtherActor (Utilities|Array|Get(acopy) _outactors))
    (Variables|Default|SetIsOverlappingBubble true)))

(event Custom|Bubble%20Fully%20Expanded
  (if (Variables|Default|GetIsOverlappingBubble)
    (Utilities|FlowControl|DoOnce false
      (:Completed
        (bind _outactors (Actor|GetAllActorsOfClass "/Game/Blueprints/HoverCar_BP.HoverCar_BP_C"))
        (bind _ashover_car_bp (Utilities|Casting|CastToHoverCar_BP (Utilities|Array|Get(acopy) _outactors)))
        (Default|SetSpeedto0 _ashover_car_bp)))))

(event Custom|Bubble%20Not%20Expanded
  (bind _outactors (Actor|GetAllActorsOfClass "/Game/Blueprints/HoverCar_BP.HoverCar_BP_C"))
  (bind _ashover_car_bp (Utilities|Casting|CastToHoverCar_BP (Utilities|Array|Get(acopy) _outactors)))
  (Default|SetSpeedtoNormal _ashover_car_bp))

(fn ConstructionScript
  (|CallParentFunction))