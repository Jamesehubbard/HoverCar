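; Track trap tile with bollards that alternate between blocking and passable states.
; BeginPlay starts a looping bollard animation on the skeletal mesh.
; BollardsDown and BollardsUp events switch the WallTrapBollardSimple0101 collision profile between NoCollision and BlockAll, and each also sets the skeletal mesh's material slot 2.
; Nothing in this graph calls those events, and the construction script only runs its parent's.
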(event Custom|Bollards%20Down
  (Collision|SetCollisionProfileName (Variables|Default|GetWall_Trap_Bollard_Simple_01_01) "NoCollision" true :!class /Script/Engine.PrimitiveComponent)
  (Rendering|Material|SetMaterial (Variables|Default|GetSkeletalMesh) 2 0))

(event Custom|Bollards%20Up
  (Collision|SetCollisionProfileName (Variables|Default|GetWall_Trap_Bollard_Simple_01_01) "BlockAll" true :!class /Script/Engine.PrimitiveComponent)
  (Rendering|Material|SetMaterial (Variables|Default|GetSkeletalMesh) 2 0))

(event EventBeginPlay
  (Components|Animation|PlayAnimation (Variables|Default|GetSkeletalMesh) "/Game/Assets/Track/Traps/Bollards/Trap_Straight_Bollard_01_03__1__Anim.Trap_Straight_Bollard_01_03__1__Anim" true))

(fn ConstructionScript
  (|CallParentFunction))