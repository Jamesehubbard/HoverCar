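; End tile of a track that randomises the four stacked buildings along its sides at BeginPlay.
; Each stack gets a random mesh for all three segments and a random absolute world Y within its side's range.
; Chained random switches hide upper segments to vary height, but hiding two segments ends the chain, leaving later stacks full height.
; GetAttachPoint returns the Arrow component's world transform.
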(event EventBeginPlay
  (bind _building_square_r_02_top (Variables|Default|GetBuilding_Square_R_02_Top))
  (bind _building_square_r_01_top (Variables|Default|GetBuilding_Square_R_01_Top))
  (bind _building_square_l_02_bottom (Variables|Default|GetBuilding_Square_L_02_Bottom))
  (bind _building_square_r_01_bottom (Variables|Default|GetBuilding_Square_R_01_Bottom))
  (bind _building_square_l_01_bottom (Variables|Default|GetBuilding_Square_L_01_Bottom))
  (bind _building_square_l_01_middle (Variables|Default|GetBuilding_Square_L_01_Middle))
  (bind _building_square_l_01_top (Variables|Default|GetBuilding_Square_L_01_Top))
  (bind _building_square_l_02_middle (Variables|Default|GetBuilding_Square_L_02_Middle))
  (bind _building_square_l_02_top (Variables|Default|GetBuilding_Square_L_02_Top))
  (bind _building_square_r_01_middle (Variables|Default|GetBuilding_Square_R_01_Middle))
  (bind _building_square_r_02_bottom (Variables|Default|GetBuilding_Square_R_02_Bottom))
  (bind _building_square_r_02_middle (Variables|Default|GetBuilding_Square_R_02_Middle))
  (bind _returnvalue (Transformation|GetWorldLocation _building_square_r_02_top))
  (bind _returnvalue_2 (Transformation|GetWorldLocation _building_square_r_01_top))
  (bind _returnvalue_3 (Transformation|GetWorldLocation _building_square_l_02_bottom))
  (bind _returnvalue_4 (Transformation|GetWorldLocation _building_square_r_01_bottom))
  (bind _returnvalue_5 (Transformation|GetWorldLocation _building_square_l_01_bottom))
  (bind _returnvalue_6 (Transformation|GetWorldLocation _building_square_l_01_middle))
  (bind _returnvalue_7 (Transformation|GetWorldLocation _building_square_l_01_top))
  (bind _returnvalue_8 (Transformation|GetWorldLocation _building_square_l_02_middle))
  (bind _returnvalue_9 (Transformation|GetWorldLocation _building_square_l_02_top))
  (bind _returnvalue_10 (Transformation|GetWorldLocation _building_square_r_01_middle))
  (bind _returnvalue_11 (Transformation|GetWorldLocation _building_square_r_02_bottom))
  (bind _returnvalue_12 (Transformation|GetWorldLocation _building_square_r_02_middle))
  (Utilities|FlowControl|Sequence
    (:then_0
      (bind _output_get (Variables|Default|SetBuilding%20Square%20L%2001%20Mesh (.OutItem (Utilities|Array|Random (Variables|Default|GetBuilding%20Meshes)))))
      (Components|StaticMesh|SetStaticMesh (Variables|Default|GetBuilding_Square_L_01_Bottom) _output_get)
      (Components|StaticMesh|SetStaticMesh (Variables|Default|GetBuilding_Square_L_01_Top) (Variables|Default|GetBuilding%20Square%20L%2001%20Mesh))
      (Components|StaticMesh|SetStaticMesh (Variables|Default|GetBuilding_Square_L_01_Middle) (Variables|Default|GetBuilding%20Square%20L%2001%20Mesh))
      (bind _output_get_2 (Variables|Default|SetBuilding%20Square%20L%2002%20Mesh (.OutItem (Utilities|Array|Random (Variables|Default|GetBuilding%20Meshes)))))
      (Components|StaticMesh|SetStaticMesh (Variables|Default|GetBuilding_Square_L_02_Bottom) _output_get_2)
      (Components|StaticMesh|SetStaticMesh (Variables|Default|GetBuilding_Square_L_02_Middle) (Variables|Default|GetBuilding%20Square%20L%2002%20Mesh))
      (Components|StaticMesh|SetStaticMesh (Variables|Default|GetBuilding_Square_L_02_Top) (Variables|Default|GetBuilding%20Square%20L%2002%20Mesh))
      (bind _output_get_3 (Variables|Default|SetBuilding%20Square%20R%2001%20Mesh (.OutItem (Utilities|Array|Random (Variables|Default|GetBuilding%20Meshes)))))
      (Components|StaticMesh|SetStaticMesh (Variables|Default|GetBuilding_Square_R_01_Bottom) _output_get_3)
      (Components|StaticMesh|SetStaticMesh (Variables|Default|GetBuilding_Square_R_01_Middle) (Variables|Default|GetBuilding%20Square%20R%2001%20Mesh))
      (Components|StaticMesh|SetStaticMesh (Variables|Default|GetBuilding_Square_R_01_Top) (Variables|Default|GetBuilding%20Square%20R%2001%20Mesh))
      (bind _output_get_4 (Variables|Default|SetBuilding%20Square%20R%2002%20Mesh (.OutItem (Utilities|Array|Random (Variables|Default|GetBuilding%20Meshes)))))
      (Components|StaticMesh|SetStaticMesh (Variables|Default|GetBuilding_Square_R_02_Bottom) _output_get_4)
      (Components|StaticMesh|SetStaticMesh (Variables|Default|GetBuilding_Square_R_02_Middle) (Variables|Default|GetBuilding%20Square%20R%2002%20Mesh))
      (Components|StaticMesh|SetStaticMesh (Variables|Default|GetBuilding_Square_R_02_Top) (Variables|Default|GetBuilding%20Square%20R%2002%20Mesh)))
    (:then_1
      (switch int (Math|Random|RandomIntegerinRange 0 2)
        (:0
          (switch int (Math|Random|RandomIntegerinRange 0 2) :!label _label
            (:0
              (switch int (Math|Random|RandomIntegerinRange 0 2) :!label _label_2
                (:0
                  (switch int (Math|Random|RandomIntegerinRange 0 2) :!label _label_3
                    (:1
                      (Development|SetHiddeninGame (Variables|Default|GetBuilding_Square_L_02_Top) true false))
                    (:2
                      (Development|SetHiddeninGame (Variables|Default|GetBuilding_Square_L_02_Top) true false)
                      (Development|SetHiddeninGame (Variables|Default|GetBuilding_Square_L_02_Middle) true false))))
                (:1
                  (Development|SetHiddeninGame (Variables|Default|GetBuilding_Square_R_02_Top) true false)
                  (goto _label_3))
                (:2
                  (Development|SetHiddeninGame (Variables|Default|GetBuilding_Square_R_02_Top) true false)
                  (Development|SetHiddeninGame (Variables|Default|GetBuilding_Square_R_02_Middle) true false))))
            (:1
              (Development|SetHiddeninGame (Variables|Default|GetBuilding_Square_L_01_Top) true false)
              (goto _label_2))
            (:2
              (Development|SetHiddeninGame (Variables|Default|GetBuilding_Square_L_01_Top) true false)
              (Development|SetHiddeninGame (Variables|Default|GetBuilding_Square_L_01_Middle) true false))))
        (:1
          (Development|SetHiddeninGame (Variables|Default|GetBuilding_Square_R_01_Top) true false)
          (goto _label))
        (:2
          (Development|SetHiddeninGame (Variables|Default|GetBuilding_Square_R_01_Top) true false)
          (Development|SetHiddeninGame (Variables|Default|GetBuilding_Square_R_01_Middle) true false))))
    (:then_2
      (bind _output_get_5 (Variables|Default|SetSquare%20L%2001%20Location (Math|Random|RandomFloatinRange -1e+03 0.0)))
      (Transformation|SetWorldLocation _building_square_l_01_bottom (Math|Vector|MakeVector (.x _returnvalue_5) _output_get_5 (.z _returnvalue_5)) false false)
      (Transformation|SetWorldLocation _building_square_l_01_middle (Math|Vector|MakeVector (.x _returnvalue_6) (Variables|Default|GetSquare%20L%2001%20Location) (.z _returnvalue_6)) false false)
      (Transformation|SetWorldLocation _building_square_l_01_top (Math|Vector|MakeVector (.x _returnvalue_7) (Variables|Default|GetSquare%20L%2001%20Location) (.z _returnvalue_7)) false false)
      (bind _output_get_6 (Variables|Default|SetSquare%20L%2002%20Location (Math|Random|RandomFloatinRange -1e+03 0.0)))
      (Transformation|SetWorldLocation _building_square_l_02_bottom (Math|Vector|MakeVector (.x _returnvalue_3) _output_get_6 (.z _returnvalue_3)) false false)
      (Transformation|SetWorldLocation _building_square_l_02_middle (Math|Vector|MakeVector (.x _returnvalue_8) (Variables|Default|GetSquare%20L%2002%20Location) (.z _returnvalue_8)) false false)
      (Transformation|SetWorldLocation _building_square_l_02_top (Math|Vector|MakeVector (.x _returnvalue_9) (Variables|Default|GetSquare%20L%2002%20Location) (.z _returnvalue_9)) false false)
      (bind _output_get_7 (Variables|Default|SetSquare%20R%2001%20Location (Math|Random|RandomFloatinRange 3e+03 4e+03)))
      (Transformation|SetWorldLocation _building_square_r_01_bottom (Math|Vector|MakeVector (.x _returnvalue_4) _output_get_7 (.z _returnvalue_4)) false false)
      (Transformation|SetWorldLocation _building_square_r_01_middle (Math|Vector|MakeVector (.x _returnvalue_10) (Variables|Default|GetSquare%20R%2001%20Location) (.z _returnvalue_10)) false false)
      (Transformation|SetWorldLocation _building_square_r_01_top (Math|Vector|MakeVector (.x _returnvalue_2) (Variables|Default|GetSquare%20R%2001%20Location) (.z _returnvalue_2)) false false)
      (bind _output_get_8 (Variables|Default|SetSquare%20R%2002%20Location (Math|Random|RandomFloatinRange 3e+03 4e+03)))
      (Transformation|SetWorldLocation _building_square_r_02_bottom (Math|Vector|MakeVector (.x _returnvalue_11) _output_get_8 (.z _returnvalue_11)) false false)
      (Transformation|SetWorldLocation _building_square_r_02_middle (Math|Vector|MakeVector (.x _returnvalue_12) (Variables|Default|GetSquare%20R%2002%20Location) (.z _returnvalue_12)) false false)
      (Transformation|SetWorldLocation _building_square_r_02_top (Math|Vector|MakeVector (.x _returnvalue) (Variables|Default|GetSquare%20R%2002%20Location) (.z _returnvalue)) false false))))

(fn ConstructionScript)

(fn GetAttachPoint
  (return (Transformation|GetWorldTransform (Variables|Default|GetArrow))))