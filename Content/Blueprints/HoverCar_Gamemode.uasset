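; Game mode for a hover car game that builds an endless track from randomly chosen floor tiles.
; BeginPlay spawns the initial tiles, each placed at the previous tile's attach point.
; AddFloor counts consecutive straights and inserts a random turn piece after a fixed run of them.
; ExtendFloor appends a tile and destroys the oldest once the track exceeds its size limit, keeping a rolling window.
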(event EventBeginPlay
  (for _index (range 0 (- (Variables|Default|GetNumber%20Of%20Tiles) 1))
    (CallFunction|AddFloor)))

(fn ConstructionScript)

(fn AddFloor
  (if (> (Variables|Default|GetCurrentStraights) 7)
    (CallFunction|AddFloorTurn)
    (else
      (bind _returnvalue (Game|SpawnActorfromClass (Utilities|Array|Get(acopy) (Variables|Default|GetFloor%20Tiles) (Math|Random|RandomIntegerinRange 0 (Utilities|Array|LastIndex (Variables|Default|GetFloor%20Tiles)))) (Variables|Default|GetNext%20Spawn%20Point) "Undefined" "MultiplyWithRoot" 0 0))
      (bind _asfloor_bp (Utilities|Casting|CastToFloor_BP _returnvalue))
      (bind _returnvalue_2 (Default|GetAttachPoint _asfloor_bp))
      (Variables|Default|SetNext%20Spawn%20Point _returnvalue_2)
      (Variables|Default|SetCurrentStraights (+ (Variables|Default|GetCurrentStraights) 1))
      (Utilities|Array|Add (Variables|Default|GetFloors) _asfloor_bp))))

(fn AddFloorTurn
  (bind _returnvalue (Game|SpawnActorfromClass (Utilities|Array|Get(acopy) (Variables|Default|GetFloor%20Turns) (Math|Random|RandomIntegerinRange 0 (Utilities|Array|LastIndex (Variables|Default|GetFloor%20Turns)))) (Variables|Default|GetNext%20Spawn%20Point) "Undefined" "MultiplyWithRoot" 0 0))
  (bind _asfloor_bp (Utilities|Casting|CastToFloor_BP _returnvalue))
  (bind _returnvalue_2 (Default|GetAttachPoint _asfloor_bp))
  (Variables|Default|SetNext%20Spawn%20Point _returnvalue_2)
  (Variables|Default|SetCurrentStraights 0)
  (Utilities|Array|Add (Variables|Default|GetFloors) _asfloor_bp))

(fn ExtendFloor
  (bind _floors (Variables|Default|GetFloors))
  (bind _output (Utilities|Array|Get(acopy) _floors))
  (CallFunction|AddFloor)
  (if (> (Utilities|Array|Length (Variables|Default|GetFloors)) (+ (Variables|Default|GetNumber%20Of%20Tiles) 1))
    (Actor|DestroyActor _output)
    (Utilities|Array|RemoveItem _floors _output)))