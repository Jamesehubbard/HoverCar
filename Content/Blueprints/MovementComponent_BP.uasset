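; Movement component that drives its owner's physics-simulated root body toward a target linear and angular speed.
; On BeginPlay it caches the owner's root primitive component.
; Each tick it measures speed along the body's right vector and yaw rate around its up vector.
; Proportional control then turns each speed error into force and torque on those axes, leaving other motion to physics.
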(event EventBeginPlay
  (bind _asprimitive_component (Utilities|Casting|CastToPrimitiveComponent (Variables|/Script/Engine.Actor|GetRootComponent (Components|GetOwner))))
  (Variables|Default|SetBody%20Reference _asprimitive_component))

(event EventTick
  (params (DeltaSeconds :type Float%20%28single-precision%29))
  (bind _body_reference (Variables|Default|GetBody%20Reference))
  (bind _body_reference_2 (Variables|Default|GetBody%20Reference)
    (:then
      (bind _returnvalue (Physics|GetPhysicsLinearVelocity _body_reference_2 "None"))
      (Variables|Default|SetCurrentSpeed (Math|Vector|DotProduct _returnvalue (Math|Vector|GetRightVector _body_reference_2)))
      (Variables|Default|SetCurrentAngularSpeed (Math|Vector|DotProduct (Physics|GetPhysicsAngularVelocityinDegrees _body_reference "None") (Math|Vector|GetUpVector _body_reference)))
      (Physics|AddForce (Variables|Default|GetBody%20Reference) (* (Math|Vector|GetRightVector (Variables|Default|GetBody%20Reference)) (* (- (Variables|Default|GetTargetSpeed) (Variables|Default|GetCurrentSpeed)) (Variables|Default|GetSpeedToForceFactor))) "None" false)
      (Class|PrimitiveComponent|AddTorqueinDegrees (Variables|Default|GetBody%20Reference) (* (Math|Vector|GetUpVector (Variables|Default|GetBody%20Reference)) (* (- (Variables|Default|GetTargetAngularSpeed) (Variables|Default|GetCurrentAngularSpeed)) (Variables|Default|GetAngularSpeedToTorqueFactor))) "None" false))
    (:else)))