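; NewHoverCar_BP is a player-controlled hover car that drives by applying physics forces to its Body component.
; On BeginPlay it adds its Enhanced Input mapping context to the player's subsystem and shows the mouse cursor.
; The Move input's X axis applies yaw torque for steering, while Y applies thrust along the body's right vector, which serves as the driving axis.
; The graph contains no hover or suspension logic.
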(event Input|EnhancedActionEvents|EnhancedInputActionMove_IA
  (params (ActionValue :type Vector%202D%20Structure) (ElapsedSeconds :type Float%20%28double-precision%29) (TriggeredSeconds :type Float%20%28double-precision%29) (InputAction :type Input%20Action%20Object%20Reference :default "/Game/Input/Move_IA.Move_IA"))
  (Class|PrimitiveComponent|AddTorqueinRadians (Variables|Default|GetBody) (Math|Vector|MakeVector 0.0 0.0 (* (.x ActionValue) 4e+08)) "None" false)
  (Physics|AddForce (Variables|Default|GetBody) (* (* (Math|Vector|GetRightVector (Variables|Default|GetBody)) 3.4e+07) (.y ActionValue)) "None" false))

(event EventBeginPlay
  (bind _asplayer_controller (Utilities|Casting|CastToPlayerController (Pawn|GetController)))
  (Utilities|IsValid (PlayerController|LocalPlayerSubsystems|GetEnhancedInputLocalPlayerSubsystem _asplayer_controller)
    (:Is%20Valid
      (Input|AddMappingContext (PlayerController|LocalPlayerSubsystems|GetEnhancedInputLocalPlayerSubsystem _asplayer_controller) "/Game/Input/InputMappingContext.InputMappingContext" 0 "(bIgnoreAllPressedKeysUntilRelease=True,bForceImmediately=False,bNotifyUserSettings=False)")
      (Variables|/Script/Engine.PlayerController|SetbShowMouseCursor (Game|GetPlayerController 0) true))))

(fn ConstructionScript)