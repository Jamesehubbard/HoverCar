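; BP_HoverComponent is a suspension point that keeps its owning BP_HoverVehicle floating above surfaces.
; On BeginPlay it caches the owner, then each tick it line-traces down its own up vector up to HoverDistance, with debug drawing.
; On a hit, a spring-damper computed from the compression and its rate of change pushes the vehicle's root primitive along that up vector at the component's location.
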(event EventBeginPlay
  (bind _asbp_hover_vehicle (Utilities|Casting|CastToBP_HoverVehicle (Components|GetOwner)))
  (Variables|Default|SetParentVehicle _asbp_hover_vehicle))

(event EventTick
  (params (DeltaSeconds :type Float%20%28single-precision%29))
  (bind _returnvalue (Transformation|GetWorldLocation))
  (Utilities|IsValid (Variables|Default|GetParentVehicle)
    (:Is%20Valid
      (bind (_outhit _returnvalue_2) (Collision|LineTraceByChannel _returnvalue (- _returnvalue (* (Math|Vector|GetUpVector) (Variables|Default|GetHoverDistance))) "TraceTypeQuery1" false 0 "ForOneFrame"))
      (Variables|Default|SetOut%20Hit _outhit)
      (if _returnvalue_2
        (bind _output_get (Variables|Default|SetHoverDelta (- (Variables|Default|GetHoverDistance) (.Distance (Collision|BreakHitResult (Variables|Default|GetOut%20Hit))))))
        (bind _asprimitive_component (Utilities|Casting|CastToPrimitiveComponent (Variables|/Script/Engine.Actor|GetRootComponent (Variables|Default|GetParentVehicle))))
        (Class|PrimitiveComponent|AddForceatLocation _asprimitive_component (* (Math|Vector|GetUpVector) (+ (* (/ (- _output_get (Variables|Default|GetPrevious%20Hover%20Delta)) (Utilities|Time|GetWorldDeltaSeconds)) (Variables|Default|GetDampingCoefficent)) (* _output_get (Variables|Default|GetSpringCoefficent)))) (Transformation|GetWorldLocation) "None")
        (Variables|Default|SetPrevious%20Hover%20Delta (Variables|Default|GetHoverDelta))))))