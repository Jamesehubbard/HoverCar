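; Player-driven hover car Pawn that moves kinematically along its right vector, with no physics or sweep.
; Throttle and Steer axes ease speed and steering angle, which Tick turns into world offset and speed-scaled yaw.
; Look axes rotate the spring arm, while Tick lengthens it at speed.
; The shortening branch tests against MaxSpeed rather than the lengthening threshold, so both interpolations can run in one frame.
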(event EventTick
  (params (DeltaSeconds :type Float%20%28single-precision%29))
  (bind _currentspeed (Variables|Default|GetCurrentSpeed))
  (Transformation|AddActorWorldOffset (* DeltaSeconds (* (Transformation|GetActorRightVector) (Variables|Default|GetCurrentSpeed))))
  (Class|Actor|AddActorWorldRotation (Math|Rotator|MakeRotator 0.0 0.0 (* (Variables|Default|GetCurrentSpeed) (Variables|Default|GetCurrentSteeringAngle) (Variables|Default|GetSpeedToRotationFactor) (Utilities|Time|GetWorldDeltaSeconds))))
  ;[1 1 1] Adjusting spring arm based on speed
  (Utilities|FlowControl|Sequence
    (:then_0
      (if (> _currentspeed 3e+02)
        (Variables|/Script/Engine.SpringArmComponent|SetTargetArmLength (Variables|Default|GetSpringArm) (Math|Interpolation|FInterpTo (Variables|/Script/Engine.SpringArmComponent|GetTargetArmLength (Variables|Default|GetSpringArm)) 1e+03 (Utilities|Time|GetWorldDeltaSeconds) 5.0))))
    (:then_1
      (if (<= _currentspeed (Variables|Default|GetMaxSpeed))
        (Variables|/Script/Engine.SpringArmComponent|SetTargetArmLength (Variables|Default|GetSpringArm) (Math|Interpolation|FInterpTo (Variables|/Script/Engine.SpringArmComponent|GetTargetArmLength (Variables|Default|GetSpringArm)) 6e+02 (Utilities|Time|GetWorldDeltaSeconds) 3.0))))))

(event Input|AxisEvents|InputAxisThrottle
  (params (AxisValue :type Float%20%28single-precision%29))
  (Variables|Default|SetCurrentSpeed (Math|Interpolation|FInterpTo (Variables|Default|GetCurrentSpeed) (* AxisValue (Variables|Default|GetMaxSpeed)) (Utilities|Time|GetWorldDeltaSeconds) 4.0)))

(event Input|AxisEvents|InputAxisSteer
  (params (AxisValue :type Float%20%28single-precision%29))
  (Variables|Default|SetCurrentSteeringAngle (Math|Interpolation|FInterpTo (Variables|Default|GetCurrentSteeringAngle) (* AxisValue (Variables|Default|GetMaxSteeringAngle)) (Utilities|Time|GetWorldDeltaSeconds) 4.0)))

(event Input|AxisEvents|InputAxisLookRight
  (params (AxisValue :type Float%20%28single-precision%29))
  (Transformation|AddRelativeRotation (Variables|Default|GetSpringArm) (Math|Rotator|MakeRotator 0.0 0.0 AxisValue) false false))

(event Input|AxisEvents|InputAxisLookUp
  (params (AxisValue :type Float%20%28single-precision%29))
  (Transformation|AddRelativeRotation (Variables|Default|GetSpringArm) (Math|Rotator|MakeRotator 0.0 AxisValue 0.0) false false))

(fn ConstructionScript)