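; Player hover car pawn for a two-player chase game, cast as runner or chaser by spawn X position with differing top speeds.
; Interpolated throttle and steer inputs move it by unswept transform offsets, with a speed-based spring arm.
; The runner's power-ups slow the chaser until A is mashed, or briefly invert its controls, via gamemode player references.
; RPM drives engine audio, but only its decay is wired.
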(event Custom|Set%20Speed%20to%20Normal
  (Variables|Default|SetCurrentSpeed 2.5e+03))

(event Custom|Set%20Speed%20to%200
  (Variables|Default|SetCurrentSpeed 0.0))

(event EventTick
  (params (DeltaSeconds :type Float%20%28single-precision%29))
  (Audio|Parameter|SetFloatParameter (Variables|Default|GetMS_Engine) "Crossfade RPM Range" (Variables|Default|GetRPM) :!class /Script/AudioExtensions.AudioParameterControllerInterface)
  (Audio|Parameter|SetFloatParameter (Variables|Default|GetMS_Motor) "Crossfade RPM Range" (Variables|Default|GetRPM) :!class /Script/AudioExtensions.AudioParameterControllerInterface)
  (if (== (Input|AxisValues|GetThrottle) 0.0)
    (if (>= (Variables|Default|GetRPM) 0.0)
      (Variables|Default|SetRPM (- (Variables|Default|GetRPM) 0.1))
      (Audio|Components|Audio|SetVolumeMultiplier (Variables|Default|GetMS_Engine) (Variables|/Game/Hover_Car/Blueprints/Engine/HC_Gamemode.HC_Gamemode_C|GetMasterVolume (Variables|Default|GetMy_Gamemode)) :!class /Script/Engine.AudioComponent))))

(event EventBeginPlay
  (bind _ashc_gamemode (Utilities|Casting|CastToHC_Gamemode (Game|GetGameMode)))
  (Variables|Default|SetMy_Gamemode _ashc_gamemode)
  (Input|DisableInput 0)
  (Utilities|FlowControl|Delay 1.0)
  (if (> (.x (Transformation|GetWorldLocation (Variables|Default|GetStaticMesh))) -1e+03)
    (Variables|Default|SetIs%20Runner true)
    (Variables|Default|SetIs%20Chaser false)
    (Variables|Default|SetMaxSpeed 2e+03)
    (Utilities|FlowControl|Delay 2.0)
    (Input|EnableInput 0)
    (Utilities|FlowControl|DoOnce false :!label _label
      (:Completed
        (bind _returnvalue (UserInterface|CreateWidget "/Game/Hover_Car/UI/InGame/WBP_InGame.WBP_InGame_C"))
        (bind _output_get (Variables|Default|SetIn%20Game%20Widget _returnvalue))
        (UserInterface|Viewport|AddtoViewport _output_get 0)))
    (else
      (Variables|Default|SetIs%20Chaser true)
      (Variables|Default|SetIs%20Runner false)
      (Variables|Default|SetMaxSpeed 1.5e+03)
      (Utilities|FlowControl|Delay 2.0)
      (Input|EnableInput 0)
      (Utilities|FlowControl|Sequence
        (:then_0
          (goto _label))
        (:then_1
          (Utilities|FlowControl|Delay 1e+01)
          (Variables|Default|SetMaxSpeed 2.5e+03))))))

(event Input|ActionEvents|InputActionAButton
  (params (Key :type Key%20Structure :default "None"))
  (:Pressed
    (if (Variables|Default|GetSlow%20Down%20Effect%20Active)
      (Math|Integer|IncrementInt (Variables|Default|GetA%20Button%20Pressed)
        (:%20%20
          (if (> (Variables|Default|GetA%20Button%20Pressed) (Math|Random|RandomIntegerinRange 5 8))
            (Variables|Default|SetMaxSpeed 2.5e+03)
            (Variables|Default|SetA%20Button%20Pressed 0)
            (Variables|Default|SetSlow%20Down%20Effect%20Active false)))))))

(event Input|ActionEvents|InputActionPowerUpButton
  (params (Key :type Key%20Structure :default "None"))
  (:Pressed
    (if (Variables|Default|GetIs%20Runner)
      (if (Variables|Default|GetHas%20Slow%20Power-Up)
        (Default|SlowPower-UpUsed (Variables|Default|GetIn%20Game%20Widget))
        (bind _ashc_gamemode (Utilities|Casting|CastToHC_Gamemode (Game|GetGameMode)))
        (Variables|Default|SetMy_Gamemode _ashc_gamemode)
        (if (Variables|/Game/Hover_Car/Blueprints/Engine/HC_Gamemode.HC_Gamemode_C|GetIsP1Chaser _ashc_gamemode)
          (Variables|HoverCar_BP_C|SetMaxSpeed (Variables|/Game/Hover_Car/Blueprints/Engine/HC_Gamemode.HC_Gamemode_C|GetPlayer1 (Variables|Default|GetMy_Gamemode)) 1e+02)
          (Variables|HoverCar_BP_C|SetSlow%20Down%20Effect%20Active (Variables|/Game/Hover_Car/Blueprints/Engine/HC_Gamemode.HC_Gamemode_C|GetPlayer1 (Variables|Default|GetMy_Gamemode)) true)
          (Variables|HoverCar_BP_C|SetHas%20Slow%20Power-Up (Variables|/Game/Hover_Car/Blueprints/Engine/HC_Gamemode.HC_Gamemode_C|GetPlayer2 (Variables|Default|GetMy_Gamemode)) false)
          (else
            (Variables|HoverCar_BP_C|SetMaxSpeed (Variables|/Game/Hover_Car/Blueprints/Engine/HC_Gamemode.HC_Gamemode_C|GetPlayer2 (Variables|Default|GetMy_Gamemode)) 1e+02)
            (Variables|HoverCar_BP_C|SetSlow%20Down%20Effect%20Active (Variables|/Game/Hover_Car/Blueprints/Engine/HC_Gamemode.HC_Gamemode_C|GetPlayer2 (Variables|Default|GetMy_Gamemode)) true)
            (Variables|HoverCar_BP_C|SetHas%20Slow%20Power-Up (Variables|/Game/Hover_Car/Blueprints/Engine/HC_Gamemode.HC_Gamemode_C|GetPlayer1 (Variables|Default|GetMy_Gamemode)) false)))
        (elif (Variables|Default|GetHas%20Reverse%20Power-Up)
          (Default|ReversePower-UpUsed (Variables|Default|GetIn%20Game%20Widget))
          (bind _ashc_gamemode_2 (Utilities|Casting|CastToHC_Gamemode (Game|GetGameMode)))
          (Variables|Default|SetMy_Gamemode _ashc_gamemode_2)
          (if (Variables|/Game/Hover_Car/Blueprints/Engine/HC_Gamemode.HC_Gamemode_C|GetIsP1Chaser _ashc_gamemode_2)
            (Variables|HoverCar_BP_C|SetThrottle%20Axis (Variables|/Game/Hover_Car/Blueprints/Engine/HC_Gamemode.HC_Gamemode_C|GetPlayer1 (Variables|Default|GetMy_Gamemode)) -1.0)
            (Variables|HoverCar_BP_C|SetSteer%20Axis (Variables|/Game/Hover_Car/Blueprints/Engine/HC_Gamemode.HC_Gamemode_C|GetPlayer1 (Variables|Default|GetMy_Gamemode)) -1.0)
            (Variables|HoverCar_BP_C|SetHas%20Reverse%20Power-Up (Variables|/Game/Hover_Car/Blueprints/Engine/HC_Gamemode.HC_Gamemode_C|GetPlayer2 (Variables|Default|GetMy_Gamemode)) false)
            (Utilities|FlowControl|Delay 3.0)
            (Variables|HoverCar_BP_C|SetThrottle%20Axis (Variables|/Game/Hover_Car/Blueprints/Engine/HC_Gamemode.HC_Gamemode_C|GetPlayer1 (Variables|Default|GetMy_Gamemode)) 1.0)
            (Variables|HoverCar_BP_C|SetSteer%20Axis (Variables|/Game/Hover_Car/Blueprints/Engine/HC_Gamemode.HC_Gamemode_C|GetPlayer1 (Variables|Default|GetMy_Gamemode)) 1.0)
            (else
              (Variables|HoverCar_BP_C|SetThrottle%20Axis (Variables|/Game/Hover_Car/Blueprints/Engine/HC_Gamemode.HC_Gamemode_C|GetPlayer2 (Variables|Default|GetMy_Gamemode)) -1.0)
              (Variables|HoverCar_BP_C|SetSteer%20Axis (Variables|/Game/Hover_Car/Blueprints/Engine/HC_Gamemode.HC_Gamemode_C|GetPlayer2 (Variables|Default|GetMy_Gamemode)) -1.0)
              (Variables|HoverCar_BP_C|SetHas%20Reverse%20Power-Up (Variables|/Game/Hover_Car/Blueprints/Engine/HC_Gamemode.HC_Gamemode_C|GetPlayer1 (Variables|Default|GetMy_Gamemode)) false)
              (Utilities|FlowControl|Delay 3.0)
              (Variables|HoverCar_BP_C|SetThrottle%20Axis (Variables|/Game/Hover_Car/Blueprints/Engine/HC_Gamemode.HC_Gamemode_C|GetPlayer2 (Variables|Default|GetMy_Gamemode)) 1.0)
              (Variables|HoverCar_BP_C|SetSteer%20Axis (Variables|/Game/Hover_Car/Blueprints/Engine/HC_Gamemode.HC_Gamemode_C|GetPlayer2 (Variables|Default|GetMy_Gamemode)) 1.0))))))))

(event Input|AxisEvents|InputAxisThrottle
  (params (AxisValue :type Float%20%28single-precision%29))
  (Variables|Default|SetCurrentSpeed (Math|Interpolation|FInterpTo (Variables|Default|GetCurrentSpeed) (* (* AxisValue (Variables|Default|GetThrottle%20Axis)) (Variables|Default|GetMaxSpeed)) (Utilities|Time|GetWorldDeltaSeconds) 4.0))
  (Transformation|AddActorWorldOffset (* (Utilities|Time|GetWorldDeltaSeconds) (* (Transformation|GetActorRightVector) (Variables|Default|GetCurrentSpeed))))
  ;[1 1 1] Adjusting spring arm based on speed
  (Utilities|FlowControl|Sequence
    (:then_0
      (if (> (Variables|Default|GetCurrentSpeed) 3e+02)
        (Variables|/Script/Engine.SpringArmComponent|SetTargetArmLength (Variables|Default|GetSpringArm) (Math|Interpolation|FInterpTo (Variables|/Script/Engine.SpringArmComponent|GetTargetArmLength (Variables|Default|GetSpringArm)) 1e+03 (Utilities|Time|GetWorldDeltaSeconds) 5.0))))
    (:then_1
      (if (<= (Variables|Default|GetCurrentSpeed) (Variables|Default|GetMaxSpeed))
        (Variables|/Script/Engine.SpringArmComponent|SetTargetArmLength (Variables|Default|GetSpringArm) (Math|Interpolation|FInterpTo (Variables|/Script/Engine.SpringArmComponent|GetTargetArmLength (Variables|Default|GetSpringArm)) 6e+02 (Utilities|Time|GetWorldDeltaSeconds) 3.0))))))

(event Input|AxisEvents|InputAxisSteer
  (params (AxisValue :type Float%20%28single-precision%29))
  (Variables|Default|SetCurrentSteeringAngle (Math|Interpolation|FInterpTo (Variables|Default|GetCurrentSteeringAngle) (* (* AxisValue (Variables|Default|GetSteer%20Axis)) (Variables|Default|GetMaxSteeringAngle)) (Utilities|Time|GetWorldDeltaSeconds) 4.0))
  (Class|Actor|AddActorWorldRotation (Math|Rotator|MakeRotator 0.0 0.0 (* (Variables|Default|GetCurrentSpeed) (Variables|Default|GetCurrentSteeringAngle) (Variables|Default|GetSpeedToRotationFactor) (Utilities|Time|GetWorldDeltaSeconds)))))

(event Input|AxisEvents|InputAxisLookRight
  (params (AxisValue :type Float%20%28single-precision%29))
  (Transformation|AddRelativeRotation (Variables|Default|GetSpringArm) (Math|Rotator|MakeRotator 0.0 0.0 AxisValue) false false))

(event Input|AxisEvents|InputAxisLookUp
  (params (AxisValue :type Float%20%28single-precision%29))
  (Transformation|AddRelativeRotation (Variables|Default|GetSpringArm) (Math|Rotator|MakeRotator 0.0 AxisValue 0.0) false false))

(fn ConstructionScript)