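; Spawn-obstacle power-up pickup for the hover car game, a child Blueprint that currently adds no behavior of its own.
; Overlap and construction pass straight to the parent class, and its PowerupPickedUp event is empty.
; Disconnected logic, which never runs, would grant a runner vehicle the Reverse power-up, notify the in-game widget and play the Reverse sound, with no obstacle spawning.
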(event EventPowerupPickedUp)

(event Collision|EventActorBeginOverlap
  (params (OtherActor :type Actor%20Object%20Reference))
  (|CallParentFunction OtherActor))

(fn ConstructionScript
  (|CallParentFunction))