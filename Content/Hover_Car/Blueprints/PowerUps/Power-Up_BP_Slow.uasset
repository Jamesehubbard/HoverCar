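; Slow-down power-up for the hover car game, a child Blueprint that defers overlap and construction to its parent.
; On pickup it flags the first HoverCar_BP found in the level as able to activate the slow-down.
; On activation it calls the slow-down effect on the second car found and plays force feedback for player 0.
; Both cars are chosen by fixed array index, regardless of who triggered the power-up.
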(event EventPowerupPickedUp
  (bind _outactors (Actor|GetAllActorsOfClass "/Game/Hover_Car/Blueprints/HoverCar_BP.HoverCar_BP_C"))
  (bind _ashover_car_bp (Utilities|Casting|CastToHoverCar_BP (Utilities|Array|Get(acopy) _outactors)))
  (Variables|/Game/Hover_Car/Blueprints/HoverCar_BP.HoverCar_BP_C|SetSlow%20Down%20Activatable _ashover_car_bp true))

(event Collision|EventActorBeginOverlap
  (params (OtherActor :type Actor%20Object%20Reference))
  (|CallParentFunction OtherActor))

(event EventPowerUpActivated
  (bind _outactors (Actor|GetAllActorsOfClass "/Game/Hover_Car/Blueprints/HoverCar_BP.HoverCar_BP_C"))
  (bind _ashover_car_bp (Utilities|Casting|CastToHoverCar_BP (Utilities|Array|Get(acopy) _outactors 1)))
  (Default|SlowDownEffect _ashover_car_bp)
  (Game|Feedback|ClientPlayForceFeedback (Game|GetPlayerController 0) "/Game/Hover_Car/Blueprints/FFB_Powerup.FFB_Powerup" "None" false false false))

(fn ConstructionScript
  (|CallParentFunction))