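; Base pickup actor for power-ups in the hover car game, collectible only by runner vehicles not already holding one.
; A box overlap stores the hover vehicle and calls PowerupPickedUp, an empty event that child Blueprints can override.
; After a short delay, it flags the vehicle as holding a power-up and destroys itself.
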(event OnComponentBeginOverlap(Box)
  (params (OverlappedComponent :type Primitive%20Component%20Object%20Reference) (OtherActor :type Actor%20Object%20Reference) (OtherComp :type Primitive%20Component%20Object%20Reference) (OtherBodyIndex :type Integer) (bFromSweep :type Boolean) (SweepResult :type Hit%20Result%20Structure%20%28by%20ref%29))
  (bind _asbp_hover_vehicle (Utilities|Casting|CastToBP_HoverVehicle OtherActor))
  (bind _output_get (Variables|Default|SetAs%20BP%20Hover%20Vehicle _asbp_hover_vehicle))
  (if (Variables|/Game/Hover_Car/Blueprints/BP_HoverVehicle.BP_HoverVehicle_C|GetIs%20Runner _output_get)
    (if (not (Variables|/Game/Hover_Car/Blueprints/BP_HoverVehicle.BP_HoverVehicle_C|GetHolding%20PowerUp _output_get))
      (CallFunction|PowerupPickedUp)
      (Utilities|FlowControl|Delay 0.1)
      (Variables|/Game/Hover_Car/Blueprints/BP_HoverVehicle.BP_HoverVehicle_C|SetHolding%20PowerUp (Variables|Default|GetAs%20BP%20Hover%20Vehicle) true)
      (Actor|DestroyActor))))

(event Custom|Powerup%20Picked%20Up)

(fn ConstructionScript)