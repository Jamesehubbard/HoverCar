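; Reverse-steering power-up pickup for the hover car game, built on a parent power-up Blueprint that receives its overlap events.
; On BeginPlay it creates a dynamic material instance on its skeletal mesh and drives the emissiveness with a timeline.
; When picked up by a runner vehicle, it sets that vehicle's reverse-steering power-up flag and notifies the in-game HUD widget.
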(event EventPowerupPickedUp
  (bind _as_bp_hover_vehicle (Variables|Default|GetAs%20BP%20Hover%20Vehicle))
  (if (Variables|/Game/Hover_Car/Blueprints/Car/BP_HoverVehicle.BP_HoverVehicle_C|GetIs%20Runner _as_bp_hover_vehicle)
    (Variables|/Game/Hover_Car/Blueprints/Car/BP_HoverVehicle.BP_HoverVehicle_C|SetHas%20Reverse%20Steering%20PowerUp _as_bp_hover_vehicle true)
    (bind _foundwidgets (Widget|GetAllWidgetsOfClass "/Game/Hover_Car/UI/InGame/WBP_InGame.WBP_InGame_C" true))
    (Default|ReverseSteeringPower-UpPickedUp (Utilities|Array|Get(acopy) _foundwidgets))))

(event Collision|EventActorBeginOverlap
  (params (OtherActor :type Actor%20Object%20Reference))
  (|CallParentFunction OtherActor))

(event EventBeginPlay
  (bind _returnvalue (Rendering|Material|CreateDynamicMaterialInstance (Variables|Default|GetSkeletalMesh) 0 "/Game/Hover_Car/Assets/PowerUps/Power-Up_Steering_Mat.Power-Up_Steering_Mat" "None" :!class /Script/Engine.PrimitiveComponent))
  (bind _newtrack_0 (Timeline|Timeline PlayFromStart)
    (:Update
      (Rendering|Material|SetScalarParameterValue _returnvalue "Emissiveness" _newtrack_0 :!class /Script/Engine.MaterialInstanceDynamic))))

(fn ConstructionScript
  (|CallParentFunction))