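; Steering power-up pickup for the hover car game, a child Blueprint that hands overlap and construction to its parent.
; On pickup, it acts only if the hover vehicle is the runner, setting that vehicle's steering power-up flag.
; It then notifies the first top-level in-game HUD widget found and plays a 2D sound through a DoOnce gate.
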(event EventPowerupPickedUp
  (bind _as_bp_hover_vehicle (Variables|Default|GetAs%20BP%20Hover%20Vehicle))
  (if (Variables|/Game/Hover_Car/Blueprints/Car/BP_HoverVehicle.BP_HoverVehicle_C|GetIs%20Runner _as_bp_hover_vehicle)
    (Variables|/Game/Hover_Car/Blueprints/Car/BP_HoverVehicle.BP_HoverVehicle_C|SetHas%20Steering%20Power-Up _as_bp_hover_vehicle true)
    (bind _foundwidgets (Widget|GetAllWidgetsOfClass "/Game/Hover_Car/UI/InGame/WBP_InGame.WBP_InGame_C" true))
    (Default|SteeringPower-UpPickedUp (Utilities|Array|Get(acopy) _foundwidgets))
    (Utilities|FlowControl|DoOnce false
      (:Completed
        (Audio|PlaySound2D 0 1.0 1.0 0.0 0 0)))))

(event Collision|EventActorBeginOverlap
  (params (OtherActor :type Actor%20Object%20Reference))
  (|CallParentFunction OtherActor))

(fn ConstructionScript
  (|CallParentFunction))