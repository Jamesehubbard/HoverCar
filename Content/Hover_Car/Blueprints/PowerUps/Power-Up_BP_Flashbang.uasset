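; Flashbang power-up pickup for the hover car game, extending a parent power-up that handles overlap.
; On begin play it creates a dynamic material and animates its emissive glow with a timeline.
; On pickup it flags the vehicle as holding a flashbang and notifies the in-game HUD widget.
; In runner-chaser mode only the runner receives it; otherwise the HUD update targets player one or two.
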(event EventPowerupPickedUp
  (bind _as_bp_hover_vehicle (Variables|Default|GetAs%20BP%20Hover%20Vehicle))
  (if (Variables|/Game/Hover_Car/Blueprints/Engine/HC_Gamemode.HC_Gamemode_C|GetRunner/Chaser (Variables|Default|GetMy_Gamemode))
    (if (Variables|/Game/Hover_Car/Blueprints/Car/BP_HoverVehicle.BP_HoverVehicle_C|GetIs%20Runner _as_bp_hover_vehicle)
      (Variables|/Game/Hover_Car/Blueprints/Car/BP_HoverVehicle.BP_HoverVehicle_C|SetHas%20Flashbang%20PowerUp _as_bp_hover_vehicle true)
      (bind _foundwidgets (Widget|GetAllWidgetsOfClass "/Game/Hover_Car/UI/InGame/WBP_InGame.WBP_InGame_C" true))
      (Default|FlashbangPower-UpPickedUp (Utilities|Array|Get(acopy) _foundwidgets)))
    (elif (Variables|/Game/Hover_Car/Blueprints/Car/BP_HoverVehicle.BP_HoverVehicle_C|GetIs%20Player%201 (Variables|Default|GetAs%20BP%20Hover%20Vehicle))
      (Variables|/Game/Hover_Car/Blueprints/Car/BP_HoverVehicle.BP_HoverVehicle_C|SetHas%20Flashbang%20PowerUp (Variables|Default|GetAs%20BP%20Hover%20Vehicle) true)
      (bind _foundwidgets_2 (Widget|GetAllWidgetsOfClass "/Game/Hover_Car/UI/InGame/WBP_InGame.WBP_InGame_C" true))
      (Default|FlashbangPower-UpPickedUpPlayer1 (Utilities|Array|Get(acopy) _foundwidgets_2))
      (else
        (Variables|/Game/Hover_Car/Blueprints/Car/BP_HoverVehicle.BP_HoverVehicle_C|SetHas%20Flashbang%20PowerUp (Variables|Default|GetAs%20BP%20Hover%20Vehicle) true)
        (bind _foundwidgets_3 (Widget|GetAllWidgetsOfClass "/Game/Hover_Car/UI/InGame/WBP_InGame.WBP_InGame_C" true))
        (Default|FlashbangPower-UpPickedUpPlayer2 (Utilities|Array|Get(acopy) _foundwidgets_3))))))

(event Collision|EventActorBeginOverlap
  (params (OtherActor :type Actor%20Object%20Reference))
  (|CallParentFunction OtherActor))

(event EventBeginPlay
  (bind _returnvalue (Rendering|Material|CreateDynamicMaterialInstance (Variables|Default|GetStaticMesh) 0 "/Game/Hover_Car/Assets/PowerUps/Power-Up_Flashbang_Mat.Power-Up_Flashbang_Mat" "None" :!class /Script/Engine.PrimitiveComponent))
  (bind _newtrack_0 (Timeline|Timeline PlayFromStart)
    (:Update
      (Rendering|Material|SetScalarParameterValue _returnvalue "Emissiveness" _newtrack_0 :!class /Script/Engine.MaterialInstanceDynamic))))

(fn ConstructionScript
  (|CallParentFunction))