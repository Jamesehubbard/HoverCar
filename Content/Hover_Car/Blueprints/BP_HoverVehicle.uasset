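; Player hover car for a two-player chase game, assigned runner or chaser from its starting X position.
; Four corner hover components are initialised; throttle timelines lerp speed and camera offset, and Tick moves the car by unswept world offset.
; Steering applies physics torque toward a target yaw rate.
; Runner power-ups alter the chaser's MaxSpeed, throttle or steering via the gamemode; chasers mash Interact to escape slowdown.
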(event OnComponentHit(Mesh)
  (params (HitComponent :type Primitive%20Component%20Object%20Reference) (OtherActor :type Actor%20Object%20Reference) (OtherComp :type Primitive%20Component%20Object%20Reference) (NormalImpulse :type Vector :default "0, 0, 0") (Hit :type Hit%20Result%20Structure%20%28by%20ref%29))
  (if (not (== OtherActor self))
    (if (not (Actor|ActorHasTag OtherActor "Banked"))
      (if (Components|ComponentHasTag OtherComp "Collision")
        (Variables|Default|SetCurrentSpeed 0.0)))))

(event Custom|Load%20Audio%20Settings
  (CallFunction|LoadSettings (Variables|Default|GetSlotName)))

(event Custom|CustomEvent
  (bind _output_get (Variables|Default|SetElapsed%20TImer (+ 0.1 (Variables|Default|GetElapsed%20TImer))))
  (if (> _output_get (Variables|Default|GetLength%20of%20HD%20Curve))
    (Variables|Default|SetElapsed%20TImer (- (Variables|Default|GetElapsed%20TImer) (Variables|Default|GetLength%20of%20HD%20Curve))))
  (Variables|/Game/Hover_Car/Blueprints/BP_HoverComponent.BP_HoverComponent_C|SetHoverDistance (Variables|Default|GetFL_HoverComponent) (Math|Curves|GetFloatValue (Variables|Default|GetHoverDistanceCurve) (Variables|Default|GetElapsed%20TImer)))
  (Variables|/Game/Hover_Car/Blueprints/BP_HoverComponent.BP_HoverComponent_C|SetHoverDistance (Variables|Default|GetBL_HoverComponent) (Math|Curves|GetFloatValue (Variables|Default|GetHoverDistanceCurve) (Variables|Default|GetElapsed%20TImer)))
  (Variables|/Game/Hover_Car/Blueprints/BP_HoverComponent.BP_HoverComponent_C|SetHoverDistance (Variables|Default|GetFR_HoverComponent) (Math|Curves|GetFloatValue (Variables|Default|GetHoverDistanceCurve) (Variables|Default|GetElapsed%20TImer)))
  (Variables|/Game/Hover_Car/Blueprints/BP_HoverComponent.BP_HoverComponent_C|SetHoverDistance (Variables|Default|GetBR_HoverComponent) (Math|Curves|GetFloatValue (Variables|Default|GetHoverDistanceCurve) (Variables|Default|GetElapsed%20TImer))))

(event Custom|Game%20Loaded
  (bind _ashc_gamemode (Utilities|Casting|CastToHC_Gamemode (Game|GetGameMode)))
  (Variables|Default|SetMy_Gamemode _ashc_gamemode)
  (Input|DisableInput 0)
  (Utilities|FlowControl|Delay 1.0)
  (if (> (.x (Transformation|GetWorldLocation (Variables|Default|GetMesh))) -1e+03)
    (Variables|Default|SetIs%20Runner true)
    (Variables|Default|SetIs%20Chaser false)
    (Variables|Default|SetMaxSpeed 3.5e+03)
    (Utilities|FlowControl|Delay 2.0)
    (Input|EnableInput 0)
    (else
      (Variables|Default|SetIs%20Chaser true)
      (Variables|Default|SetIs%20Runner false)
      (Variables|Default|SetMaxSpeed 1.5e+03)
      (Utilities|FlowControl|Delay 2.0)
      (Input|EnableInput 0)
      (Utilities|FlowControl|Delay 1e+01)
      (Variables|Default|SetMaxSpeed 4e+03))))

(event Custom|Boost
  (Variables|Default|SetCurrentSpeed 55.0))

(event Custom|Set%20Speed%20to%20Normal
  (Variables|Default|SetCurrentSpeed 2.5e+03))

(event Custom|Set%20Speed%20to%200
  (Variables|Default|SetCurrentSpeed 0.0))

(event Input|EnhancedActionEvents|EnhancedInputActionIA_Interact
  (params (ActionValue :type Boolean) (ElapsedSeconds :type Float%20%28double-precision%29) (TriggeredSeconds :type Float%20%28double-precision%29) (InputAction :type Input%20Action%20Object%20Reference :default "/Game/Hover_Car/Input/IA_Interact.IA_Interact"))
  (if (Variables|Default|GetIs%20Runner)
    (if (Variables|Default|GetHas%20Slow%20Power-Up)
      (bind _foundwidgets (Widget|GetAllWidgetsOfClass "/Game/Hover_Car/UI/InGame/WBP_InGame.WBP_InGame_C" true))
      (Default|SlowPower-UpUsed (Utilities|Array|Get(acopy) _foundwidgets))
      (Audio|PlaySound2D "/Game/Hover_Car/Audio/PowerUp_Slow.PowerUp_Slow" 1.0 1.0 0.0 0 0)
      (bind _ashc_gamemode (Utilities|Casting|CastToHC_Gamemode (Game|GetGameMode)))
      (Variables|Default|SetMy_Gamemode _ashc_gamemode)
      (if (Variables|/Game/Hover_Car/Blueprints/Engine/HC_Gamemode.HC_Gamemode_C|GetIsP1Chaser _ashc_gamemode)
        (Variables|BP_HoverVehicle_C|SetMaxSpeed (Variables|/Game/Hover_Car/Blueprints/Engine/HC_Gamemode.HC_Gamemode_C|GetPlayer1 (Variables|Default|GetMy_Gamemode)) 1e+02)
        (Variables|BP_HoverVehicle_C|SetSlow%20Down%20Effect%20Active (Variables|/Game/Hover_Car/Blueprints/Engine/HC_Gamemode.HC_Gamemode_C|GetPlayer1 (Variables|Default|GetMy_Gamemode)) true)
        (Variables|BP_HoverVehicle_C|SetHas%20Slow%20Power-Up (Variables|/Game/Hover_Car/Blueprints/Engine/HC_Gamemode.HC_Gamemode_C|GetPlayer2 (Variables|Default|GetMy_Gamemode)) false)
        (else
          (Variables|BP_HoverVehicle_C|SetMaxSpeed (Variables|/Game/Hover_Car/Blueprints/Engine/HC_Gamemode.HC_Gamemode_C|GetPlayer2 (Variables|Default|GetMy_Gamemode)) 1e+02)
          (Variables|BP_HoverVehicle_C|SetSlow%20Down%20Effect%20Active (Variables|/Game/Hover_Car/Blueprints/Engine/HC_Gamemode.HC_Gamemode_C|GetPlayer2 (Variables|Default|GetMy_Gamemode)) true)
          (Variables|BP_HoverVehicle_C|SetHas%20Slow%20Power-Up (Variables|/Game/Hover_Car/Blueprints/Engine/HC_Gamemode.HC_Gamemode_C|GetPlayer1 (Variables|Default|GetMy_Gamemode)) false)))
      (elif (Variables|Default|GetHas%20Reverse%20Power-Up)
        (bind _foundwidgets_2 (Widget|GetAllWidgetsOfClass "/Game/Hover_Car/UI/InGame/WBP_InGame.WBP_InGame_C" true))
        (Default|ReversePower-UpUsed (Utilities|Array|Get(acopy) _foundwidgets_2))
        (Audio|PlaySound2D "/Game/Hover_Car/Audio/PowerUp_Reverse.PowerUp_Reverse" 1.0 1.0 0.0 0 0)
        (bind _ashc_gamemode_2 (Utilities|Casting|CastToHC_Gamemode (Game|GetGameMode)))
        (Variables|Default|SetMy_Gamemode _ashc_gamemode_2)
        (if (Variables|/Game/Hover_Car/Blueprints/Engine/HC_Gamemode.HC_Gamemode_C|GetIsP1Chaser _ashc_gamemode_2)
          (Variables|BP_HoverVehicle_C|SetThrottle%20Axis (Variables|/Game/Hover_Car/Blueprints/Engine/HC_Gamemode.HC_Gamemode_C|GetPlayer1 (Variables|Default|GetMy_Gamemode)) -1.0)
          (Variables|BP_HoverVehicle_C|SetHas%20Reverse%20Power-Up (Variables|/Game/Hover_Car/Blueprints/Engine/HC_Gamemode.HC_Gamemode_C|GetPlayer2 (Variables|Default|GetMy_Gamemode)) false)
          (Utilities|FlowControl|Delay 3.0)
          (Variables|BP_HoverVehicle_C|SetThrottle%20Axis (Variables|/Game/Hover_Car/Blueprints/Engine/HC_Gamemode.HC_Gamemode_C|GetPlayer1 (Variables|Default|GetMy_Gamemode)) 1.0)
          (else
            (Variables|BP_HoverVehicle_C|SetThrottle%20Axis (Variables|/Game/Hover_Car/Blueprints/Engine/HC_Gamemode.HC_Gamemode_C|GetPlayer2 (Variables|Default|GetMy_Gamemode)) -1.0)
            (Variables|BP_HoverVehicle_C|SetHas%20Reverse%20Power-Up (Variables|/Game/Hover_Car/Blueprints/Engine/HC_Gamemode.HC_Gamemode_C|GetPlayer1 (Variables|Default|GetMy_Gamemode)) false)
            (Utilities|FlowControl|Delay 3.0)
            (Variables|BP_HoverVehicle_C|SetThrottle%20Axis (Variables|/Game/Hover_Car/Blueprints/Engine/HC_Gamemode.HC_Gamemode_C|GetPlayer2 (Variables|Default|GetMy_Gamemode)) 1.0)))
        (elif (Variables|Default|GetHas%20Steering%20Power-Up)
          (bind _foundwidgets_3 (Widget|GetAllWidgetsOfClass "/Game/Hover_Car/UI/InGame/WBP_InGame.WBP_InGame_C" true))
          (Default|SteeringPower-UpUsed (Utilities|Array|Get(acopy) _foundwidgets_3))
          (Audio|PlaySound2D 0 1.0 1.0 0.0 0 0)
          (bind _ashc_gamemode_3 (Utilities|Casting|CastToHC_Gamemode (Game|GetGameMode)))
          (Variables|Default|SetMy_Gamemode _ashc_gamemode_3)
          (if (Variables|/Game/Hover_Car/Blueprints/Engine/HC_Gamemode.HC_Gamemode_C|GetIsP1Chaser _ashc_gamemode_3)
            (Variables|BP_HoverVehicle_C|SetSteer%20Axis (Variables|/Game/Hover_Car/Blueprints/Engine/HC_Gamemode.HC_Gamemode_C|GetPlayer1 (Variables|Default|GetMy_Gamemode)) 5.0)
            (Variables|Default|SetHas%20Steering%20Power-Up (Variables|/Game/Hover_Car/Blueprints/Engine/HC_Gamemode.HC_Gamemode_C|GetPlayer2 (Variables|Default|GetMy_Gamemode)) false)
            (Utilities|FlowControl|Delay 3.0)
            (Variables|Default|SetSteer%20Axis (Variables|/Game/Hover_Car/Blueprints/Engine/HC_Gamemode.HC_Gamemode_C|GetPlayer1 (Variables|Default|GetMy_Gamemode)) 1.0)
            (else
              (Variables|Default|SetSteer%20Axis (Variables|/Game/Hover_Car/Blueprints/Engine/HC_Gamemode.HC_Gamemode_C|GetPlayer2 (Variables|Default|GetMy_Gamemode)) 5.0)
              (Variables|Default|SetHas%20Steering%20Power-Up (Variables|/Game/Hover_Car/Blueprints/Engine/HC_Gamemode.HC_Gamemode_C|GetPlayer1 (Variables|Default|GetMy_Gamemode)) false)
              (Utilities|FlowControl|Delay 3.0)
              (Variables|Default|SetSteer%20Axis (Variables|/Game/Hover_Car/Blueprints/Engine/HC_Gamemode.HC_Gamemode_C|GetPlayer2 (Variables|Default|GetMy_Gamemode)) 0.0))))))
    (elif (Variables|Default|GetSlow%20Down%20Effect%20Active)
      (Math|Integer|IncrementInt (Variables|Default|GetA%20Button%20Pressed)
        (:%20%20
          (if (> (Variables|Default|GetA%20Button%20Pressed) (Math|Random|RandomIntegerinRange 5 8))
            (Variables|Default|SetMaxSpeed 2.5e+03)
            (Variables|Default|SetA%20Button%20Pressed 0)
            (Variables|Default|SetSlow%20Down%20Effect%20Active false)))))))

(event Input|EnhancedActionEvents|EnhancedInputActionIA_Pause
  (params (ActionValue :type Boolean) (ElapsedSeconds :type Float%20%28double-precision%29) (TriggeredSeconds :type Float%20%28double-precision%29) (InputAction :type Input%20Action%20Object%20Reference :default "/Game/Hover_Car/Input/IA_Pause.IA_Pause"))
  (bind _returnvalue (UserInterface|CreateWidget "/Game/Hover_Car/UI/Menus/WBP_HoverCar_PausedMenu.WBP_HoverCar_PausedMenu_C"))
  (Input|SetInputModeUIOnly (Game|GetPlayerController 0) _returnvalue "DoNotLock" false)
  (UserInterface|Viewport|AddtoViewport _returnvalue 0))

(event Input|EnhancedActionEvents|EnhancedInputActionIA_Boost
  (params (ActionValue :type Boolean) (ElapsedSeconds :type Float%20%28double-precision%29) (TriggeredSeconds :type Float%20%28double-precision%29) (InputAction :type Input%20Action%20Object%20Reference :default "/Game/Hover_Car/Input/IA_Boost.IA_Boost"))
  (Variables|Default|SetCurrentSpeed 55.0))

(event Input|EnhancedActionEvents|EnhancedInputActionIA_ForwardMovement
  (params (ActionValue :type Vector%202D%20Structure) (ElapsedSeconds :type Float%20%28double-precision%29) (TriggeredSeconds :type Float%20%28double-precision%29) (InputAction :type Input%20Action%20Object%20Reference :default "/Game/Hover_Car/Input/IA_ForwardMovement.IA_ForwardMovement"))
  (:Triggered
    (Variables|Default|SetGoing%20Forwards true)
    (bind _newtrack_0 (Timeline|Forward%20Throttle%20Add%20Speed PlayFromStart)
      (:Update
        (Audio|Components|Audio|Stop (Variables|Default|GetForward%20Throttle%20Subtract%20Speed))
        (Audio|Components|Audio|Stop (Variables|Default|GetBackwards%20Throttle%20Subtract%20Speed))
        (Variables|Default|SetCurrentSpeed (Math|Float|Lerp (Variables|Default|GetCurrentSpeed) 5e+01 _newtrack_0))
        (Variables|Default|SetThrottle%20Axis 1.0)
        (Variables|Default|SetSteer%20Axis 1.0)
        (Variables|/Script/Engine.SpringArmComponent|SetSocketOffset (Variables|Default|GetSpringArm) (Math|Vector|Lerp(Vector) (Variables|/Script/Engine.SpringArmComponent|GetSocketOffset (Variables|Default|GetSpringArm)) "-400.000000,0.000000,100.000000" _newtrack_0)))))
  (:Completed
    (Audio|Components|Audio|Stop (Variables|Default|GetForward%20Throttle%20Add%20Speed))
    (Audio|Components|Audio|Stop (Variables|Default|GetBackwards%20Throttle%20Subtract%20Speed))
    (bind _newtrack_0_2 (Timeline|Forward%20Throttle%20Subtract%20Speed PlayFromStart)
      (:Update
        (Variables|Default|SetCurrentSpeed (Math|Float|Lerp (Variables|Default|GetCurrentSpeed) 0.0 _newtrack_0_2))
        (if (not (Variables|Default|GetBlock%20Forward))
          (Variables|Default|SetSteer%20Axis 1.0))))))

(event Input|EnhancedActionEvents|EnhancedInputActionIA_BackwardsMovement
  (params (ActionValue :type Vector%202D%20Structure) (ElapsedSeconds :type Float%20%28double-precision%29) (TriggeredSeconds :type Float%20%28double-precision%29) (InputAction :type Input%20Action%20Object%20Reference :default "/Game/Hover_Car/Input/IA_BackwardsMovement.IA_BackwardsMovement"))
  (:Triggered
    (if (> (Variables|Default|GetCurrentSpeed) 5.0)
      (Utilities|FlowControl|Delay (/ (Variables|Default|GetCurrentSpeed) 1e+01))
      (Variables|Default|SetGoing%20Forwards false)
      (else
        (Variables|Default|SetGoing%20Forwards true)
        (Audio|Components|Audio|Stop (Variables|Default|GetForward%20Throttle%20Add%20Speed))
        (Audio|Components|Audio|Stop (Variables|Default|GetForward%20Throttle%20Subtract%20Speed))
        (Audio|Components|Audio|Stop (Variables|Default|GetBackwards%20Throttle%20Subtract%20Speed))
        (Audio|Components|Audio|Stop (Variables|Default|GetForward%20Throttle%20Subtract%20Speed))
        (Audio|Components|Audio|Stop (Variables|Default|GetForward%20Throttle%20Add%20Speed))
        (bind _newtrack_0 (Timeline|Backwards%20Throttle%20Subtract%20Speed PlayFromStart)
          (:Update
            (Variables|Default|SetCurrentSpeed (Math|Float|Lerp (Variables|Default|GetCurrentSpeed) 0.0 _newtrack_0))
            (Variables|Default|SetThrottle%20Axis -1.0)
            (Variables|Default|SetSteer%20Axis -1.0)
            (Variables|/Script/Engine.SpringArmComponent|SetSocketOffset (Variables|Default|GetSpringArm) (Math|Vector|Lerp(Vector) (Variables|/Script/Engine.SpringArmComponent|GetSocketOffset (Variables|Default|GetSpringArm)) "-200.000000,0.000000,250.000000" _newtrack_0)))))))
  (:Completed
    (bind _newtrack_0_2 (Timeline|Timeline PlayFromStart)
      (:Update
        (Variables|/Script/Engine.SpringArmComponent|SetSocketOffset (Variables|Default|GetSpringArm) (Math|Vector|Lerp(Vector) (Variables|/Script/Engine.SpringArmComponent|GetSocketOffset (Variables|Default|GetSpringArm)) "-200.000000,0.000000,250.000000" _newtrack_0_2))))))

(event Input|EnhancedActionEvents|EnhancedInputActionIA_Steering
  (params (ActionValue :type Vector%202D%20Structure) (ElapsedSeconds :type Float%20%28double-precision%29) (TriggeredSeconds :type Float%20%28double-precision%29) (InputAction :type Input%20Action%20Object%20Reference :default "/Game/Hover_Car/Input/IA_Steering.IA_Steering"))
  (bind _mesh (Variables|Default|GetMesh))
  (bind _mesh_2 (Variables|Default|GetMesh))
  (Variables|Default|SetTargetAngularSpeed (* (* (.x ActionValue) (Variables|Default|GetSteer%20Axis)) 5e+08))
  (Variables|Default|SetCurrentAngularSpeed (Math|Vector|DotProduct (Physics|GetPhysicsAngularVelocityinDegrees _mesh_2 "None") (Math|Vector|GetUpVector _mesh_2)))
  (Class|PrimitiveComponent|AddTorqueinDegrees _mesh (* (Math|Vector|GetUpVector _mesh) (* (- (Variables|Default|GetTargetAngularSpeed) (Variables|Default|GetCurrentAngularSpeed)) (Variables|Default|GetAngularSpeedToTorqueFactor))) "None" false))

(event EventTick
  (params (DeltaSeconds :type Float%20%28single-precision%29))
  (Utilities|FlowControl|Sequence
    (:then_0
      (if (Variables|Default|GetGoing%20Forwards)
        (CallFunction|Movement)))))

(event EventBeginPlay
  (Utilities|FlowControl|Sequence
    (:then_0
      (Default|Initialise (Variables|Default|GetFR_HoverComponent)))
    (:then_1
      (Input|AddMappingContext (PlayerController|LocalPlayerSubsystems|GetEnhancedInputLocalPlayerSubsystem (Game|GetPlayerController 0)) "/Game/Hover_Car/Input/IMC_HoverCar.IMC_HoverCar" 0 "(bIgnoreAllPressedKeysUntilRelease=True,bForceImmediately=False,bNotifyUserSettings=False)"))))

(fn ConstructionScript)

(fn Movement
  (Transformation|AddActorWorldOffset (* (Transformation|GetActorForwardVector) (* (Variables|Default|GetCurrentSpeed) (Variables|Default|GetThrottle%20Axis)))))

(fn LoadSettings
  (params (SlotName :type String)))