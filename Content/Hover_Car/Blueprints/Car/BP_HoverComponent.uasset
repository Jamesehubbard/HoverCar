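; Hover suspension component for BP_HoverVehicle that pushes the car off the surface beneath it.
; Each tick, a downward line trace drives a spring-damper force applied at the component's location.
; The trace also toggles the vehicle's airborne state, linear damping and mid-air slowdown, while surface tags flag humps (setting hover distance) and banking.
; A debug check prints wrong/correct way by comparing the vehicle arrow's yaw with the Floor_BP arrow's pitch.
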(event Custom|Initialise
  (bind _asbp_hover_vehicle (Utilities|Casting|CastToBP_HoverVehicle (Components|GetOwner)))
  (Variables|Default|SetParentVehicle _asbp_hover_vehicle))

(event EventTick
  (params (DeltaSeconds :type Float%20%28single-precision%29))
  (bind _returnvalue (Transformation|GetWorldLocation))
  (bind _parentvehicle (Variables|Default|GetParentVehicle))
  (bind _parentvehicle_2 (Variables|Default|GetParentVehicle))
  (Utilities|IsValid (Variables|Default|GetParentVehicle)
    (:Is%20Valid
      (bind (_outhit _returnvalue_2) (Collision|LineTraceByChannel _returnvalue (- _returnvalue (* (Math|Vector|GetUpVector) (Variables|Default|GetHoverDistance))) "TraceTypeQuery1" false 0 "None"))
      (Variables|Default|SetOut%20Hit _outhit)
      (CallFunction|NewFunction)
      (if _returnvalue_2
        (Variables|/Game/Hover_Car/Blueprints/Car/BP_HoverVehicle.BP_HoverVehicle_C|SetIsInAir _parentvehicle_2 false)
        (Variables|/Game/Hover_Car/Blueprints/Car/BP_HoverVehicle.BP_HoverVehicle_C|SetStop%20MidAir%20Speed%20SlowDown _parentvehicle_2 true)
        (if (Actor|ActorHasTag (.HitActor (Collision|BreakHitResult (Variables|Default|GetOut%20Hit))) "Ump")
          (Variables|Default|SetHoverDistance 2e+02)
          (Variables|/Game/Hover_Car/Blueprints/Car/BP_HoverVehicle.BP_HoverVehicle_C|SetGoingOverHump (Variables|Default|GetParentVehicle) true)
          (else
            (Variables|/Game/Hover_Car/Blueprints/Car/BP_HoverVehicle.BP_HoverVehicle_C|SetGoingOverHump (Variables|Default|GetParentVehicle) false)))
        (if (Actor|ActorHasTag (.HitActor (Collision|BreakHitResult (Variables|Default|GetOut%20Hit))) "Banked")
          (Variables|Default|SetDont%20Roll true)
          (else
            (Variables|Default|SetDont%20Roll false)))
        (Class|PrimitiveComponent|SetLinearDamping (Variables|/Game/Hover_Car/Blueprints/Car/BP_HoverVehicle.BP_HoverVehicle_C|GetMesh (Variables|Default|GetParentVehicle)) 5.0)
        (bind _output_get (Variables|Default|SetHoverDelta (- (Variables|Default|GetHoverDistance) (.Distance (Collision|BreakHitResult (Variables|Default|GetOut%20Hit))))))
        (bind _asprimitive_component (Utilities|Casting|CastToPrimitiveComponent (Variables|/Script/Engine.Actor|GetRootComponent (Variables|Default|GetParentVehicle))))
        (Class|PrimitiveComponent|AddForceatLocation _asprimitive_component (* (Math|Vector|GetUpVector) (+ (* (/ (- _output_get (Variables|Default|GetPrevious%20Hover%20Delta)) (Utilities|Time|GetWorldDeltaSeconds)) (Variables|Default|GetDampingCoefficent)) (* _output_get (Variables|Default|GetSpringCoefficent)))) (Transformation|GetWorldLocation) "None")
        (Variables|Default|SetPrevious%20Hover%20Delta (Variables|Default|GetHoverDelta))
        (else
          (Class|PrimitiveComponent|SetLinearDamping (Variables|/Game/Hover_Car/Blueprints/Car/BP_HoverVehicle.BP_HoverVehicle_C|GetMesh (Variables|Default|GetParentVehicle)) 0.01)
          (Variables|/Game/Hover_Car/Blueprints/Car/BP_HoverVehicle.BP_HoverVehicle_C|SetIsInAir (Variables|Default|GetParentVehicle) true)
          (Default|MidAirSlowCurrentSpeed _parentvehicle)
          (Variables|/Game/Hover_Car/Blueprints/Car/BP_HoverVehicle.BP_HoverVehicle_C|SetStop%20MidAir%20Speed%20SlowDown _parentvehicle false))))))

(fn NewFunction
  (bind _parentvehicle (Variables|Default|GetParentVehicle))
  (bind _arrow (Variables|/Game/Hover_Car/Blueprints/Car/BP_HoverVehicle.BP_HoverVehicle_C|GetArrow _parentvehicle))
  (bind _returnvalue (Transformation|GetWorldRotation _arrow))
  (LocalVariables|SetNewLocalVar 0)
  (bind _asfloor_bp (Utilities|Casting|CastToFloor_BP (.HitActor (Collision|BreakHitResult (Variables|Default|GetOut%20Hit)))))
  (Development|PrintString (Utilities|String|ToString(Float) (.yaw _returnvalue)))
  (Development|PrintString (Utilities|String|ToString(Rotator) (Transformation|GetWorldRotation (Variables|/Game/Hover_Car/Blueprints/Track/Straight/Floor_BP.Floor_BP_C|GetArrow _asfloor_bp))))
  (if (or (<= (.yaw _returnvalue) (- (.pitch (Transformation|GetWorldRotation (Variables|/Game/Hover_Car/Blueprints/Track/Straight/Floor_BP.Floor_BP_C|GetArrow _asfloor_bp))) 1.2e+02)) (>= (.yaw _returnvalue) (+ (.pitch (Transformation|GetWorldRotation (Variables|/Game/Hover_Car/Blueprints/Track/Straight/Floor_BP.Floor_BP_C|GetArrow _asfloor_bp))) 1.2e+02)))
    (Development|PrintString "WRONG WAY" true true "(R=1.000000,G=0.889432,B=0.000000,A=1.000000)")
    (else
      (Development|PrintString "CORRECT WAY" true true "(R=1.000000,G=0.889432,B=0.000000,A=1.000000)"))))