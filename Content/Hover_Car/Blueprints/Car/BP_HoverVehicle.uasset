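; Player hover car for a two-player runner-versus-chaser game, assigning its role from starting X position on game load.
; Input adjusts a speed value that drives swept forward offsets, camera FOV and engine audio, while steering applies torque and banking roll.
; Four hover components float the car with timeline-driven height.
; Interact fires the runner's held power-up against the chaser, or lets the chaser boost or mash out of slowdowns; collisions kill speed.
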(event OnComponentHit(Mesh)
  (params (HitComponent :type Primitive%20Component%20Object%20Reference) (OtherActor :type Actor%20Object%20Reference) (OtherComp :type Primitive%20Component%20Object%20Reference) (NormalImpulse :type Vector :default "0, 0, 0") (Hit :type Hit%20Result%20Structure%20%28by%20ref%29))
  (if (not (== OtherActor self))
    (if (not (Actor|ActorHasTag OtherActor "Banked"))
      (if (Components|ComponentHasTag OtherComp "Collision")
        (if (Variables|Default|GetBoost%20Available)
          (bind _foundwidgets (Widget|GetAllWidgetsOfClass "/Game/Hover_Car/UI/InGame/WBP_InGame.WBP_InGame_C" true))
          (bind _aswbp_in_game (Utilities|Casting|CastToWBP_InGame (Utilities|Array|Get(acopy) _foundwidgets)))
          (Rendering|Components|TextRender|SetText (Variables|/Game/Hover_Car/UI/InGame/WBP_InGame.WBP_InGame_C|GetBoostAvailableText _aswbp_in_game) "Boost Pads Activated ")
          (Variables|/Script/UMG.Widget|SetVisibility (Variables|/Game/Hover_Car/UI/InGame/WBP_InGame.WBP_InGame_C|GetBoostAvailableText _aswbp_in_game) "Visible"))
        (Variables|Default|SetBoost%20Available false)
        (Variables|Default|SetCurrentSpeed 0.0)
        (Variables|Default|SetBoosting false)
        (Variables|Default|SetSpeed%20Increase 0.1)
        (Variables|Default|SetMax%20Field%20of%20View 1.1e+02)))))

(event Custom|Load%20Audio%20Settings
  (CallFunction|LoadSettings (Variables|Default|GetSlotName)))

(event Custom|CustomEvent
  (params (CurrentDevice :type String))
  (Development|PrintString "Hello" true true "(R=0.000000,G=0.660000,B=1.000000,A=1.000000)" 1e+02))

(event Custom|Game%20Loaded
  (CallFunction|VerticalMovement)
  (bind _ashc_gamemode (Utilities|Casting|CastToHC_Gamemode (Game|GetGameMode)))
  (Variables|Default|SetMy_Gamemode _ashc_gamemode)
  (Input|DisableInput 0)
  (Utilities|FlowControl|Delay 1.0)
  (if (> (.x (Transformation|GetWorldLocation (Variables|Default|GetMesh))) -1e+03)
    (Variables|Default|SetIs%20Runner true)
    (Variables|Default|SetIs%20Chaser false)
    (Variables|Default|SetPlayer%20Index 0)
    (Variables|Default|SetMaxSpeed 5e+01)
    (Utilities|FlowControl|Delay 2.0)
    (Input|EnableInput 0)
    (Components|Activation|Deactivate (Variables|Default|GetMS_Engine_Right))
    (else
      (Variables|Default|SetIs%20Chaser true)
      (Variables|Default|SetIs%20Runner false)
      (Variables|Default|SetPlayer%20Index 1)
      (Variables|Default|SetMaxSpeed 4e+01)
      (Utilities|FlowControl|Delay 2.0)
      (Input|EnableInput 0)
      (Components|Activation|Deactivate (Variables|Default|GetMS_Engine_Left))
      (Utilities|FlowControl|Delay 1e+01)
      (Variables|Default|SetMaxSpeed 6e+01))))

(event Custom|Boost
  (Variables|Default|SetSpeed%20Increase 1.0)
  (Variables|Default|SetBoosting true)
  (Variables|Default|SetMaxSpeed 55.0)
  (Variables|Default|SetMax%20Field%20of%20View (Math|Float|Clamp(Float) (+ (Variables|Default|GetMax%20Field%20of%20View) 1.0) 1.1e+02 1.2e+02)))

(event Custom|Set%20Speed%20to%20Normal
  (Variables|Default|SetCurrentSpeed (Variables|Default|GetMaxSpeed)))

(event Custom|Set%20Speed%20to%200
  (Variables|Default|SetCurrentSpeed (Variables|Default|GetMin%20Speed)))

(event Custom|Slow%20Current%20Speed
  (if (not (Variables|Default|GetStop%20Speed%20SlowDown)) :!label _label
    (Variables|Default|SetCurrentSpeed (Math|Float|Clamp(Float) (- (Variables|Default|GetCurrentSpeed) 0.25) (Variables|Default|GetMin%20Speed) (Variables|Default|GetMaxSpeed)))
    (Variables|/Script/Engine.SpringArmComponent|SetSocketOffset (Variables|Default|GetSpringArm) (Math|Vector|MakeVector (.x (Variables|/Script/Engine.SpringArmComponent|GetSocketOffset (Variables|Default|GetSpringArm))) (.y (Variables|/Script/Engine.SpringArmComponent|GetSocketOffset (Variables|Default|GetSpringArm))) (Math|Float|Clamp(Float) (+ (.z (Variables|/Script/Engine.SpringArmComponent|GetSocketOffset (Variables|Default|GetSpringArm))) 1.0) 1.5e+02 2.5e+02)))
    (Utilities|FlowControl|Delay 0.01)
    (goto _label)))

(event Custom|MidAir%20Slow%20Current%20Speed
  (if (not (Variables|Default|GetStop%20MidAir%20Speed%20SlowDown)) :!label _label
    (Variables|Default|SetCurrentSpeed (Math|Float|Clamp(Float) (- (Variables|Default|GetCurrentSpeed) 0.05) (Variables|Default|GetMin%20Speed) (Variables|Default|GetMaxSpeed)))
    (Utilities|FlowControl|Delay 0.01)
    (goto _label)))

(event Custom|Vertical%20Movement
  (bind _newtrack_0 (Timeline|Timeline PlayFromStart)
    (:Update
      (if (not (Variables|Default|GetGoingOverHump))
        (Variables|/Game/Hover_Car/Blueprints/Car/BP_HoverComponent.BP_HoverComponent_C|SetHoverDistance (Variables|Default|GetFL_HoverComponent) _newtrack_0)
        (Variables|/Game/Hover_Car/Blueprints/Car/BP_HoverComponent.BP_HoverComponent_C|SetHoverDistance (Variables|Default|GetBR_HoverComponent) _newtrack_0)
        (Variables|/Game/Hover_Car/Blueprints/Car/BP_HoverComponent.BP_HoverComponent_C|SetHoverDistance (Variables|Default|GetFR_HoverComponent) _newtrack_0)
        (Variables|/Game/Hover_Car/Blueprints/Car/BP_HoverComponent.BP_HoverComponent_C|SetHoverDistance (Variables|Default|GetBL_HoverComponent) _newtrack_0)))))

(event Input|EnhancedActionEvents|EnhancedInputActionIA_Interact
  (params (ActionValue :type Boolean) (ElapsedSeconds :type Float%20%28double-precision%29) (TriggeredSeconds :type Float%20%28double-precision%29) (InputAction :type Input%20Action%20Object%20Reference :default "/Game/Hover_Car/Input/IA_Interact.IA_Interact"))
  (if (Variables|Default|GetIs%20Runner)
    (if (Variables|Default|GetHas%20Slow%20Power-Up)
      (bind _foundwidgets (Widget|GetAllWidgetsOfClass "/Game/Hover_Car/UI/InGame/WBP_InGame.WBP_InGame_C" true))
      (Default|SlowPower-UpUsed (Utilities|Array|Get(acopy) _foundwidgets))
      (Audio|PlaySound2D "/Game/Hover_Car/Audio/PowerUp/PowerUp_Slow.PowerUp_Slow" 1.0 1.0 0.0 0 0)
      (Variables|Default|SetHolding%20PowerUp false)
      (bind _ashc_gamemode (Utilities|Casting|CastToHC_Gamemode (Game|GetGameMode)))
      (Variables|Default|SetMy_Gamemode _ashc_gamemode)
      (if (Variables|/Game/Hover_Car/Blueprints/Engine/HC_Gamemode.HC_Gamemode_C|GetIsP1Chaser _ashc_gamemode)
        (Variables|BP_HoverVehicle_C|SetMaxSpeed (Variables|/Game/Hover_Car/Blueprints/Engine/HC_Gamemode.HC_Gamemode_C|GetPlayer1 (Variables|Default|GetMy_Gamemode)) 1e+02)
        (Variables|BP_HoverVehicle_C|SetSlow%20Down%20Effect%20Active (Variables|/Game/Hover_Car/Blueprints/Engine/HC_Gamemode.HC_Gamemode_C|GetPlayer1 (Variables|Default|GetMy_Gamemode)) true)
        (Variables|BP_HoverVehicle_C|SetHas%20Slow%20Power-Up (Variables|/Game/Hover_Car/Blueprints/Engine/HC_Gamemode.HC_Gamemode_C|GetPlayer2 (Variables|Default|GetMy_Gamemode)) false)
        (else
          (Variables|BP_HoverVehicle_C|SetMaxSpeed (Variables|/Game/Hover_Car/Blueprints/Engine/HC_Gamemode.HC_Gamemode_C|GetPlayer2 (Variables|Default|GetMy_Gamemode)) 1e+02)
          (Variables|BP_HoverVehicle_C|SetSlow%20Down%20Effect%20Active (Variables|/Game/Hover_Car/Blueprints/Engine/HC_Gamemode.HC_Gamemode_C|GetPlayer2 (Variables|Default|GetMy_Gamemode)) true)
          (Variables|BP_HoverVehicle_C|SetHas%20Slow%20Power-Up (Variables|/Game/Hover_Car/Blueprints/Engine/HC_Gamemode.HC_Gamemode_C|GetPlayer1 (Variables|Default|GetMy_Gamemode)) false)))
      (elif (Variables|Default|GetHas%20Reverse%20Power-Up)
        (bind _foundwidgets_2 (Widget|GetAllWidgetsOfClass "/Game/Hover_Car/UI/InGame/WBP_InGame.WBP_InGame_C" true))
        (Default|ReversePower-UpUsed (Utilities|Array|Get(acopy) _foundwidgets_2))
        (Audio|PlaySound2D "/Game/Hover_Car/Audio/PowerUp/PowerUp_Reverse.PowerUp_Reverse" 1.0 1.0 0.0 0 0)
        (Variables|Default|SetHolding%20PowerUp false)
        (bind _ashc_gamemode_2 (Utilities|Casting|CastToHC_Gamemode (Game|GetGameMode)))
        (Variables|Default|SetMy_Gamemode _ashc_gamemode_2)
        (if (Variables|/Game/Hover_Car/Blueprints/Engine/HC_Gamemode.HC_Gamemode_C|GetIsP1Chaser _ashc_gamemode_2)
          (Variables|BP_HoverVehicle_C|SetThrottle%20Axis (Variables|/Game/Hover_Car/Blueprints/Engine/HC_Gamemode.HC_Gamemode_C|GetPlayer1 (Variables|Default|GetMy_Gamemode)) -1.0)
          (Variables|BP_HoverVehicle_C|SetHas%20Reverse%20Power-Up (Variables|/Game/Hover_Car/Blueprints/Engine/HC_Gamemode.HC_Gamemode_C|GetPlayer2 (Variables|Default|GetMy_Gamemode)) false)
          (Utilities|FlowControl|Delay 3.0)
          (Variables|BP_HoverVehicle_C|SetThrottle%20Axis (Variables|/Game/Hover_Car/Blueprints/Engine/HC_Gamemode.HC_Gamemode_C|GetPlayer1 (Variables|Default|GetMy_Gamemode)) 1.0)
          (else
            (Variables|BP_HoverVehicle_C|SetThrottle%20Axis (Variables|/Game/Hover_Car/Blueprints/Engine/HC_Gamemode.HC_Gamemode_C|GetPlayer2 (Variables|Default|GetMy_Gamemode)) -1.0)
            (Variables|BP_HoverVehicle_C|SetHas%20Reverse%20Power-Up (Variables|/Game/Hover_Car/Blueprints/Engine/HC_Gamemode.HC_Gamemode_C|GetPlayer1 (Variables|Default|GetMy_Gamemode)) false)
            (Utilities|FlowControl|Delay 3.0)
            (Variables|BP_HoverVehicle_C|SetThrottle%20Axis (Variables|/Game/Hover_Car/Blueprints/Engine/HC_Gamemode.HC_Gamemode_C|GetPlayer2 (Variables|Default|GetMy_Gamemode)) 1.0)))
        (elif (Variables|Default|GetHas%20Steering%20Power-Up)
          (bind _foundwidgets_3 (Widget|GetAllWidgetsOfClass "/Game/Hover_Car/UI/InGame/WBP_InGame.WBP_InGame_C" true))
          (Default|SteeringPower-UpUsed (Utilities|Array|Get(acopy) _foundwidgets_3))
          (Audio|PlaySound2D "/Game/Hover_Car/Audio/PowerUp/PowerUp_SteeringMulti.PowerUp_SteeringMulti" 1.0 1.0 0.0 0 0)
          (Variables|Default|SetHolding%20PowerUp false)
          (bind _ashc_gamemode_3 (Utilities|Casting|CastToHC_Gamemode (Game|GetGameMode)))
          (Variables|Default|SetMy_Gamemode _ashc_gamemode_3)
          (if (Variables|/Game/Hover_Car/Blueprints/Engine/HC_Gamemode.HC_Gamemode_C|GetIsP1Chaser _ashc_gamemode_3)
            (Variables|BP_HoverVehicle_C|SetSteer%20Axis (Variables|/Game/Hover_Car/Blueprints/Engine/HC_Gamemode.HC_Gamemode_C|GetPlayer1 (Variables|Default|GetMy_Gamemode)) 5.0)
            (Variables|Default|SetHas%20Steering%20Power-Up (Variables|/Game/Hover_Car/Blueprints/Engine/HC_Gamemode.HC_Gamemode_C|GetPlayer2 (Variables|Default|GetMy_Gamemode)) false)
            (Utilities|FlowControl|Delay 3.0)
            (Variables|Default|SetSteer%20Axis (Variables|/Game/Hover_Car/Blueprints/Engine/HC_Gamemode.HC_Gamemode_C|GetPlayer1 (Variables|Default|GetMy_Gamemode)) 1.0)
            (else
              (Variables|Default|SetSteer%20Axis (Variables|/Game/Hover_Car/Blueprints/Engine/HC_Gamemode.HC_Gamemode_C|GetPlayer2 (Variables|Default|GetMy_Gamemode)) 5.0)
              (Variables|Default|SetHas%20Steering%20Power-Up (Variables|/Game/Hover_Car/Blueprints/Engine/HC_Gamemode.HC_Gamemode_C|GetPlayer1 (Variables|Default|GetMy_Gamemode)) false)
              (Utilities|FlowControl|Delay 3.0)
              (Variables|Default|SetSteer%20Axis (Variables|/Game/Hover_Car/Blueprints/Engine/HC_Gamemode.HC_Gamemode_C|GetPlayer2 (Variables|Default|GetMy_Gamemode)) 1.0)))
          (elif (Variables|Default|GetHas%20Reverse%20Steering%20PowerUp)
            (bind _foundwidgets_4 (Widget|GetAllWidgetsOfClass "/Game/Hover_Car/UI/InGame/WBP_InGame.WBP_InGame_C" true))
            (Default|ReverseSteeringPower-UpUsed (Utilities|Array|Get(acopy) _foundwidgets_4))
            (Audio|PlaySound2D 0 1.0 1.0 0.0 0 0)
            (Variables|Default|SetHolding%20PowerUp false)
            (bind _ashc_gamemode_4 (Utilities|Casting|CastToHC_Gamemode (Game|GetGameMode)))
            (Variables|Default|SetMy_Gamemode _ashc_gamemode_4)
            (if (Variables|/Game/Hover_Car/Blueprints/Engine/HC_Gamemode.HC_Gamemode_C|GetIsP1Chaser _ashc_gamemode_4)
              (Variables|BP_HoverVehicle_C|SetSteer%20Axis (Variables|/Game/Hover_Car/Blueprints/Engine/HC_Gamemode.HC_Gamemode_C|GetPlayer1 (Variables|Default|GetMy_Gamemode)) -1.0)
              (Variables|BP_HoverVehicle_C|SetHas%20Reverse%20Steering%20PowerUp (Variables|/Game/Hover_Car/Blueprints/Engine/HC_Gamemode.HC_Gamemode_C|GetPlayer2 (Variables|Default|GetMy_Gamemode)) false)
              (Utilities|FlowControl|Delay 3.0)
              (Variables|Default|SetSteer%20Axis (Variables|/Game/Hover_Car/Blueprints/Engine/HC_Gamemode.HC_Gamemode_C|GetPlayer1 (Variables|Default|GetMy_Gamemode)) 1.0)
              (else
                (Variables|Default|SetSteer%20Axis (Variables|/Game/Hover_Car/Blueprints/Engine/HC_Gamemode.HC_Gamemode_C|GetPlayer2 (Variables|Default|GetMy_Gamemode)) -1.0)
                (Variables|BP_HoverVehicle_C|SetHas%20Reverse%20Steering%20PowerUp (Variables|/Game/Hover_Car/Blueprints/Engine/HC_Gamemode.HC_Gamemode_C|GetPlayer1 (Variables|Default|GetMy_Gamemode)) false)
                (Utilities|FlowControl|Delay 3.0)
                (Variables|Default|SetSteer%20Axis (Variables|/Game/Hover_Car/Blueprints/Engine/HC_Gamemode.HC_Gamemode_C|GetPlayer2 (Variables|Default|GetMy_Gamemode)) 1.0)))
            (elif (Variables|Default|GetHas%20Flashbang%20PowerUp)
              (Utilities|FlowControl|DoOnce false :!label _label
                (:Completed
                  (bind _foundwidgets_5 (Widget|GetAllWidgetsOfClass "/Game/Hover_Car/UI/InGame/WBP_InGame.WBP_InGame_C" true))
                  (Default|FlashbangPower-UpUsed (Utilities|Array|Get(acopy) _foundwidgets_5))
                  (Audio|PlaySound2D 0 1.0 1.0 0.0 0 0)
                  (Variables|Default|SetHolding%20PowerUp false)
                  (bind _ashc_gamemode_5 (Utilities|Casting|CastToHC_Gamemode (Game|GetGameMode)))
                  (Variables|Default|SetMy_Gamemode _ashc_gamemode_5)
                  (if (Variables|/Game/Hover_Car/Blueprints/Engine/HC_Gamemode.HC_Gamemode_C|GetIsP1Chaser _ashc_gamemode_5)
                    (Default|FlashbangPlayer1 (Utilities|Array|Get(acopy) _foundwidgets_5))
                    (Variables|BP_HoverVehicle_C|SetHas%20Flashbang%20PowerUp (Variables|/Game/Hover_Car/Blueprints/Engine/HC_Gamemode.HC_Gamemode_C|GetPlayer2 (Variables|Default|GetMy_Gamemode)) false)
                    (Utilities|FlowControl|Delay 3.0)
                    (goto _label Reset)
                    (else
                      (Default|FlashbangPlayer2 (Utilities|Array|Get(acopy) _foundwidgets_5))
                      (Variables|BP_HoverVehicle_C|SetHas%20Flashbang%20PowerUp (Variables|/Game/Hover_Car/Blueprints/Engine/HC_Gamemode.HC_Gamemode_C|GetPlayer1 (Variables|Default|GetMy_Gamemode)) false)
                      (Utilities|FlowControl|Delay 3.0)
                      (goto _label Reset)))))
              (elif (Variables|Default|GetHas%20SpawnObstacle%20PowerUp)
                (bind _foundwidgets_6 (Widget|GetAllWidgetsOfClass "/Game/Hover_Car/UI/InGame/WBP_InGame.WBP_InGame_C" true))
                (Default|SpawnObstaclePowerUpUsed (Utilities|Array|Get(acopy) _foundwidgets_6))
                (Audio|PlaySound2D 0 1.0 1.0 0.0 0 0)
                (Variables|Default|SetHolding%20PowerUp false)
                (bind _ashc_gamemode_6 (Utilities|Casting|CastToHC_Gamemode (Game|GetGameMode)))
                (Variables|Default|SetMy_Gamemode _ashc_gamemode_6)
                (if (Variables|/Game/Hover_Car/Blueprints/Engine/HC_Gamemode.HC_Gamemode_C|GetIsP1Chaser _ashc_gamemode_6)
                  (Game|SpawnActorfromClass "/Game/Hover_Car/Blueprints/Obstacles/BP_SpawnedObstacle.BP_SpawnedObstacle_C" (Transformation|GetWorldTransform (Variables|BP_HoverVehicle_C|GetObstacle%20Spawn%20location (Variables|/Game/Hover_Car/Blueprints/Engine/HC_Gamemode.HC_Gamemode_C|GetPlayer2 (Variables|Default|GetMy_Gamemode)))) "Undefined" "MultiplyWithRoot" 0 0)
                  (Variables|BP_HoverVehicle_C|SetHas%20SpawnObstacle%20PowerUp (Variables|/Game/Hover_Car/Blueprints/Engine/HC_Gamemode.HC_Gamemode_C|GetPlayer2 (Variables|Default|GetMy_Gamemode)) false)
                  (else
                    (Game|SpawnActorfromClass "/Game/Hover_Car/Blueprints/Obstacles/BP_SpawnedObstacle.BP_SpawnedObstacle_C" (Transformation|GetWorldTransform (Variables|BP_HoverVehicle_C|GetObstacle%20Spawn%20location (Variables|/Game/Hover_Car/Blueprints/Engine/HC_Gamemode.HC_Gamemode_C|GetPlayer1 (Variables|Default|GetMy_Gamemode)))) "Undefined" "MultiplyWithRoot" 0 0)
                    (Variables|BP_HoverVehicle_C|SetHas%20SpawnObstacle%20PowerUp (Variables|/Game/Hover_Car/Blueprints/Engine/HC_Gamemode.HC_Gamemode_C|GetPlayer1 (Variables|Default|GetMy_Gamemode)) false)))))))))
    (elif (Variables|Default|GetBoost%20Available)
      (CallFunction|Boost)
      (bind _foundwidgets_7 (Widget|GetAllWidgetsOfClass "/Game/Hover_Car/UI/InGame/WBP_InGame.WBP_InGame_C" true))
      (bind _aswbp_in_game (Utilities|Casting|CastToWBP_InGame (Utilities|Array|Get(acopy) _foundwidgets_7)))
      (Variables|/Script/UMG.Widget|SetVisibility (Variables|/Game/Hover_Car/UI/InGame/WBP_InGame.WBP_InGame_C|GetBoostAvailableText _aswbp_in_game) "Hidden")
      (elif (Variables|Default|GetSlow%20Down%20Effect%20Active)
        (Math|Integer|IncrementInt (Variables|Default|GetA%20Button%20Pressed)
          (:%20%20
            (if (> (Variables|Default|GetA%20Button%20Pressed) (Math|Random|RandomIntegerinRange 5 8))
              (Variables|Default|SetMaxSpeed 2.5e+03)
              (Variables|Default|SetA%20Button%20Pressed 0)
              (Variables|Default|SetSlow%20Down%20Effect%20Active false))))))))

(event Input|EnhancedActionEvents|EnhancedInputActionIA_Pause
  (params (ActionValue :type Boolean) (ElapsedSeconds :type Float%20%28double-precision%29) (TriggeredSeconds :type Float%20%28double-precision%29) (InputAction :type Input%20Action%20Object%20Reference :default "/Game/Hover_Car/Input/IA_Pause.IA_Pause"))
  (bind _returnvalue (UserInterface|CreateWidget "/Game/Hover_Car/UI/Menus/WBP_HoverCar_PausedMenu.WBP_HoverCar_PausedMenu_C"))
  (Input|SetInputModeUIOnly (Game|GetPlayerController 0) _returnvalue "DoNotLock" false)
  (UserInterface|Viewport|AddtoViewport _returnvalue 0))

(event Input|EnhancedActionEvents|EnhancedInputActionIA_ForwardMovement
  (params (ActionValue :type Vector%202D%20Structure) (ElapsedSeconds :type Float%20%28double-precision%29) (TriggeredSeconds :type Float%20%28double-precision%29) (InputAction :type Input%20Action%20Object%20Reference :default "/Game/Hover_Car/Input/IA_ForwardMovement.IA_ForwardMovement"))
  (:Triggered
    (if (not (Variables|Default|GetIsInAir))
      (Variables|Default|SetStop%20Speed%20SlowDown true)
      (Variables|Default|SetThrottle%20Axis 1.0)
      (Variables|Default|SetSteer%20Axis 1.0)
      (Variables|Default|SetCurrentSpeed (Math|Float|Clamp(Float) (+ (Variables|Default|GetCurrentSpeed) (Variables|Default|GetSpeed%20Increase)) (Variables|Default|GetMin%20Speed) (Variables|Default|GetMaxSpeed)))
      (Variables|/Script/Engine.SpringArmComponent|SetSocketOffset (Variables|Default|GetSpringArm) (Math|Vector|MakeVector (.x (Variables|/Script/Engine.SpringArmComponent|GetSocketOffset (Variables|Default|GetSpringArm))) (.y (Variables|/Script/Engine.SpringArmComponent|GetSocketOffset (Variables|Default|GetSpringArm))) (Math|Float|Clamp(Float) (+ (.z (Variables|/Script/Engine.SpringArmComponent|GetSocketOffset (Variables|Default|GetSpringArm))) -0.5) 1.5e+02 2.5e+02)))))
  (:Completed
    (if (not (Variables|Default|GetBoosting))
      (Variables|Default|SetSteer%20Axis 1.0)
      (Variables|Default|SetStop%20Speed%20SlowDown false)
      (Utilities|FlowControl|Delay 0.2)
      (CallFunction|SlowCurrentSpeed))))

(event Input|EnhancedActionEvents|EnhancedInputActionIA_BackwardsMovement
  (params (ActionValue :type Vector%202D%20Structure) (ElapsedSeconds :type Float%20%28double-precision%29) (TriggeredSeconds :type Float%20%28double-precision%29) (InputAction :type Input%20Action%20Object%20Reference :default "/Game/Hover_Car/Input/IA_BackwardsMovement.IA_BackwardsMovement"))
  (:Triggered
    (if (not (Variables|Default|GetBoosting))
      (if (not (Variables|Default|GetIsInAir))
        (Variables|Default|SetStop%20Speed%20SlowDown true)
        (if (Variables|Default|GetReversing)
          (Variables|Default|SetThrottle%20Axis -1.0)
          (Variables|Default|SetSteer%20Axis -1.0)
          (Variables|Default|SetCurrentSpeed (Math|Float|Clamp(Float) (+ (Variables|Default|GetCurrentSpeed) 0.1) (Variables|Default|GetMin%20Speed) 2e+01))
          (elif (> (Variables|Default|GetCurrentSpeed) 0.2)
            (Variables|Default|SetCurrentSpeed (Math|Float|Clamp(Float) (- (Variables|Default|GetCurrentSpeed) 0.5) (Variables|Default|GetMin%20Speed) (Variables|Default|GetMaxSpeed)))
            (else
              (Variables|Default|SetReversing true)))))))
  (:Completed
    (Variables|Default|SetReversing false)
    (Variables|Default|SetStop%20Speed%20SlowDown false)
    (Utilities|FlowControl|Delay 0.1)
    (CallFunction|SlowCurrentSpeed)))

(event Input|EnhancedActionEvents|EnhancedInputActionIA_Steering
  (params (ActionValue :type Vector%202D%20Structure) (ElapsedSeconds :type Float%20%28double-precision%29) (TriggeredSeconds :type Float%20%28double-precision%29) (InputAction :type Input%20Action%20Object%20Reference :default "/Game/Hover_Car/Input/IA_Steering.IA_Steering"))
  (bind _mesh (Variables|Default|GetMesh))
  (bind _mesh_2 (Variables|Default|GetMesh))
  (bind _mesh_3 (Variables|Default|GetMesh))
  (bind _mesh_4 (Variables|Default|GetMesh))
  (bind _returnvalue (Transformation|GetWorldRotation _mesh))
  (bind _returnvalue_2 (Transformation|GetWorldRotation _mesh_2))
  (Variables|Default|SetTargetAngularSpeed (* (* (.x ActionValue) (Variables|Default|GetSteer%20Axis)) 1.4e+06))
  (Variables|Default|SetCurrentAngularSpeed (Math|Vector|DotProduct (Physics|GetPhysicsAngularVelocityinDegrees _mesh_4 "None") (Math|Vector|GetUpVector _mesh_4)))
  (Class|PrimitiveComponent|AddTorqueinDegrees _mesh_3 (* (Math|Vector|GetUpVector _mesh_3) (* (- (Variables|Default|GetTargetAngularSpeed) (Variables|Default|GetCurrentAngularSpeed)) (Variables|Default|GetAngularSpeedToTorqueFactor))) "None" false)
  (if (Variables|/Game/Hover_Car/Blueprints/Car/BP_HoverComponent.BP_HoverComponent_C|GetDont%20Roll (Variables|Default|GetFL_HoverComponent))
    (Utilities|FlowControl|DoOnce false :!label _label
      (:Completed
        (Transformation|SetWorldRotation (Variables|Default|GetMesh) (Math|Rotator|MakeRotator (Math|Interpolation|FInterpTo (.roll _returnvalue) 0.0 (Utilities|Time|GetWorldDeltaSeconds) 0.2) (.pitch _returnvalue) (.yaw _returnvalue)) false false)))
    (else
      (Utilities|FlowControl|Sequence
        (:then_0
          (goto _label Reset))
        (:then_1
          (Transformation|SetWorldRotation (Variables|Default|GetMesh) (Math|Rotator|MakeRotator (+ (.roll _returnvalue_2) (/ (* (Variables|Default|GetCurrentSpeed) (.x ActionValue)) 75.0)) (.pitch _returnvalue_2) (.yaw _returnvalue_2)) false false))))))

(event EventTick
  (params (DeltaSeconds :type Float%20%28single-precision%29))
  (Utilities|FlowControl|Sequence
    (:then_0
      (CallFunction|Movement DeltaSeconds)
      (Development|PrintString (Class|KismetSystemLibrary|GetDeviceId)))
    (:then_1
      (Variables|/Script/Engine.CameraComponent|SetFieldOfView (Variables|Default|GetCamera) (Math|Float|Clamp(Float) (+ (Variables|Default|GetCurrentSpeed) 9e+01) 9e+01 (Variables|Default|GetMax%20Field%20of%20View))))
    (:then_2
      (Audio|Parameter|SetFloatParameter (Variables|Default|GetMS_Engine_Left) "RPM" (/ (Variables|Default|GetCurrentSpeed) 1e+01) :!class /Script/AudioExtensions.AudioParameterControllerInterface)
      (Audio|Parameter|SetFloatParameter (Variables|Default|GetMS_Engine_Right) "RPM" (/ (Variables|Default|GetCurrentSpeed) 1e+01) :!class /Script/AudioExtensions.AudioParameterControllerInterface))))

(event EventBeginPlay
  (Default|Initialise (Variables|Default|GetFR_HoverComponent)))

(fn ConstructionScript)

(fn Movement
  (params (Delta%20Seconds :type Float%20%28double-precision%29))
  (Transformation|AddActorWorldOffset (* (Transformation|GetActorForwardVector) (* (* (Variables|Default|GetCurrentSpeed) (Variables|Default|GetThrottle%20Axis)) (* Delta%20Seconds 1e+02))) true true))

(fn LoadSettings
  (params (SlotName :type String)))