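; Trap track tile for the hover car game, with randomized roadside buildings and an Arrow transform exposed as an attach point.
; On BeginPlay each of four three-piece building stacks gets a random mesh and sideways offset, while nested random switches hide upper pieces to vary height.
; A runner hover vehicle entering the Box calls ActivateTrap after a half-second delay; that event is empty here.
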(event OnComponentBeginOverlap(Box)
  (params (OverlappedComponent :type Primitive%20Component%20Object%20Reference) (OtherActor :type Actor%20Object%20Reference) (OtherComp :type Primitive%20Component%20Object%20Reference) (OtherBodyIndex :type Integer) (bFromSweep :type Boolean) (SweepResult :type Hit%20Result%20Structure%20%28by%20ref%29))
  (bind _asbp_hover_vehicle (Utilities|Casting|CastToBP_HoverVehicle OtherActor))
  (if (Variables|/Game/Hover_Car/Blueprints/BP_HoverVehicle.BP_HoverVehicle_C|GetIs%20Runner _asbp_hover_vehicle)
    (Utilities|FlowControl|Delay 0.5)
    (CallFunction|ActivateTrap)))

(event Custom|Activate%20Trap)

(event EventBeginPlay
  (bind _building_square_r_02_top (Variables|Default|GetBuilding_Square_R_02_Top))
  (bind _building_square_r_01_top (Variables|Default|GetBuilding_Square_R_01_Top))
  (bind _building_square_l_02_bottom (Variables|Default|GetBuilding_Square_L_02_Bottom))
  (bind _building_square_r_01_bottom (Variables|Default|GetBuilding_Square_R_01_Bottom))
  (bind _building_square_l_01_bottom (Variables|Default|GetBuilding_Square_L_01_Bottom))
  (bind _building_square_l_01_middle (Variables|Default|GetBuilding_Square_L_01_Middle))
  (bind _building_square_l_01_top (Variables|Default|GetBuilding_Square_L_01_Top))
  (bind _building_square_l_02_middle (Variables|Default|GetBuilding_Square_L_02_Middle))
  (bind _building_square_l_02_top (Variables|Default|GetBuilding_Square_L_02_Top))
  (bind _building_square_r_01_middle (Variables|Default|GetBuilding_Square_R_01_Middle))
  (bind _building_square_r_02_bottom (Variables|Default|GetBuilding_Square_R_02_Bottom))
  (bind _building_square_r_02_middle (Variables|Default|GetBuilding_Square_R_02_Middle))
  (bind _relativelocation (Variables|/Script/Engine.SceneComponent|GetRelativeLocation _building_square_l_01_bottom))
  (bind _relativelocation_2 (Variables|/Script/Engine.SceneComponent|GetRelativeLocation _building_square_r_02_top))
  (bind _relativelocation_3 (Variables|/Script/Engine.SceneComponent|GetRelativeLocation _building_square_l_01_middle))
  (bind _relativelocation_4 (Variables|/Script/Engine.SceneComponent|GetRelativeLocation _building_square_l_01_top))
  (bind _relativelocation_5 (Variables|/Script/Engine.SceneComponent|GetRelativeLocation _building_square_l_02_bottom))
  (bind _relativelocation_6 (Variables|/Script/Engine.SceneComponent|GetRelativeLocation _building_square_l_02_middle))
  (bind _relativelocation_7 (Variables|/Script/Engine.SceneComponent|GetRelativeLocation _building_square_l_02_top))
  (bind _relativelocation_8 (Variables|/Script/Engine.SceneComponent|GetRelativeLocation _building_square_r_01_bottom))
  (bind _relativelocation_9 (Variables|/Script/Engine.SceneComponent|GetRelativeLocation _building_square_r_01_middle))
  (bind _relativelocation_10 (Variables|/Script/Engine.SceneComponent|GetRelativeLocation _building_square_r_01_top))
  (bind _relativelocation_11 (Variables|/Script/Engine.SceneComponent|GetRelativeLocation _building_square_r_02_bottom))
  (bind _relativelocation_12 (Variables|/Script/Engine.SceneComponent|GetRelativeLocation _building_square_r_02_middle))
  (Utilities|FlowControl|Sequence
    (:then_0
      (bind _output_get (Variables|Default|SetBuilding%20Square%20L%2001%20Mesh (.OutItem (Utilities|Array|Random (Variables|Default|GetBuilding%20Meshes)))))
      (Components|StaticMesh|SetStaticMesh (Variables|Default|GetBuilding_Square_L_01_Bottom) _output_get)
      (Components|StaticMesh|SetStaticMesh (Variables|Default|GetBuilding_Square_L_01_Top) (Variables|Default|GetBuilding%20Square%20L%2001%20Mesh))
      (Components|StaticMesh|SetStaticMesh (Variables|Default|GetBuilding_Square_L_01_Middle) (Variables|Default|GetBuilding%20Square%20L%2001%20Mesh))
      (bind _output_get_2 (Variables|Default|SetBuilding%20Square%20L%2002%20Mesh (.OutItem (Utilities|Array|Random (Variables|Default|GetBuilding%20Meshes)))))
      (Components|StaticMesh|SetStaticMesh (Variables|Default|GetBuilding_Square_L_02_Bottom) _output_get_2)
      (Components|StaticMesh|SetStaticMesh (Variables|Default|GetBuilding_Square_L_02_Middle) (Variables|Default|GetBuilding%20Square%20L%2002%20Mesh))
      (Components|StaticMesh|SetStaticMesh (Variables|Default|GetBuilding_Square_L_02_Top) (Variables|Default|GetBuilding%20Square%20L%2002%20Mesh))
      (bind _output_get_3 (Variables|Default|SetBuilding%20Square%20R%2001%20Mesh (.OutItem (Utilities|Array|Random (Variables|Default|GetBuilding%20Meshes)))))
      (Components|StaticMesh|SetStaticMesh (Variables|Default|GetBuilding_Square_R_01_Bottom) _output_get_3)
      (Components|StaticMesh|SetStaticMesh (Variables|Default|GetBuilding_Square_R_01_Middle) (Variables|Default|GetBuilding%20Square%20R%2001%20Mesh))
      (Components|StaticMesh|SetStaticMesh (Variables|Default|GetBuilding_Square_R_01_Top) (Variables|Default|GetBuilding%20Square%20R%2001%20Mesh))
      (bind _output_get_4 (Variables|Default|SetBuilding%20Square%20R%2002%20Mesh (.OutItem (Utilities|Array|Random (Variables|Default|GetBuilding%20Meshes)))))
      (Components|StaticMesh|SetStaticMesh (Variables|Default|GetBuilding_Square_R_02_Bottom) _output_get_4)
      (Components|StaticMesh|SetStaticMesh (Variables|Default|GetBuilding_Square_R_02_Middle) (Variables|Default|GetBuilding%20Square%20R%2002%20Mesh))
      (Components|StaticMesh|SetStaticMesh (Variables|Default|GetBuilding_Square_R_02_Top) (Variables|Default|GetBuilding%20Square%20R%2002%20Mesh)))
    (:then_1
      (switch int (Math|Random|RandomIntegerinRange 0 2)
        (:0
          (switch int (Math|Random|RandomIntegerinRange 0 1) :!label _label
            (:0
              (switch int (Math|Random|RandomIntegerinRange 0 2) :!label _label_2
                (:0
                  (switch int (Math|Random|RandomIntegerinRange 0 2) :!label _label_3
                    (:1
                      (Development|SetHiddeninGame (Variables|Default|GetBuilding_Square_L_02_Top) true false))
                    (:2
                      (Development|SetHiddeninGame (Variables|Default|GetBuilding_Square_L_02_Top) true false)
                      (Development|SetHiddeninGame (Variables|Default|GetBuilding_Square_L_02_Middle) true false))))
                (:1
                  (Development|SetHiddeninGame (Variables|Default|GetBuilding_Square_R_02_Top) true false)
                  (goto _label_3))
                (:2
                  (Development|SetHiddeninGame (Variables|Default|GetBuilding_Square_R_02_Top) true false)
                  (Development|SetHiddeninGame (Variables|Default|GetBuilding_Square_R_02_Middle) true false))))
            (:1
              (Development|SetHiddeninGame (Variables|Default|GetBuilding_Square_L_01_Top) true false)
              (goto _label_2))
            (:2
              (Development|SetHiddeninGame (Variables|Default|GetBuilding_Square_L_01_Top) true false)
              (Development|SetHiddeninGame (Variables|Default|GetBuilding_Square_L_01_Middle) true false))))
        (:1
          (Development|SetHiddeninGame (Variables|Default|GetBuilding_Square_R_01_Top) true false)
          (goto _label))
        (:2
          (Development|SetHiddeninGame (Variables|Default|GetBuilding_Square_R_01_Top) true false)
          (Development|SetHiddeninGame (Variables|Default|GetBuilding_Square_R_01_Middle) true false))))
    (:then_2
      (bind _output_get_5 (Variables|Default|SetSquare%20L%2001%20Location (Math|Random|RandomFloatinRange -1e+03 0.0)))
      (Transformation|SetRelativeLocation _building_square_l_01_bottom (Math|Vector|MakeVector (.x _relativelocation) _output_get_5 (.z _relativelocation)) false false)
      (Transformation|SetRelativeLocation _building_square_l_01_middle (Math|Vector|MakeVector (.x _relativelocation_3) (Variables|Default|GetSquare%20L%2001%20Location) (.z _relativelocation_3)) false false)
      (Transformation|SetRelativeLocation _building_square_l_01_top (Math|Vector|MakeVector (.x _relativelocation_4) (Variables|Default|GetSquare%20L%2001%20Location) (.z _relativelocation_4)) false false)
      (bind _output_get_6 (Variables|Default|SetSquare%20L%2002%20Location (Math|Random|RandomFloatinRange -1e+03 0.0)))
      (Transformation|SetRelativeLocation _building_square_l_02_bottom (Math|Vector|MakeVector (.x _relativelocation_5) _output_get_6 (.z _relativelocation_5)) false false)
      (Transformation|SetRelativeLocation _building_square_l_02_middle (Math|Vector|MakeVector (.x _relativelocation_6) (Variables|Default|GetSquare%20L%2002%20Location) (.z _relativelocation_6)) false false)
      (Transformation|SetRelativeLocation _building_square_l_02_top (Math|Vector|MakeVector (.x _relativelocation_7) (Variables|Default|GetSquare%20L%2002%20Location) (.z _relativelocation_7)) false false)
      (bind _output_get_7 (Variables|Default|SetSquare%20R%2001%20Location (Math|Random|RandomFloatinRange 3e+03 4e+03)))
      (Transformation|SetRelativeLocation _building_square_r_01_bottom (Math|Vector|MakeVector (.x _relativelocation_8) _output_get_7 (.z _relativelocation_8)) false false)
      (Transformation|SetRelativeLocation _building_square_r_01_middle (Math|Vector|MakeVector (.x _relativelocation_9) (Variables|Default|GetSquare%20R%2001%20Location) (.z _relativelocation_9)) false false)
      (Transformation|SetRelativeLocation _building_square_r_01_top (Math|Vector|MakeVector (.x _relativelocation_10) (Variables|Default|GetSquare%20R%2001%20Location) (.z _relativelocation_10)) false false)
      (bind _output_get_8 (Variables|Default|SetSquare%20R%2002%20Location (Math|Random|RandomFloatinRange 3e+03 4e+03)))
      (Transformation|SetRelativeLocation _building_square_r_02_bottom (Math|Vector|MakeVector (.x _relativelocation_11) _output_get_8 (.z _relativelocation_11)) false false)
      (Transformation|SetRelativeLocation _building_square_r_02_middle (Math|Vector|MakeVector (.x _relativelocation_12) (Variables|Default|GetSquare%20R%2002%20Location) (.z _relativelocation_12)) false false)
      (Transformation|SetRelativeLocation _building_square_r_02_top (Math|Vector|MakeVector (.x _relativelocation_2) (Variables|Default|GetSquare%20R%2002%20Location) (.z _relativelocation_2)) false false))))

(fn ConstructionScript)

(fn GetAttachPoint
  (return (Transformation|GetWorldTransform (Variables|Default|GetArrow))))