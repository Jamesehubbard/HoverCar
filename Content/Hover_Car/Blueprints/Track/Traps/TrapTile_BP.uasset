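; Track tile for the hover-car game that carries a trap and four randomised roadside buildings, exposing an Arrow transform as its attach point.
; BeginPlay randomises building meshes, materials, sideways offsets and window glow and colour, then after a short delay shifts texture UVs and stacks up to two extra floors.
; When a runner hover vehicle overlaps the Box, a delayed call fires ActivateTrap, an empty event here.
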(event OnComponentBeginOverlap(Box)
  (params (OverlappedComponent :type Primitive%20Component%20Object%20Reference) (OtherActor :type Actor%20Object%20Reference) (OtherComp :type Primitive%20Component%20Object%20Reference) (OtherBodyIndex :type Integer) (bFromSweep :type Boolean) (SweepResult :type Hit%20Result%20Structure%20%28by%20ref%29))
  (bind _asbp_hover_vehicle (Utilities|Casting|CastToBP_HoverVehicle OtherActor))
  (if (Variables|/Game/Hover_Car/Blueprints/Car/BP_HoverVehicle.BP_HoverVehicle_C|GetIs%20Runner _asbp_hover_vehicle)
    (Utilities|FlowControl|Delay 0.5)
    (CallFunction|ActivateTrap)))

(event Custom|Activate%20Trap)

(event EventBeginPlay
  (CallFunction|RandomiseBuildingMeshes)
  (CallFunction|RandomiseBuildingTextures)
  (CallFunction|AddRandomYLocationOffset)
  (CallFunction|RandomWIndowEmissiveness)
  (CallFunction|RandomWindowColour)
  (Utilities|FlowControl|Delay 0.2)
  (CallFunction|RandomiseBuildingUVS)
  (CallFunction|AddRandomBuildingFloors))

(fn ConstructionScript)

(fn GetAttachPoint
  (return (Transformation|GetWorldTransform (Variables|Default|GetArrow))))

(fn RandomiseBuildingMeshes
  (Utilities|FlowControl|DoOnce false
    (:Completed
      (bind _output_get (Variables|Default|SetBuilding_01%20Mesh (.OutItem (Utilities|Array|Random (Variables|Default|GetBuilding%20Meshes)))))
      (Components|StaticMesh|SetStaticMesh (Variables|Default|GetBuilding_01) _output_get)
      (bind _output_get_2 (Variables|Default|SetBuilding_02%20Mesh (.OutItem (Utilities|Array|Random (Variables|Default|GetBuilding%20Meshes)))))
      (Components|StaticMesh|SetStaticMesh (Variables|Default|GetBuilding_02) _output_get_2)
      (bind _output_get_3 (Variables|Default|SetBuilding_03%20Mesh (.OutItem (Utilities|Array|Random (Variables|Default|GetBuilding%20Meshes)))))
      (Components|StaticMesh|SetStaticMesh (Variables|Default|GetBuilding_03) _output_get_3)
      (bind _output_get_4 (Variables|Default|SetBuilding_04%20Mesh (.OutItem (Utilities|Array|Random (Variables|Default|GetBuilding%20Meshes)))))
      (Components|StaticMesh|SetStaticMesh (Variables|Default|GetBuilding_04) _output_get_4))))

(fn RandomiseBuildingTextures
  (Utilities|FlowControl|Sequence
    (:then_0
      (switch int (Math|Random|RandomIntegerinRange 0 3)
        (:0
          (Rendering|Material|SetMaterial (Variables|Default|GetBuilding_01) 0 "/Game/Hover_Car/Assets/Buildings/Materials/Hover_Buildings_Base_Mat.Hover_Buildings_Base_Mat"))
        (:1
          (Rendering|Material|SetMaterial (Variables|Default|GetBuilding_01) 0 "/Game/Hover_Car/Assets/Buildings/Materials/Hover_Buildings_Base2_Mat.Hover_Buildings_Base2_Mat"))
        (:2
          (Rendering|Material|SetMaterial (Variables|Default|GetBuilding_01) 0 "/Game/Hover_Car/Assets/Buildings/Materials/Hover_Buildings_Base3_Mat.Hover_Buildings_Base3_Mat"))
        (:3
          (Rendering|Material|SetMaterial (Variables|Default|GetBuilding_01) 0 "/Game/Hover_Car/Assets/Buildings/Materials/Hover_Buildings_Base4_Mat.Hover_Buildings_Base4_Mat"))))
    (:then_1
      (switch int (Math|Random|RandomIntegerinRange 0 3)
        (:0
          (Rendering|Material|SetMaterial (Variables|Default|GetBuilding_02) 0 "/Game/Hover_Car/Assets/Buildings/Materials/Hover_Buildings_Base_Mat.Hover_Buildings_Base_Mat"))
        (:1
          (Rendering|Material|SetMaterial (Variables|Default|GetBuilding_02) 0 "/Game/Hover_Car/Assets/Buildings/Materials/Hover_Buildings_Base2_Mat.Hover_Buildings_Base2_Mat"))
        (:2
          (Rendering|Material|SetMaterial (Variables|Default|GetBuilding_02) 0 "/Game/Hover_Car/Assets/Buildings/Materials/Hover_Buildings_Base3_Mat.Hover_Buildings_Base3_Mat"))
        (:3
          (Rendering|Material|SetMaterial (Variables|Default|GetBuilding_02) 0 "/Game/Hover_Car/Assets/Buildings/Materials/Hover_Buildings_Base4_Mat.Hover_Buildings_Base4_Mat"))))
    (:then_2
      (switch int (Math|Random|RandomIntegerinRange 0 3)
        (:0
          (Rendering|Material|SetMaterial (Variables|Default|GetBuilding_03) 0 "/Game/Hover_Car/Assets/Buildings/Materials/Hover_Buildings_Base_Mat.Hover_Buildings_Base_Mat"))
        (:1
          (Rendering|Material|SetMaterial (Variables|Default|GetBuilding_03) 0 "/Game/Hover_Car/Assets/Buildings/Materials/Hover_Buildings_Base2_Mat.Hover_Buildings_Base2_Mat"))
        (:2
          (Rendering|Material|SetMaterial (Variables|Default|GetBuilding_03) 0 "/Game/Hover_Car/Assets/Buildings/Materials/Hover_Buildings_Base3_Mat.Hover_Buildings_Base3_Mat"))
        (:3
          (Rendering|Material|SetMaterial (Variables|Default|GetBuilding_03) 0 "/Game/Hover_Car/Assets/Buildings/Materials/Hover_Buildings_Base4_Mat.Hover_Buildings_Base4_Mat"))))
    (:then_3
      (switch int (Math|Random|RandomIntegerinRange 0 3)
        (:0
          (Rendering|Material|SetMaterial (Variables|Default|GetBuilding_04) 0 "/Game/Hover_Car/Assets/Buildings/Materials/Hover_Buildings_Base_Mat.Hover_Buildings_Base_Mat"))
        (:1
          (Rendering|Material|SetMaterial (Variables|Default|GetBuilding_04) 0 "/Game/Hover_Car/Assets/Buildings/Materials/Hover_Buildings_Base2_Mat.Hover_Buildings_Base2_Mat"))
        (:2
          (Rendering|Material|SetMaterial (Variables|Default|GetBuilding_04) 0 "/Game/Hover_Car/Assets/Buildings/Materials/Hover_Buildings_Base3_Mat.Hover_Buildings_Base3_Mat"))
        (:3
          (Rendering|Material|SetMaterial (Variables|Default|GetBuilding_04) 0 "/Game/Hover_Car/Assets/Buildings/Materials/Hover_Buildings_Base4_Mat.Hover_Buildings_Base4_Mat"))))))

(fn AddRandomYLocationOffset
  (bind _building_04 (Variables|Default|GetBuilding_04))
  (bind _building_02 (Variables|Default|GetBuilding_02))
  (bind _building_03 (Variables|Default|GetBuilding_03))
  (bind _building_01 (Variables|Default|GetBuilding_01))
  (bind _relativelocation (Variables|/Script/Engine.SceneComponent|GetRelativeLocation _building_03))
  (bind _relativelocation_2 (Variables|/Script/Engine.SceneComponent|GetRelativeLocation _building_04))
  (bind _relativelocation_3 (Variables|/Script/Engine.SceneComponent|GetRelativeLocation _building_01))
  (bind _relativelocation_4 (Variables|/Script/Engine.SceneComponent|GetRelativeLocation _building_02))
  (Transformation|SetRelativeLocation (Variables|Default|GetBuilding_01) (Math|Vector|MakeVector (.x _relativelocation_3) (- (.y _relativelocation_3) (Math|Random|RandomFloatinRange 1e+03 0.0)) (.z _relativelocation_3)) false false)
  (Transformation|SetRelativeLocation (Variables|Default|GetBuilding_02) (Math|Vector|MakeVector (.x _relativelocation_4) (- (.y _relativelocation_4) (Math|Random|RandomFloatinRange 1e+03 0.0)) (.z _relativelocation_4)) false false)
  (Transformation|SetRelativeLocation (Variables|Default|GetBuilding_03) (Math|Vector|MakeVector (.x _relativelocation) (+ (.y _relativelocation) (Math|Random|RandomFloatinRange 1e+03 0.0)) (.z _relativelocation)) false false)
  (Transformation|SetRelativeLocation (Variables|Default|GetBuilding_04) (Math|Vector|MakeVector (.x _relativelocation_2) (+ (.y _relativelocation_2) (Math|Random|RandomFloatinRange 1e+03 0.0)) (.z _relativelocation_2)) false false))

(fn RandomWIndowEmissiveness
  (bind _returnvalue (Rendering|Material|CreateDynamicMaterialInstance (Variables|Default|GetBuilding_01) 1 "/Game/Hover_Car/Assets/Buildings/Materials/Hover_Buildings_Windows_Mat.Hover_Buildings_Windows_Mat" "None" :!class /Script/Engine.PrimitiveComponent))
  (Rendering|Material|SetScalarParameterValue _returnvalue "Emissiveness" (Math|Random|RandomFloatinRange 5.0 1e+01) :!class /Script/Engine.MaterialInstanceDynamic)
  (bind _returnvalue_2 (Rendering|Material|CreateDynamicMaterialInstance (Variables|Default|GetBuilding_02) 1 "/Game/Hover_Car/Assets/Buildings/Materials/Hover_Buildings_Windows_Mat.Hover_Buildings_Windows_Mat" "None" :!class /Script/Engine.PrimitiveComponent))
  (Rendering|Material|SetScalarParameterValue _returnvalue_2 "Emissiveness" (Math|Random|RandomFloatinRange 5.0 1e+01) :!class /Script/Engine.MaterialInstanceDynamic)
  (bind _returnvalue_3 (Rendering|Material|CreateDynamicMaterialInstance (Variables|Default|GetBuilding_03) 1 "/Game/Hover_Car/Assets/Buildings/Materials/Hover_Buildings_Windows_Mat.Hover_Buildings_Windows_Mat" "None" :!class /Script/Engine.PrimitiveComponent))
  (Rendering|Material|SetScalarParameterValue _returnvalue_3 "Emissiveness" (Math|Random|RandomFloatinRange 5.0 1e+01) :!class /Script/Engine.MaterialInstanceDynamic)
  (bind _returnvalue_4 (Rendering|Material|CreateDynamicMaterialInstance (Variables|Default|GetBuilding_04) 1 "/Game/Hover_Car/Assets/Buildings/Materials/Hover_Buildings_Windows_Mat.Hover_Buildings_Windows_Mat" "None" :!class /Script/Engine.PrimitiveComponent))
  (Rendering|Material|SetScalarParameterValue _returnvalue_4 "Emissiveness" (Math|Random|RandomFloatinRange 5.0 1e+01) :!class /Script/Engine.MaterialInstanceDynamic))

(fn RandomWindowColour
  (Utilities|FlowControl|Sequence
    (:then_0
      (switch int (Math|Random|RandomIntegerinRange 0 4)
        (:0
          (bind _returnvalue (Rendering|Material|CreateDynamicMaterialInstance (Variables|Default|GetBuilding_01) 1 "/Game/Hover_Car/Assets/Buildings/Materials/Hover_Buildings_Windows_Mat.Hover_Buildings_Windows_Mat" "None" :!class /Script/Engine.PrimitiveComponent))
          (Rendering|Material|SetVectorParameterValue :self _returnvalue :ParameterName "Colour" :!class /Script/Engine.MaterialInstanceDynamic)
          (bind _returnvalue_2 (Rendering|Material|GetVectorParameterValue _returnvalue "Colour" :!class /Script/Engine.MaterialInstanceDynamic))
          (Variables|Default|SetBuilding_01%20Window%20Colour _returnvalue_2))
        (:1
          (bind _returnvalue_3 (Rendering|Material|CreateDynamicMaterialInstance (Variables|Default|GetBuilding_01) 1 "/Game/Hover_Car/Assets/Buildings/Materials/Hover_Buildings_Windows_Mat.Hover_Buildings_Windows_Mat" "None" :!class /Script/Engine.PrimitiveComponent))
          (Rendering|Material|SetVectorParameterValue _returnvalue_3 "Colour" "(R=1.000000,G=1.000000,B=1.000000,A=1.000000)" :!class /Script/Engine.MaterialInstanceDynamic)
          (bind _returnvalue_4 (Rendering|Material|GetVectorParameterValue _returnvalue_3 "Colour" :!class /Script/Engine.MaterialInstanceDynamic))
          (Variables|Default|SetBuilding_01%20Window%20Colour _returnvalue_4))
        (:2
          (bind _returnvalue_5 (Rendering|Material|CreateDynamicMaterialInstance (Variables|Default|GetBuilding_01) 1 "/Game/Hover_Car/Assets/Buildings/Materials/Hover_Buildings_Windows_Mat.Hover_Buildings_Windows_Mat" "None" :!class /Script/Engine.PrimitiveComponent))
          (Rendering|Material|SetVectorParameterValue _returnvalue_5 "Colour" "(R=1.000000,G=0.964563,B=0.700000,A=1.000000)" :!class /Script/Engine.MaterialInstanceDynamic)
          (bind _returnvalue_6 (Rendering|Material|GetVectorParameterValue _returnvalue_5 "Colour" :!class /Script/Engine.MaterialInstanceDynamic))
          (Variables|Default|SetBuilding_01%20Window%20Colour _returnvalue_6))
        (:3
          (bind _returnvalue_7 (Rendering|Material|CreateDynamicMaterialInstance (Variables|Default|GetBuilding_01) 1 "/Game/Hover_Car/Assets/Buildings/Materials/Hover_Buildings_Windows_Mat.Hover_Buildings_Windows_Mat" "None" :!class /Script/Engine.PrimitiveComponent))
          (Rendering|Material|SetVectorParameterValue _returnvalue_7 "Colour" "(R=1.000000,G=0.799677,B=0.700000,A=1.000000)" :!class /Script/Engine.MaterialInstanceDynamic)
          (bind _returnvalue_8 (Rendering|Material|GetVectorParameterValue _returnvalue_7 "Colour" :!class /Script/Engine.MaterialInstanceDynamic))
          (Variables|Default|SetBuilding_01%20Window%20Colour _returnvalue_8))))
    (:then_1
      (switch int (Math|Random|RandomIntegerinRange 0 4)
        (:0
          (bind _returnvalue_9 (Rendering|Material|CreateDynamicMaterialInstance (Variables|Default|GetBuilding_02) 1 "/Game/Hover_Car/Assets/Buildings/Materials/Hover_Buildings_Windows_Mat.Hover_Buildings_Windows_Mat" "None" :!class /Script/Engine.PrimitiveComponent))
          (Rendering|Material|SetVectorParameterValue :self _returnvalue_9 :ParameterName "Colour" :!class /Script/Engine.MaterialInstanceDynamic)
          (bind _returnvalue_10 (Rendering|Material|GetVectorParameterValue _returnvalue_9 "Colour" :!class /Script/Engine.MaterialInstanceDynamic))
          (Variables|Default|SetBuilding_02%20Window%20Colour _returnvalue_10))
        (:1
          (bind _returnvalue_11 (Rendering|Material|CreateDynamicMaterialInstance (Variables|Default|GetBuilding_02) 1 "/Game/Hover_Car/Assets/Buildings/Materials/Hover_Buildings_Windows_Mat.Hover_Buildings_Windows_Mat" "None" :!class /Script/Engine.PrimitiveComponent))
          (Rendering|Material|SetVectorParameterValue _returnvalue_11 "Colour" "(R=1.000000,G=1.000000,B=1.000000,A=1.000000)" :!class /Script/Engine.MaterialInstanceDynamic)
          (bind _returnvalue_12 (Rendering|Material|GetVectorParameterValue _returnvalue_11 "Colour" :!class /Script/Engine.MaterialInstanceDynamic))
          (Variables|Default|SetBuilding_02%20Window%20Colour _returnvalue_12))
        (:2
          (bind _returnvalue_13 (Rendering|Material|CreateDynamicMaterialInstance (Variables|Default|GetBuilding_02) 1 "/Game/Hover_Car/Assets/Buildings/Materials/Hover_Buildings_Windows_Mat.Hover_Buildings_Windows_Mat" "None" :!class /Script/Engine.PrimitiveComponent))
          (Rendering|Material|SetVectorParameterValue _returnvalue_13 "Colour" "(R=1.000000,G=0.964563,B=0.700000,A=1.000000)" :!class /Script/Engine.MaterialInstanceDynamic)
          (bind _returnvalue_14 (Rendering|Material|GetVectorParameterValue _returnvalue_13 "Colour" :!class /Script/Engine.MaterialInstanceDynamic))
          (Variables|Default|SetBuilding_02%20Window%20Colour _returnvalue_14))
        (:3
          (bind _returnvalue_15 (Rendering|Material|CreateDynamicMaterialInstance (Variables|Default|GetBuilding_02) 1 "/Game/Hover_Car/Assets/Buildings/Materials/Hover_Buildings_Windows_Mat.Hover_Buildings_Windows_Mat" "None" :!class /Script/Engine.PrimitiveComponent))
          (Rendering|Material|SetVectorParameterValue _returnvalue_15 "Colour" "(R=1.000000,G=0.799677,B=0.700000,A=1.000000)" :!class /Script/Engine.MaterialInstanceDynamic)
          (bind _returnvalue_16 (Rendering|Material|GetVectorParameterValue _returnvalue_15 "Colour" :!class /Script/Engine.MaterialInstanceDynamic))
          (Variables|Default|SetBuilding_02%20Window%20Colour _returnvalue_16))))
    (:then_2
      (switch int (Math|Random|RandomIntegerinRange 0 4)
        (:0
          (bind _returnvalue_17 (Rendering|Material|CreateDynamicMaterialInstance (Variables|Default|GetBuilding_03) 1 "/Game/Hover_Car/Assets/Buildings/Materials/Hover_Buildings_Windows_Mat.Hover_Buildings_Windows_Mat" "None" :!class /Script/Engine.PrimitiveComponent))
          (Rendering|Material|SetVectorParameterValue :self _returnvalue_17 :ParameterName "Colour" :!class /Script/Engine.MaterialInstanceDynamic)
          (bind _returnvalue_18 (Rendering|Material|GetVectorParameterValue _returnvalue_17 "Colour" :!class /Script/Engine.MaterialInstanceDynamic))
          (Variables|Default|SetBuilding_03%20Window%20Colour _returnvalue_18))
        (:1
          (bind _returnvalue_19 (Rendering|Material|CreateDynamicMaterialInstance (Variables|Default|GetBuilding_03) 1 "/Game/Hover_Car/Assets/Buildings/Materials/Hover_Buildings_Windows_Mat.Hover_Buildings_Windows_Mat" "None" :!class /Script/Engine.PrimitiveComponent))
          (Rendering|Material|SetVectorParameterValue _returnvalue_19 "Colour" "(R=1.000000,G=1.000000,B=1.000000,A=1.000000)" :!class /Script/Engine.MaterialInstanceDynamic)
          (bind _returnvalue_20 (Rendering|Material|GetVectorParameterValue _returnvalue_19 "Colour" :!class /Script/Engine.MaterialInstanceDynamic))
          (Variables|Default|SetBuilding_03%20Window%20Colour _returnvalue_20))
        (:2
          (bind _returnvalue_21 (Rendering|Material|CreateDynamicMaterialInstance (Variables|Default|GetBuilding_03) 1 "/Game/Hover_Car/Assets/Buildings/Materials/Hover_Buildings_Windows_Mat.Hover_Buildings_Windows_Mat" "None" :!class /Script/Engine.PrimitiveComponent))
          (Rendering|Material|SetVectorParameterValue _returnvalue_21 "Colour" "(R=1.000000,G=0.964563,B=0.700000,A=1.000000)" :!class /Script/Engine.MaterialInstanceDynamic)
          (bind _returnvalue_22 (Rendering|Material|GetVectorParameterValue _returnvalue_21 "Colour" :!class /Script/Engine.MaterialInstanceDynamic))
          (Variables|Default|SetBuilding_03%20Window%20Colour _returnvalue_22))
        (:3
          (bind _returnvalue_23 (Rendering|Material|CreateDynamicMaterialInstance (Variables|Default|GetBuilding_03) 1 "/Game/Hover_Car/Assets/Buildings/Materials/Hover_Buildings_Windows_Mat.Hover_Buildings_Windows_Mat" "None" :!class /Script/Engine.PrimitiveComponent))
          (Rendering|Material|SetVectorParameterValue _returnvalue_23 "Colour" "(R=1.000000,G=0.799677,B=0.700000,A=1.000000)" :!class /Script/Engine.MaterialInstanceDynamic)
          (bind _returnvalue_24 (Rendering|Material|GetVectorParameterValue _returnvalue_23 "Colour" :!class /Script/Engine.MaterialInstanceDynamic))
          (Variables|Default|SetBuilding_03%20Window%20Colour _returnvalue_24))))
    (:then_3
      (switch int (Math|Random|RandomIntegerinRange 0 4)
        (:0
          (bind _returnvalue_25 (Rendering|Material|CreateDynamicMaterialInstance (Variables|Default|GetBuilding_04) 1 "/Game/Hover_Car/Assets/Buildings/Materials/Hover_Buildings_Windows_Mat.Hover_Buildings_Windows_Mat" "None" :!class /Script/Engine.PrimitiveComponent))
          (Rendering|Material|SetVectorParameterValue :self _returnvalue_25 :ParameterName "Colour" :!class /Script/Engine.MaterialInstanceDynamic)
          (bind _returnvalue_26 (Rendering|Material|GetVectorParameterValue _returnvalue_25 "Colour" :!class /Script/Engine.MaterialInstanceDynamic))
          (Variables|Default|SetBuilding_04%20Window%20Colour _returnvalue_26))
        (:1
          (bind _returnvalue_27 (Rendering|Material|CreateDynamicMaterialInstance (Variables|Default|GetBuilding_04) 1 "/Game/Hover_Car/Assets/Buildings/Materials/Hover_Buildings_Windows_Mat.Hover_Buildings_Windows_Mat" "None" :!class /Script/Engine.PrimitiveComponent))
          (Rendering|Material|SetVectorParameterValue _returnvalue_27 "Colour" "(R=1.000000,G=1.000000,B=1.000000,A=1.000000)" :!class /Script/Engine.MaterialInstanceDynamic)
          (bind _returnvalue_28 (Rendering|Material|GetVectorParameterValue _returnvalue_27 "Colour" :!class /Script/Engine.MaterialInstanceDynamic))
          (Variables|Default|SetBuilding_04%20Window%20Colour _returnvalue_28))
        (:2
          (bind _returnvalue_29 (Rendering|Material|CreateDynamicMaterialInstance (Variables|Default|GetBuilding_04) 1 "/Game/Hover_Car/Assets/Buildings/Materials/Hover_Buildings_Windows_Mat.Hover_Buildings_Windows_Mat" "None" :!class /Script/Engine.PrimitiveComponent))
          (Rendering|Material|SetVectorParameterValue _returnvalue_29 "Colour" "(R=1.000000,G=0.964563,B=0.700000,A=1.000000)" :!class /Script/Engine.MaterialInstanceDynamic)
          (bind _returnvalue_30 (Rendering|Material|GetVectorParameterValue _returnvalue_29 "Colour" :!class /Script/Engine.MaterialInstanceDynamic))
          (Variables|Default|SetBuilding_04%20Window%20Colour _returnvalue_30))
        (:3
          (bind _returnvalue_31 (Rendering|Material|CreateDynamicMaterialInstance (Variables|Default|GetBuilding_04) 1 "/Game/Hover_Car/Assets/Buildings/Materials/Hover_Buildings_Windows_Mat.Hover_Buildings_Windows_Mat" "None" :!class /Script/Engine.PrimitiveComponent))
          (Rendering|Material|SetVectorParameterValue _returnvalue_31 "Colour" "(R=1.000000,G=0.799677,B=0.700000,A=1.000000)" :!class /Script/Engine.MaterialInstanceDynamic)
          (bind _returnvalue_32 (Rendering|Material|GetVectorParameterValue _returnvalue_31 "Colour" :!class /Script/Engine.MaterialInstanceDynamic))
          (Variables|Default|SetBuilding_04%20Window%20Colour _returnvalue_32))))))

(fn AddRandomBuildingFloors
  (bind _building_04 (Variables|Default|GetBuilding_04))
  (bind _building_03 (Variables|Default|GetBuilding_03))
  (bind _building_01 (Variables|Default|GetBuilding_01))
  (bind _building_02 (Variables|Default|GetBuilding_02))
  (bind _building_04_2 (Variables|Default|GetBuilding_04))
  (bind _building_01_2 (Variables|Default|GetBuilding_01))
  (bind _building_02_2 (Variables|Default|GetBuilding_02))
  (bind _building_03_2 (Variables|Default|GetBuilding_03))
  (bind _returnvalue (Rendering|Material|GetMaterial _building_01_2 0))
  (bind _returnvalue_2 (Rendering|Material|GetMaterial _building_02_2 0))
  (bind _returnvalue_3 (Rendering|Material|GetMaterial _building_03_2 0))
  (bind _returnvalue_4 (Rendering|Material|GetMaterial _building_04 0))
  (bind _relativelocation (Variables|/Script/Engine.SceneComponent|GetRelativeLocation _building_03))
  (bind _relativelocation_2 (Variables|/Script/Engine.SceneComponent|GetRelativeLocation _building_01))
  (bind _relativelocation_3 (Variables|/Script/Engine.SceneComponent|GetRelativeLocation _building_02))
  (bind _relativelocation_4 (Variables|/Script/Engine.SceneComponent|GetRelativeLocation _building_04_2))
  (Utilities|FlowControl|Sequence
    (:then_0
      (switch int (Math|Random|RandomIntegerinRange 0 1)
        (:1
          (bind _returnvalue_5 (AddComponent|AddStaticMeshComponent false (Math|Transform|MakeTransform (Math|Vector|MakeVector (.x _relativelocation_2) (.y _relativelocation_2) (+ (.z _relativelocation_2) 1.2e+03)) (Variables|/Script/Engine.SceneComponent|GetRelativeRotation (Variables|Default|GetBuilding_01)) "1.000000,1.000000,1.000000")))
          (Components|StaticMesh|SetStaticMesh _returnvalue_5 (Variables|/Script/Engine.StaticMeshComponent|GetStaticMesh (Variables|Default|GetBuilding_01)))
          (Rendering|Material|SetMaterial _returnvalue_5 0 _returnvalue)
          (bind _returnvalue_6 (Rendering|Material|CreateDynamicMaterialInstance _returnvalue_5 1 "/Game/Hover_Car/Assets/Buildings/Materials/Hover_Buildings_Windows_Mat.Hover_Buildings_Windows_Mat" "None" :!class /Script/Engine.PrimitiveComponent))
          (Rendering|Material|SetScalarParameterValue _returnvalue_6 "Emissiveness" (Math|Random|RandomFloatinRange 0.0 1e+01) :!class /Script/Engine.MaterialInstanceDynamic)
          (bind _returnvalue_7 (Rendering|Material|CreateDynamicMaterialInstance _returnvalue_5 1 "/Game/Hover_Car/Assets/Buildings/Materials/Hover_Buildings_Windows_Mat.Hover_Buildings_Windows_Mat" "None" :!class /Script/Engine.PrimitiveComponent))
          (Rendering|Material|SetVectorParameterValue _returnvalue_7 "Colour" (Variables|Default|GetBuilding_01%20Window%20Colour) :!class /Script/Engine.MaterialInstanceDynamic)
          (switch int (Math|Random|RandomIntegerinRange 0 1)
            (:1
              (bind _returnvalue_8 (AddComponent|AddStaticMeshComponent false (Math|Transform|MakeTransform (Math|Vector|MakeVector (.x (Variables|/Script/Engine.SceneComponent|GetRelativeLocation _returnvalue_5)) (.y (Variables|/Script/Engine.SceneComponent|GetRelativeLocation _returnvalue_5)) (+ (.z (Variables|/Script/Engine.SceneComponent|GetRelativeLocation _returnvalue_5)) 1.2e+03)) (Variables|/Script/Engine.SceneComponent|GetRelativeRotation _returnvalue_5) "1.000000,1.000000,1.000000")))
              (Components|StaticMesh|SetStaticMesh _returnvalue_8 (Variables|/Script/Engine.StaticMeshComponent|GetStaticMesh _returnvalue_5))
              (Rendering|Material|SetMaterial _returnvalue_8 0 _returnvalue)
              (bind _returnvalue_9 (Rendering|Material|CreateDynamicMaterialInstance _returnvalue_8 1 "/Game/Hover_Car/Assets/Buildings/Materials/Hover_Buildings_Windows_Mat.Hover_Buildings_Windows_Mat" "None" :!class /Script/Engine.PrimitiveComponent))
              (Rendering|Material|SetScalarParameterValue _returnvalue_9 "Emissiveness" (Math|Random|RandomFloatinRange 0.0 1e+01) :!class /Script/Engine.MaterialInstanceDynamic)
              (bind _returnvalue_10 (Rendering|Material|CreateDynamicMaterialInstance _returnvalue_8 1 "/Game/Hover_Car/Assets/Buildings/Materials/Hover_Buildings_Windows_Mat.Hover_Buildings_Windows_Mat" "None" :!class /Script/Engine.PrimitiveComponent))
              (Rendering|Material|SetVectorParameterValue _returnvalue_10 "Colour" (Variables|Default|GetBuilding_01%20Window%20Colour) :!class /Script/Engine.MaterialInstanceDynamic))))))
    (:then_1
      (switch int (Math|Random|RandomIntegerinRange 0 1)
        (:1
          (bind _returnvalue_11 (AddComponent|AddStaticMeshComponent false (Math|Transform|MakeTransform (Math|Vector|MakeVector (.x _relativelocation_3) (.y _relativelocation_3) (+ (.z _relativelocation_3) 1.2e+03)) (Variables|/Script/Engine.SceneComponent|GetRelativeRotation (Variables|Default|GetBuilding_02)) "1.000000,1.000000,1.000000")))
          (Components|StaticMesh|SetStaticMesh _returnvalue_11 (Variables|/Script/Engine.StaticMeshComponent|GetStaticMesh (Variables|Default|GetBuilding_02)))
          (Rendering|Material|SetMaterial _returnvalue_11 0 _returnvalue_2)
          (bind _returnvalue_12 (Rendering|Material|CreateDynamicMaterialInstance _returnvalue_11 1 "/Game/Hover_Car/Assets/Buildings/Materials/Hover_Buildings_Windows_Mat.Hover_Buildings_Windows_Mat" "None" :!class /Script/Engine.PrimitiveComponent))
          (Rendering|Material|SetScalarParameterValue _returnvalue_12 "Emissiveness" (Math|Random|RandomFloatinRange 0.0 1e+01) :!class /Script/Engine.MaterialInstanceDynamic)
          (bind _returnvalue_13 (Rendering|Material|CreateDynamicMaterialInstance _returnvalue_11 1 "/Game/Hover_Car/Assets/Buildings/Materials/Hover_Buildings_Windows_Mat.Hover_Buildings_Windows_Mat" "None" :!class /Script/Engine.PrimitiveComponent))
          (Rendering|Material|SetVectorParameterValue _returnvalue_13 "Colour" (Variables|Default|GetBuilding_01%20Window%20Colour) :!class /Script/Engine.MaterialInstanceDynamic)
          (switch int (Math|Random|RandomIntegerinRange 0 1)
            (:1
              (bind _returnvalue_14 (AddComponent|AddStaticMeshComponent false (Math|Transform|MakeTransform (Math|Vector|MakeVector (.x (Variables|/Script/Engine.SceneComponent|GetRelativeLocation _returnvalue_11)) (.y (Variables|/Script/Engine.SceneComponent|GetRelativeLocation _returnvalue_11)) (+ (.z (Variables|/Script/Engine.SceneComponent|GetRelativeLocation _returnvalue_11)) 1.2e+03)) (Variables|/Script/Engine.SceneComponent|GetRelativeRotation _returnvalue_11) "1.000000,1.000000,1.000000")))
              (Components|StaticMesh|SetStaticMesh _returnvalue_14 (Variables|/Script/Engine.StaticMeshComponent|GetStaticMesh _returnvalue_11))
              (Rendering|Material|SetMaterial _returnvalue_14 0 _returnvalue_2)
              (bind _returnvalue_15 (Rendering|Material|CreateDynamicMaterialInstance _returnvalue_14 1 "/Game/Hover_Car/Assets/Buildings/Materials/Hover_Buildings_Windows_Mat.Hover_Buildings_Windows_Mat" "None" :!class /Script/Engine.PrimitiveComponent))
              (Rendering|Material|SetVectorParameterValue _returnvalue_15 "Colour" (Variables|Default|GetBuilding_02%20Window%20Colour) :!class /Script/Engine.MaterialInstanceDynamic))))))
    (:then_2
      (switch int (Math|Random|RandomIntegerinRange 0 1)
        (:1
          (bind _returnvalue_16 (AddComponent|AddStaticMeshComponent false (Math|Transform|MakeTransform (Math|Vector|MakeVector (.x _relativelocation) (.y _relativelocation) (+ (.z _relativelocation) 1.2e+03)) (Variables|/Script/Engine.SceneComponent|GetRelativeRotation (Variables|Default|GetBuilding_03)) "1.000000,1.000000,1.000000")))
          (Components|StaticMesh|SetStaticMesh _returnvalue_16 (Variables|/Script/Engine.StaticMeshComponent|GetStaticMesh (Variables|Default|GetBuilding_03)))
          (Rendering|Material|SetMaterial _returnvalue_16 0 _returnvalue_3)
          (bind _returnvalue_17 (Rendering|Material|CreateDynamicMaterialInstance _returnvalue_16 1 "/Game/Hover_Car/Assets/Buildings/Materials/Hover_Buildings_Windows_Mat.Hover_Buildings_Windows_Mat" "None" :!class /Script/Engine.PrimitiveComponent))
          (Rendering|Material|SetScalarParameterValue _returnvalue_17 "Emissiveness" (Math|Random|RandomFloatinRange 0.0 1e+01) :!class /Script/Engine.MaterialInstanceDynamic)
          (bind _returnvalue_18 (Rendering|Material|CreateDynamicMaterialInstance _returnvalue_16 1 "/Game/Hover_Car/Assets/Buildings/Materials/Hover_Buildings_Windows_Mat.Hover_Buildings_Windows_Mat" "None" :!class /Script/Engine.PrimitiveComponent))
          (Rendering|Material|SetVectorParameterValue _returnvalue_18 "Colour" (Variables|Default|GetBuilding_03%20Window%20Colour) :!class /Script/Engine.MaterialInstanceDynamic)
          (switch int (Math|Random|RandomIntegerinRange 0 1)
            (:1
              (bind _returnvalue_19 (AddComponent|AddStaticMeshComponent false (Math|Transform|MakeTransform (Math|Vector|MakeVector (.x (Variables|/Script/Engine.SceneComponent|GetRelativeLocation _returnvalue_16)) (.y (Variables|/Script/Engine.SceneComponent|GetRelativeLocation _returnvalue_16)) (+ (.z (Variables|/Script/Engine.SceneComponent|GetRelativeLocation _returnvalue_16)) 1.2e+03)) (Variables|/Script/Engine.SceneComponent|GetRelativeRotation _returnvalue_16) "1.000000,1.000000,1.000000")))
              (Components|StaticMesh|SetStaticMesh _returnvalue_19 (Variables|/Script/Engine.StaticMeshComponent|GetStaticMesh _returnvalue_16))
              (Rendering|Material|SetMaterial _returnvalue_19 0 _returnvalue_3)
              (bind _returnvalue_20 (Rendering|Material|CreateDynamicMaterialInstance _returnvalue_19 1 "/Game/Hover_Car/Assets/Buildings/Materials/Hover_Buildings_Windows_Mat.Hover_Buildings_Windows_Mat" "None" :!class /Script/Engine.PrimitiveComponent))
              (Rendering|Material|SetVectorParameterValue _returnvalue_20 "Colour" (Variables|Default|GetBuilding_03%20Window%20Colour) :!class /Script/Engine.MaterialInstanceDynamic))))))
    (:then_3
      (switch int (Math|Random|RandomIntegerinRange 0 1)
        (:1
          (bind _returnvalue_21 (AddComponent|AddStaticMeshComponent false (Math|Transform|MakeTransform (Math|Vector|MakeVector (.x _relativelocation_4) (.y _relativelocation_4) (+ (.z _relativelocation_4) 1.2e+03)) (Variables|/Script/Engine.SceneComponent|GetRelativeRotation (Variables|Default|GetBuilding_04)) "1.000000,1.000000,1.000000")))
          (Components|StaticMesh|SetStaticMesh _returnvalue_21 (Variables|/Script/Engine.StaticMeshComponent|GetStaticMesh (Variables|Default|GetBuilding_04)))
          (Rendering|Material|SetMaterial _returnvalue_21 0 _returnvalue_4)
          (bind _returnvalue_22 (Rendering|Material|CreateDynamicMaterialInstance _returnvalue_21 1 "/Game/Hover_Car/Assets/Buildings/Materials/Hover_Buildings_Windows_Mat.Hover_Buildings_Windows_Mat" "None" :!class /Script/Engine.PrimitiveComponent))
          (Rendering|Material|SetScalarParameterValue _returnvalue_22 "Emissiveness" (Math|Random|RandomFloatinRange 0.0 1e+01) :!class /Script/Engine.MaterialInstanceDynamic)
          (bind _returnvalue_23 (Rendering|Material|CreateDynamicMaterialInstance _returnvalue_21 1 "/Game/Hover_Car/Assets/Buildings/Materials/Hover_Buildings_Windows_Mat.Hover_Buildings_Windows_Mat" "None" :!class /Script/Engine.PrimitiveComponent))
          (Rendering|Material|SetVectorParameterValue _returnvalue_23 "Colour" (Variables|Default|GetBuilding_04%20Window%20Colour) :!class /Script/Engine.MaterialInstanceDynamic)
          (switch int (Math|Random|RandomIntegerinRange 0 1)
            (:1
              (bind _returnvalue_24 (AddComponent|AddStaticMeshComponent false (Math|Transform|MakeTransform (Math|Vector|MakeVector (.x (Variables|/Script/Engine.SceneComponent|GetRelativeLocation _returnvalue_21)) (.y (Variables|/Script/Engine.SceneComponent|GetRelativeLocation _returnvalue_21)) (+ (.z (Variables|/Script/Engine.SceneComponent|GetRelativeLocation _returnvalue_21)) 1.2e+03)) (Variables|/Script/Engine.SceneComponent|GetRelativeRotation _returnvalue_21) "1.000000,1.000000,1.000000")))
              (Components|StaticMesh|SetStaticMesh _returnvalue_24 (Variables|/Script/Engine.StaticMeshComponent|GetStaticMesh _returnvalue_21))
              (Rendering|Material|SetMaterial _returnvalue_24 0 _returnvalue_4)
              (bind _returnvalue_25 (Rendering|Material|CreateDynamicMaterialInstance _returnvalue_24 1 "/Game/Hover_Car/Assets/Buildings/Materials/Hover_Buildings_Windows_Mat.Hover_Buildings_Windows_Mat" "None" :!class /Script/Engine.PrimitiveComponent))
              (Rendering|Material|SetVectorParameterValue _returnvalue_25 "Colour" (Variables|Default|GetBuilding_04%20Window%20Colour) :!class /Script/Engine.MaterialInstanceDynamic))))))))

(fn RandomiseBuildingUVS
  (Utilities|FlowControl|Sequence
    (:then_0
      (switch int (Math|Random|RandomIntegerinRange 0 4)
        (:0
          (Variables|Default|SetValue 0.0))
        (:1
          (Variables|Default|SetValue 0.25))
        (:2
          (Variables|Default|SetValue 0.5))
        (:3
          (Variables|Default|SetValue 1.0)))
      (bind _returnvalue (Rendering|Material|CreateDynamicMaterialInstance (Variables|Default|GetBuilding_01) 0 (Rendering|Material|GetMaterial (Variables|Default|GetBuilding_01) 0) "None" :!class /Script/Engine.PrimitiveComponent))
      (Rendering|Material|SetScalarParameterValue _returnvalue "U Offset" (Variables|Default|GetValue) :!class /Script/Engine.MaterialInstanceDynamic))
    (:then_1
      (switch int (Math|Random|RandomIntegerinRange 0 4)
        (:0
          (Variables|Default|SetValue 0.0))
        (:1
          (Variables|Default|SetValue 0.25))
        (:2
          (Variables|Default|SetValue 0.5))
        (:3
          (Variables|Default|SetValue 1.0)))
      (bind _returnvalue_2 (Rendering|Material|CreateDynamicMaterialInstance (Variables|Default|GetBuilding_02) 0 (Rendering|Material|GetMaterial (Variables|Default|GetBuilding_02) 0) "None" :!class /Script/Engine.PrimitiveComponent))
      (Rendering|Material|SetScalarParameterValue _returnvalue_2 "U Offset" (Variables|Default|GetValue) :!class /Script/Engine.MaterialInstanceDynamic))
    (:then_2
      (switch int (Math|Random|RandomIntegerinRange 0 4)
        (:0
          (Variables|Default|SetValue 0.0))
        (:1
          (Variables|Default|SetValue 0.25))
        (:2
          (Variables|Default|SetValue 0.5))
        (:3
          (Variables|Default|SetValue 1.0)))
      (bind _returnvalue_3 (Rendering|Material|CreateDynamicMaterialInstance (Variables|Default|GetBuilding_03) 0 (Rendering|Material|GetMaterial (Variables|Default|GetBuilding_03) 0) "None" :!class /Script/Engine.PrimitiveComponent))
      (Rendering|Material|SetScalarParameterValue _returnvalue_3 "U Offset" (Variables|Default|GetValue) :!class /Script/Engine.MaterialInstanceDynamic))
    (:then_3
      (switch int (Math|Random|RandomIntegerinRange 0 4)
        (:0
          (Variables|Default|SetValue 0.0))
        (:1
          (Variables|Default|SetValue 0.25))
        (:2
          (Variables|Default|SetValue 0.5))
        (:3
          (Variables|Default|SetValue 1.0)))
      (bind _returnvalue_4 (Rendering|Material|CreateDynamicMaterialInstance (Variables|Default|GetBuilding_04) 0 (Rendering|Material|GetMaterial (Variables|Default|GetBuilding_04) 0) "None" :!class /Script/Engine.PrimitiveComponent))
      (Rendering|Material|SetScalarParameterValue _returnvalue_4 "U Offset" (Variables|Default|GetValue) :!class /Script/Engine.MaterialInstanceDynamic))))