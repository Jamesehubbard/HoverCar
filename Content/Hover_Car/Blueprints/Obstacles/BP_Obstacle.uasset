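; BP_Obstacle is an obstacle Blueprint for the Hover Car game that randomly appears as either a dummy car or a trash truck.
; On BeginPlay it assigns one of the two static meshes at random to its Mesh component.
; After a short delay it checks which mesh was chosen and sets a matching uniform world scale, shrinking the truck and enlarging the car.
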(event EventBeginPlay
  (Components|StaticMesh|SetStaticMesh (Variables|Default|GetMesh) (.OutItem (Utilities|Array|Random (Utilities|Array|MakeArray (Variables|Default|GetDummy%20Car) (Variables|Default|GetTrashTruck)))))
  (Utilities|FlowControl|Delay 0.2)
  (if (== (Variables|/Script/Engine.StaticMeshComponent|GetStaticMesh (Variables|Default|GetMesh)) (Variables|Default|GetTrashTruck))
    (Transformation|SetWorldScale3D (Variables|Default|GetMesh) "0.500000,0.500000,0.500000")
    (else
      (Transformation|SetWorldScale3D (Variables|Default|GetMesh) "1.250000,1.250000,1.250000"))))

(fn ConstructionScript)