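; Cowboy Blueprint for GunDuel that drives the mouse cursor from look input and detects clicks on head and body hit boxes.
; LookRight and LookUp pass a small deadzone into one shared SetMouseLocation call, which adds the same scaled axis value to both X and Y.
; BeginPlay sets left mouse and gamepad bottom face button as click keys.
; Clicking either box only prints "Head" or "Body".
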(event OnClicked(Box)
  (params (TouchedComponent :type Primitive%20Component%20Object%20Reference) (ButtonPressed :type Key%20Structure :default "None"))
  (Development|PrintString "Body"))

(event OnClicked(Box1)
  (params (TouchedComponent :type Primitive%20Component%20Object%20Reference) (ButtonPressed :type Key%20Structure :default "None"))
  (Development|PrintString "Head"))

(event EventBeginPlay
  (Variables|/Script/Engine.PlayerController|SetClickEventKeys (Game|GetPlayerController 0) (Utilities|Array|MakeArray "LeftMouseButton" "Gamepad_FaceButton_Bottom")))

(event Input|AxisEvents|InputAxisLookRight
  (params (AxisValue :type Float%20%28single-precision%29))
  (bind _returnvalue (Game|GetPlayerController 0))
  (bind (_locationx _locationy) (Game|Player|GetMousePosition _returnvalue))
  (if (> (Math|Float|Absolute(Float) AxisValue) 0.02)
    (Class|PlayerController|SetMouseLocation (Game|GetPlayerController 0) (Math|Float|Truncate (+ (* AxisValue 5.0) _locationx)) (Math|Float|Truncate (+ (* (stale Input|AxisEvents|InputAxisLookUp AxisValue) 5.0) _locationy)))))

(event Input|AxisEvents|InputAxisLookUp
  (params (AxisValue :type Float%20%28single-precision%29))
  (bind _returnvalue (Game|GetPlayerController 0))
  (bind (_locationx _locationy) (Game|Player|GetMousePosition _returnvalue))
  (if (> (Math|Float|Absolute(Float) AxisValue) 0.02)
    (Class|PlayerController|SetMouseLocation (Game|GetPlayerController 0) (Math|Float|Truncate (+ (* (stale Input|AxisEvents|InputAxisLookRight AxisValue) 5.0) _locationx)) (Math|Float|Truncate (+ (* AxisValue 5.0) _locationy)))))

(fn ConstructionScript)