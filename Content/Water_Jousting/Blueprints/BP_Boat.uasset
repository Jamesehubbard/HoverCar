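; Player-controlled boat for water jousting, with an Archer component that turns on the look axis and a Cylinder that performs a charged thrust.
; Throttle and steer inputs ease toward targets and move the boat by unswept offsets along its right vector, with yaw rate scaled by speed.
; Holding A builds charge; releasing plays a timeline sliding the Cylinder along Y, with charge setting rate and reach.
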(event EventTick
  (params (DeltaSeconds :type Float%20%28single-precision%29))
  (Utilities|FlowControl|Sequence
    (:then_0
      (if (Variables|Default|GetA%20Button%20Pressed)
        (Variables|Default|SetA%20Button%20Time%20Pressed (Math|Float|Clamp(Float) (+ (Variables|Default|GetA%20Button%20Time%20Pressed) 0.01)))))
    (:then_1
      (Development|PrintString (Utilities|String|ToString(Vector) (Variables|/Script/Engine.SceneComponent|GetRelativeLocation (Variables|Default|GetCylinder)))))))

(event Input|ActionEvents|InputActionAButton
  (params (Key :type Key%20Structure :default "None"))
  (bind _cylinder (Variables|Default|GetCylinder))
  (bind _relativelocation (Variables|/Script/Engine.SceneComponent|GetRelativeLocation _cylinder))
  (:Pressed
    (Variables|Default|SetA%20Button%20Pressed true))
  (:Released
    (Variables|Default|SetA%20Button%20Pressed false)
    (Components|Timeline|SetPlayRate (Variables|Default|GetTimeline_0) (/ (Variables|Default|GetA%20Button%20Time%20Pressed) 0.25))
    (bind _newtrack_0 (Timeline|Timeline_0 PlayFromStart)
      (:Update
        (Transformation|SetRelativeLocation _cylinder (Math|Vector|MakeVector (.x _relativelocation) (Math|Float|Lerp (Variables|Default|GetA) (+ (Variables|Default|GetB) (* (Variables|Default|GetA%20Button%20Time%20Pressed) 1.5e+02)) _newtrack_0) (.z _relativelocation)) false false))
      (:Finished
        (Variables|Default|SetA%20Button%20Time%20Pressed 0.0)))))

(event Input|AxisEvents|InputAxisThrottle
  (params (AxisValue :type Float%20%28single-precision%29))
  (Variables|Default|SetCurrentSpeed (Math|Interpolation|FInterpTo (Variables|Default|GetCurrentSpeed) (* (* AxisValue (Variables|Default|GetThrottle%20Axis)) (Variables|Default|GetMaxSpeed)) (Utilities|Time|GetWorldDeltaSeconds) 4.0))
  (Transformation|AddActorWorldOffset (* (Utilities|Time|GetWorldDeltaSeconds) (* (Transformation|GetActorRightVector) (Variables|Default|GetCurrentSpeed)))))

(event Input|AxisEvents|InputAxisSteer
  (params (AxisValue :type Float%20%28single-precision%29))
  (Variables|Default|SetCurrentSteeringAngle (Math|Interpolation|FInterpTo (Variables|Default|GetCurrentSteeringAngle) (* (* AxisValue (Variables|Default|GetSteer%20Axis)) (Variables|Default|GetMaxSteeringAngle)) (Utilities|Time|GetWorldDeltaSeconds) 1.0))
  (Class|Actor|AddActorWorldRotation (Math|Rotator|MakeRotator 0.0 0.0 (* (Variables|Default|GetCurrentSpeed) (Variables|Default|GetCurrentSteeringAngle) (Variables|Default|GetSpeedToRotationFactor) (Utilities|Time|GetWorldDeltaSeconds)))))

(event Input|AxisEvents|InputAxisLookRight
  (params (AxisValue :type Float%20%28single-precision%29))
  (bind _archer (Variables|Default|GetArcher))
  (bind _relativerotation (Variables|/Script/Engine.SceneComponent|GetRelativeRotation _archer))
  (Transformation|SetRelativeRotation _archer (Math|Rotator|MakeRotator (.roll _relativerotation) (.pitch _relativerotation) (+ (.yaw _relativerotation) AxisValue)) false false))

(fn ConstructionScript)